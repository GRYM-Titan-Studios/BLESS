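; AI controller for a drone that runs its behavior tree and supplies the blackboard with patrol and investigation data.
; On BeginPlay it gets the pawn's patrol path through an interface message and seeds looping, direction, wait time and start index.
; When the player is sensed status arrives, it sets the investigating flag, prints the distance, and targets the midpoint to the player, or its own location if close.
; The other interface functions are empty stubs.
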(event `self.ReceiveBeginPlay`
  (bind _returnvalue (`AIBlueprintHelperLibrary.GetBlackboard` null))
  (`self.RunBehaviorTree` "/Game/Blueprints/AI/BT_Drone.BT_Drone")
  (bind (_b_success _v_pathpoints _bp_patrolpath _start_index) (message `/Game/Blueprints/AI/BPI_NPC.Get_PatrolPath` (`self.K2_GetPawn`) false))
  (`BlackboardComponent.SetValueAsBool` _returnvalue "B_PathLooping" (`/Game/Blueprints/AI/BP_PatrolPath.B_Is_Looping` _bp_patrolpath))
  (`BlackboardComponent.SetValueAsInt` _returnvalue "I_Direction" 1)
  (`BlackboardComponent.SetValueAsFloat` _returnvalue "F_Wait_Time" (`/Game/Blueprints/AI/BP_PatrolPath.F_Wait_Time` _bp_patrolpath))
  (`BlackboardComponent.SetValueAsInt` _returnvalue "I_PatrolPath_Index" _start_index))

(fn `Alert_Level_1`
  (params (Activate :type Boolean) (Alert_Level :type Integer))
  (returns (Success :type Boolean))
  (return false))

(fn `Drone_Sensed_Player`
  (params (B_Sensed :type Boolean))
  (returns (Success :type Boolean))
  (bind _returnvalue (`AIBlueprintHelperLibrary.GetBlackboard` null))
  (bind _returnvalue_2 (`self.K2_GetActorLocation` (`GameplayStatics.GetPlayerCharacter` 0)))
  (bind _returnvalue_3 (`self.K2_GetActorLocation` (`self.K2_GetPawn`)))
  (bind _returnvalue_4 (`KismetMathLibrary.VSize` (- _returnvalue_2 _returnvalue_3)))
  (`BlackboardComponent.SetValueAsBool` _returnvalue "B_Inestigating" B_Sensed)
  (`KismetSystemLibrary.PrintString` (`KismetStringLibrary.Conv_DoubleToString` _returnvalue_4) true true (struct :`R` 0.9375 :`G` 0.130717 :`A` 1.0) 5.0)
  (`BlackboardComponent.SetValueAsVector` _returnvalue "V_TargetLocation" (select `bool` (>= _returnvalue_4 600.0) :`false` _returnvalue_3 :`true` (/ (+ _returnvalue_2 _returnvalue_3) 2.0)))
  (return false))

(fn `Enter_Charging_Pod`
  (params (B_Occupied :type Boolean))
  (returns (B_Success :type Boolean))
  (return false))

(fn `Get_Gun_Ref`
  (returns (Gun_Ref :type "ChildActorComponent Object Reference"))
  (return null))

(fn `Get_NPC_Movement_Ref`
  (params (B_Input :type Boolean))
  (returns (B_Success :type Boolean) (NPC_Character_Movement :type "CharacterMovementComponent Object Reference"))
  (return false null))

(fn `Get_PatrolPath`
  (params (B_Input :type Boolean))
  (returns (B_Success :type Boolean) (V_PathPoints :type "Array of Vector Structure") (BP_PatrolPath :type "/Game/Blueprints/AI/BP_PatrolPath Object Reference") (Start_Index :type Integer))
  (return false _ null 0))

(fn `Gun_Ready`
  (params (`Gun_UP?` :type Boolean))
  (returns (Anim_Finished :type Boolean))
  (return false))

(fn `Kill_Drone`
  (params (Input :type Boolean))
  (returns (Success :type Boolean)))

(fn `NPC_Apply_Damage`
  (params (Damage_Applied :type "Float (double-precision)"))
  (returns (Success :type Boolean) (Destroyed_Actor :type Boolean))
  (return false false))

(fn `NPC_Start_Shooting`
  (params (`B_Can_Shoot?` :type Boolean))
  (returns (Success :type Boolean) (B_Can_Fire :type Boolean))
  (return false false))

(fn `UserConstructionScript`)