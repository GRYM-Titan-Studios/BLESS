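; BP_NPC_SEC_02 is a robot NPC, apparently a security enemy, with a gun child actor attached to its mesh's Gun_Socket.
; Interface functions expose its movement component, patrol path and gun; most others are empty stubs.
; Update_Color drives a dynamic emissive material for alerted, unalerted and stunned states, forwards state to the gun and plays a guarded detection sound.
; Update_Highlight toggles custom depth rendering and prints debug text.
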(event `self.ReceiveBeginPlay`
  (`parent.ReceiveBeginPlay`))

(fn `Add_To_Player_Inventory`
  (params (Added_Item :type "/Game/Blueprints/Gameplay/STRUCT_Player_Item Structure"))
  (returns (Success :type Boolean))
  (return false))

(fn `Add_To_Ship_Inventory`
  (params (STRUCT_New_Item :type "/Game/Blueprints/Gameplay/STRUCT_Ship_Item Structure"))
  (returns (Success :type Boolean))
  (return false))

(fn `Check_Keycard`
  (params (I_Card_Ref :type Integer))
  (returns (B_Keycard_Owned :type Boolean))
  (return false))

(fn `Get_Gun_Ref`
  (returns (Gun_Ref :type "ChildActorComponent Object Reference"))
  (return (`self.ChildActor`)))

(fn `Get_NPC_Movement_Ref`
  (params (B_Input :type Boolean))
  (returns (B_Success :type Boolean) (NPC_Character_Movement :type "CharacterMovementComponent Object Reference"))
  (return false (`self.CharacterMovement`)))

(fn `Get_PatrolPath`
  (params (B_Input :type Boolean))
  (returns (B_Success :type Boolean) (V_PathPoints :type "Array of Vector Structure") (BP_PatrolPath :type "/Game/Blueprints/AI/BP_PatrolPath Object Reference") (Start_Index :type Integer))
  (bind _patrolpath (`self.PatrolPath`)
    (:`then`
      (return false (`/Game/Blueprints/AI/BP_PatrolPath.V_PathPoints` _patrolpath) _patrolpath (`self.I_Start_Index`)))
    (:`else`)))

(fn `Move_Elevator`
  (params (Elevator_Choice :type Integer) (Start_Point_In :type "Float (double-precision)"))
  (returns (Success :type Boolean) (Start_Point :type "Float (double-precision)") (Chosen_Floor :type "Float (double-precision)"))
  (return false 0.0 0.0))

(fn `Open_Elevator_Panel`
  (returns (Success :type Boolean))
  (return false))

(fn `Player_Inventory_Update`
  (params (Input :type Boolean))
  (returns (Success :type Boolean) (Player_Inventory :type "Array of /Game/Blueprints/Gameplay/STRUCT_Player_Item Structure"))
  (return false))

(fn `Player_Invisible?`
  (returns (Success :type Boolean) (Invisible :type Boolean))
  (return false false))

(fn `Ship_Energy_Update`
  (params (Input :type Boolean))
  (returns (Success :type Boolean) (Current_Energy :type Integer) (Max_Energy :type Integer))
  (return false 0 0))

(fn `Ship_Inventory_Update`
  (params (Input :type Boolean))
  (returns (Success :type Boolean) (Ship_Inventory :type "Array of /Game/Blueprints/Gameplay/STRUCT_Ship_Inventory Structure") (Current_Inventory_Count :type "Float (double-precision)") (Max_Inventory_Count :type "Float (double-precision)") (Inventory_Value :type Integer))
  (return false _ 0.0 0.0 0))

(fn `Starting_Information`
  (params (STRUCT_Weapon :type "/Game/Blueprints/Gameplay/STRUCT_Weapons Structure") (B_Check :type Boolean) (I_First :type Integer) (I_Second :type Integer) (I_Third :type Integer) (I_Fourth :type Integer) (`Actor Ref` :type "Actor Object Reference") (V_Location :type "Vector Structure"))
  (returns (Success :type Boolean) (B_Second :type Boolean) (S_String :type String) (S_String_Second :type String) (I_Ref_Int :type Integer) (I_Ref_Int_Second :type Integer))
  (return false false "" "" 0 0))

(fn `Update_Color`
  (params (B_Update :type Boolean) (B_Stunned :type Boolean))
  (returns (Success :type Boolean))
  (bind _childactor (`ChildActorComponent.ChildActor` (`self.ChildActor`)))
  (if (not B_Stunned)
    (`MaterialInstanceDynamic.SetScalarParameterValue` (`self.DMI_Emissive`) "Emissive_Power" 250.0)
    (`MaterialInstanceDynamic.SetVectorParameterValue` (`self.DMI_Emissive`) "Emissive_Colour" (select `bool` B_Update :`false` (struct :`R` 1.0 :`B` 1.0 :`A` 1.0) :`true` (struct :`R` 1.0 :`A` 1.0) :!type "LinearColor Structure"))
    (message `/Game/Blueprints/AI/BPI_NPC.Update Color (NPC)` _childactor B_Update false)
    (if (and B_Update (not (`self.B_Alert_Sounded`)))
      (set `self.B_Alert_Sounded` true)
      (`GameplayStatics.PlaySoundAtLocation` "/Game/Audio/FX/Cues/SC_Enemy_Detected.SC_Enemy_Detected" (0.0 0.0 0.0) (struct) 1.0 1.0 0.0 null null null)
      (else
        (set `self.B_Alert_Sounded` false)))
    (else
      (`MaterialInstanceDynamic.SetScalarParameterValue` (`self.DMI_Emissive`) "Emissive_Power" 0.0)
      (message `/Game/Blueprints/AI/BPI_NPC.Update Color (NPC)` _childactor false true)))
  (return false))

(fn `Update_Display`
  (params (B_Update :type Boolean))
  (returns (Success :type Boolean) (B_Second_Hint :type Boolean) (S_Interact_Type :type String) (S_Second_Interact :type String) (I_Image_Hint_Ref :type Integer))
  (return false false "" "" 0))

(fn `Update_Highlight`
  (params (Highlight :type Boolean) (Pulse_Exclusive :type Boolean))
  (returns (Success :type Boolean) (F_Percent :type "Float (double-precision)"))
  (bind _returnvalue (and Highlight Pulse_Exclusive))
  (`KismetSystemLibrary.PrintString` (`KismetStringLibrary.Concat_StrStr` "BP_NPC Update Highlight = " (`KismetStringLibrary.Conv_BoolToString` _returnvalue)))
  (`PrimitiveComponent.SetRenderCustomDepth` (`self.Mesh`) _returnvalue)
  (return false 0.0))

(fn `Update_Keycard`
  (params (I_Card_Ref :type Integer))
  (returns (Success :type Boolean))
  (return false))

(fn `UserConstructionScript`
  (`parent.UserConstructionScript`)
  (`SceneComponent.K2_AttachToComponent` (`self.ChildActor`) (`self.Mesh`) "Gun_Socket" "SnapToTarget" "SnapToTarget" "SnapToTarget" true)
  (bind _returnvalue (`PrimitiveComponent.CreateDynamicMaterialInstance` (`self.Mesh`) 1 "/Game/Materials/Robots/M_Big_Robot_Emissive.M_Big_Robot_Emissive" "None"))
  (set `self.DMI_Emissive` _returnvalue))

(fn `Within_Ship_Radius`
  (params (B_Within :type Boolean))
  (returns (B_Success :type Boolean))
  (return false))