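; Behavior tree task that measures the navigation path length from the AI pawn to a target and writes it to a Blackboard float.
; The target is the player character when the BPlayer flag is set, otherwise a location read from a Blackboard vector key.
; It finds the path synchronously, so the stored distance follows the navmesh rather than a straight line, and always finishes successfully.
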(event `self.ReceiveExecuteAI`
  (params (OwnerController :type "AIController Object Reference") (ControlledPawn :type "Pawn Object Reference"))
  (bind _returnvalue (`NavigationSystemV1.FindPathToLocationSynchronously` ControlledPawn (`Actor.K2_GetActorLocation` ControlledPawn) (select `bool` (`self.B_Player?`) :`false` (`BTFunctionLibrary.GetBlackboardValueAsVector` (`self.BB_Ref_Location`)) :`true` (`Actor.K2_GetActorLocation` (`GameplayStatics.GetPlayerCharacter` 0))) null null))
  (`BTFunctionLibrary.SetBlackboardValueAsFloat` (`self.BB_Ref`) (`NavigationPath.GetPathLength` _returnvalue))
  (`self.FinishExecute` true))