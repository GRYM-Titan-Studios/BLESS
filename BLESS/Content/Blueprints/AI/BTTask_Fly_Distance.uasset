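; Behavior tree task for a flying AI that measures its distance to player 0 and picks a point to fly toward.
; It writes the horizontal distance between the pawn and the player's mesh to a blackboard float, ignoring height.
; It sets the target location key to the midpoint between the pawn and a point raised above the player's mesh, then immediately finishes successfully.
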(event `self.ReceiveExecuteAI`
  (params (OwnerController :type "AIController Object Reference") (ControlledPawn :type "Pawn Object Reference"))
  (bind _returnvalue (`Actor.K2_GetActorLocation` ControlledPawn))
  (bind _x (.x (`SceneComponent.K2_GetComponentLocation` (`Character.Mesh` (`GameplayStatics.GetPlayerCharacter` 0)))))
  (bind _y (.y (`SceneComponent.K2_GetComponentLocation` (`Character.Mesh` (`GameplayStatics.GetPlayerCharacter` 0)))))
  (`BTFunctionLibrary.SetBlackboardValueAsFloat` (`self.BK_Distance`) (`KismetMathLibrary.VSize` (`KismetMathLibrary.MakeVector` (- (.x _returnvalue) _x) (- (.y _returnvalue) _y))))
  (`BTFunctionLibrary.SetBlackboardValueAsVector` (`self.BK_Target_Location`) (/ (+ _returnvalue (`KismetMathLibrary.MakeVector` _x _y (+ (.z (`SceneComponent.K2_GetComponentLocation` (`Character.Mesh` (`GameplayStatics.GetPlayerCharacter` 0)))) 180.0))) 2.0))
  (`self.FinishExecute` true))