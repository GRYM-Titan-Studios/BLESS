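; BP_NPC is an enemy NPC pawn that tracks health and exchanges interface messages with its AI controller.
; AnyDamage ignores same-class damage, turns EMP hits into stuns, and otherwise reduces health and updates the controller's alert.
; On death, once the controller acknowledges, it unpossesses, ragdolls and raises the GameMode threat level.
; It loads a LaserShotgun data row and supplies its patrol path, but the firing logic is disconnected and most interface functions are stubs.
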(event `Delay_Shot`
  (params (Time :type "Float (double-precision)"))
  ;[1 1 1] Delay
  (`KismetSystemLibrary.Delay` Time)
  (set `self.B_Shot_Delay_Passed` true))

(event `Delay_Reload`
  (params (Reload_Time :type "Float (double-precision)"))
  ;[1 1 1] Delay
  (`KismetSystemLibrary.Delay` Reload_Time)
  (set `self.B_Reloading` false))

(event `self.ReceiveBeginPlay`
  ;[1 1 1] Even Begin Play
  (bind _returnvalue (`|GetDataTableRow` "/Game/Blueprints/Gameplay/DT_Weapons.DT_Weapons" "LaserShotgun")
    (:`then`
      (set `self.STRCUT_Equiped_Weapon` _returnvalue))))

(event `self.ReceiveAnyDamage`
  (params (Damage :type "Float (single-precision)") (DamageType :type "DamageType Object Reference") (InstigatedBy :type "Controller Object Reference") (DamageCauser :type "Actor Object Reference"))
  (bind _f_current_health (`self.F_Current_Health`))
  (bind _returnvalue (<= _f_current_health 0.0))
  (bind _returnvalue_2 (`AIBlueprintHelperLibrary.GetAIController` self))
  ;[1 1 1] Take Damage
  (bind _b_take_damage (`self.Damage_Filter` DamageCauser))
  (if _b_take_damage
    (set `self.F_Current_Health` (- _f_current_health Damage))
    (message `/Game/Blueprints/AI/BPI_NPC.Alert_Level_1` _returnvalue_2 (not _returnvalue) 0)
    (if _returnvalue
      (bind _success (message `/Game/Blueprints/AI/BPI_NPC.NPC_Apply_Damage` _returnvalue_2 0.0))
      (if _success
        (`Controller.UnPossess` (`self.GetController`))
        (`CharacterMovementComponent.DisableMovement` (`self.CharacterMovement`))
        (`PrimitiveComponent.SetCollisionEnabled` (`self.Mesh`) "QueryAndPhysics")
        (`PrimitiveComponent.SetSimulatePhysics` (`self.Mesh`) true)
        (`PrimitiveComponent.SetSimulatePhysics` (`self.CapsuleComponent`) true)
        (message `/Game/Blueprints/Interfaces/BPI_Threat.Update_Current_Threat_Level` (`GameplayStatics.GetGameMode`) false 1.0 0)))))

(fn `Alert_Level_1`
  (params (Activate :type Boolean) (Alert_Level :type Integer))
  (returns (Success :type Boolean))
  (return false))

(fn `Call_Assist`
  (returns (B_Success :type Boolean))
  (return false))

(fn `Can Shoot`
  (returns (B_Can_Shoot :type Boolean))
  (return (and (`self.B_Shot_Delay_Passed`) (not (`self.B_Reloading`)) (> (`self.F_Current_Health`) 0.0))))

(fn `Damage_Filter`
  (params (Actor_Ref :type "Actor Object Reference"))
  (returns (B_Take_Damage :type Boolean))
  (if (`KismetStringLibrary.Contains` (`KismetSystemLibrary.GetDisplayName` Actor_Ref) "EMP")
    (message `/Game/Blueprints/AI/BPI_NPC.Stunned` (`AIBlueprintHelperLibrary.GetAIController` self))
    (elif (== (`GameplayStatics.GetObjectClass` Actor_Ref) (`GameplayStatics.GetObjectClass` self))
      _
      (else
        (return true))))
  (return false))

(fn `Doors`
  (params (B_Locked :type Boolean) (B_Paid :type Boolean) (F_Cost :type "Float (double-precision)"))
  (returns (Success :type Boolean))
  (return true))

(fn `Drone_Sensed_Player`
  (params (B_Sensed :type Boolean))
  (returns (Success :type Boolean))
  (return false))

(fn `Energy_Drain`
  (returns (Success :type Boolean) (Energy_Taken :type "Float (double-precision)") (S_Dialogue :type String))
  (return false 0.0 ""))

(fn `Enter_Charging_Pod`
  (params (B_Occupied :type Boolean))
  (returns (B_Success :type Boolean))
  (return false))

(fn `Get_Gun_Ref`
  (returns (Gun_Ref :type "ChildActorComponent Object Reference"))
  (return null))

(fn `Get_NPC_Movement_Ref`
  (params (B_Input :type Boolean))
  (returns (B_Success :type Boolean) (NPC_Character_Movement :type "CharacterMovementComponent Object Reference"))
  (return false (`self.CharacterMovement`)))

(fn `Get_PatrolPath`
  (params (B_Input :type Boolean))
  (returns (B_Success :type Boolean) (V_PathPoints :type "Array of Vector Structure") (BP_PatrolPath :type "/Game/Blueprints/AI/BP_PatrolPath Object Reference") (Start_Index :type Integer))
  (bind _patrolpath (`self.PatrolPath`)
    (:`then`
      (return false (`/Game/Blueprints/AI/BP_PatrolPath.V_PathPoints` _patrolpath) _patrolpath (`self.I_Start_Index`)))
    (:`else`)))

(fn `Gun_Ready`
  (params (`Gun_UP?` :type Boolean))
  (returns (Anim_Finished :type Boolean))
  (return false))

(fn `Hack_Successful`
  (params (Successful :type Boolean) (Cost_Paid :type Boolean) (I_Door_Cost :type Integer))
  (returns (Success :type Boolean) (Paid :type Boolean))
  (return false false))

(fn `Initiate_Hack`
  (returns (Success :type Boolean) (Unlock_Cost :type Integer) (Open_Cost :type Integer) (Door_Difficulty :type Integer))
  (return false 0 0 0))

(fn `Kill_Drone`
  (params (Input :type Boolean))
  (returns (Success :type Boolean))
  (return false))

(fn `NPC_Apply_Damage`
  (params (Damage_Applied :type "Float (double-precision)"))
  (returns (Success :type Boolean) (Destroyed_Actor :type Boolean))
  (bind _f_current_health (`self.F_Current_Health`))
  (bind _returnvalue (<= _f_current_health 0.0))
  (set `self.F_Current_Health` (- _f_current_health Damage_Applied))
  (if (not _returnvalue)
    (`KismetSystemLibrary.PrintString` "NPC_Damaged"))
  (return true _returnvalue))

(fn `NPC_Start_Shooting`
  (params (`B_Can_Shoot?` :type Boolean))
  (returns (Success :type Boolean) (B_Can_Fire :type Boolean))
  (return true (> (`self.F_Current_Health`) 0.0)))

(fn `Pick_Up_Sorting`
  (returns (Success :type Boolean) (S_Type :type String) (S_Name :type String))
  (return false "" ""))

(fn `Picked_Up`
  (returns (Success :type Boolean))
  (return false))

(fn `Player_Energy_Adjustment`
  (params (Adjustment :type "Float (double-precision)"))
  (returns (Success :type Boolean))
  (return false))

(fn `Player_Health_Adjustment`
  (params (Adjustment :type Integer))
  (returns (Success :type Boolean))
  (return false))

(fn `Set_Pod`
  (params (Pod_Ref :type "Actor Object Reference"))
  (returns (Success :type Boolean) (Send_Pod_Ref :type "Actor Object Reference"))
  (return false null))

(fn `Set_Position`
  (returns (Success :type Boolean) (V_Location :type "Vector Structure"))
  (return false (0.0 0.0 0.0)))

(fn `Spawn_SDrone`
  (returns (Success :type Boolean))
  (return false))

(fn `Stunned`
  (returns (B_Success :type Boolean))
  (return false))

(fn `Teleport_Cost`
  (params (Input :type Boolean) (F_Current_Energy :type "Float (double-precision)"))
  (returns (Success :type Boolean) (`I_Teleport Cost` :type Integer))
  (return (> (`self.F_Current_Health`) 0.0) 0))

(fn `Update Color (NPC)`
  (params (B_Alerted :type Boolean) (B_Stunned :type Boolean))
  (returns (Success :type Boolean))
  (return false))

(fn `UserConstructionScript`)