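; Behavior tree task that nudges the controlled pawn forward after a navigation path query to a Blackboard location.
; It runs a synchronous path search from the controller's location, then checks only that the returned path object is valid.
; If valid, it adds one movement input along the control rotation's yaw, not along the path, and finishes successfully at once.
; Otherwise it finishes as failed.
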(event `self.ReceiveExecuteAI`
  (params (OwnerController :type "AIController Object Reference") (ControlledPawn :type "Pawn Object Reference"))
  (bind (_returnvalue_roll _returnvalue_pitch _returnvalue_yaw) (`KismetMathLibrary.BreakRotator` (`Pawn.GetControlRotation` ControlledPawn)))
  (bind _returnvalue (`NavigationSystemV1.FindPathToLocationSynchronously` (`Actor.K2_GetActorLocation` OwnerController) (`BTFunctionLibrary.GetBlackboardValueAsVector` (`self.BB_LocationKey`)) OwnerController null))
  (`/Engine/EditorBlueprintResources/StandardMacros.IsValid` _returnvalue
    (:`Is Valid`
      (`Pawn.AddMovementInput` ControlledPawn (`KismetMathLibrary.GetForwardVector` (`KismetMathLibrary.MakeRotator` 0.0 0.0 _returnvalue_yaw)) 100.0 false)
      (`self.FinishExecute` true))
    (:`Is Not Valid`
      (`self.FinishExecute` false))))