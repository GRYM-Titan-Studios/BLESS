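; BP_PatrolPath is an AI patrol path actor that builds a list of path point positions from tagged target actors in the level.
; On BeginPlay it finds every BP_Custom_Target whose LocationTag matches its own Tag, appends that location to VPathPoints and prints both location and tag for debugging.
; The construction script holds an unconnected copy of the same gathering logic.
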(event `self.ReceiveBeginPlay`
  (bind _outactors (`GameplayStatics.GetAllActorsOfClass` "/Game/Blueprints/AI/BP_Custom_Target.BP_Custom_Target_C"))
  (for _array_element _outactors
    (bind _location_tag (`/Game/Blueprints/AI/BP_Custom_Target.Location_Tag` _array_element))
    (if (`|EnumEquality` _location_tag (`self.Tag`))
      (bind _returnvalue (`self.K2_GetActorLocation` _array_element))
      (`KismetSystemLibrary.PrintString` (`KismetStringLibrary.Conv_VectorToString` _returnvalue))
      (`KismetSystemLibrary.PrintString` (`|GetEnumeratorNameAsString` _location_tag))
      (`KismetArrayLibrary.Array_Add` (`self.V_PathPoints`) _returnvalue))))

(fn `UserConstructionScript`)