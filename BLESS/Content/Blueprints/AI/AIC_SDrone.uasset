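; AI controller for the SDrone that starts the BT_SDrone behavior tree on BeginPlay.
; Drone_Sensed_Player writes the sensed state to the B_CanSeePlayer blackboard key to feed the tree.
; Other functions, covering alerts, patrol, guns, damage and charging pods, are empty stubs.
; Unconnected logic for seeding patrol blackboard values and computing a target location between drone and player never runs.
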(event `self.ReceiveBeginPlay`
  (`self.RunBehaviorTree` "/Game/Blueprints/AI/BT_SDrone.BT_SDrone"))

(fn `Alert_Level_1`
  (params (Activate :type Boolean) (Alert_Level :type Integer))
  (returns (Success :type Boolean))
  (return false))

(fn `Drone_Sensed_Player`
  (params (B_Sensed :type Boolean))
  (returns (Success :type Boolean))
  (`BlackboardComponent.SetValueAsBool` (`AIBlueprintHelperLibrary.GetBlackboard` null) "B_CanSeePlayer" B_Sensed)
  (return false))

(fn `Enter_Charging_Pod`
  (params (B_Occupied :type Boolean))
  (returns (B_Success :type Boolean))
  (return false))

(fn `Get_Gun_Ref`
  (returns (Gun_Ref :type "ChildActorComponent Object Reference"))
  (return null))

(fn `Get_NPC_Movement_Ref`
  (params (B_Input :type Boolean))
  (returns (B_Success :type Boolean) (NPC_Character_Movement :type "CharacterMovementComponent Object Reference"))
  (return false null))

(fn `Get_PatrolPath`
  (params (B_Input :type Boolean))
  (returns (B_Success :type Boolean) (V_PathPoints :type "Array of Vector Structure") (BP_PatrolPath :type "/Game/Blueprints/AI/BP_PatrolPath Object Reference") (Start_Index :type Integer))
  (return false _ null 0))

(fn `Gun_Ready`
  (params (`Gun_UP?` :type Boolean))
  (returns (Anim_Finished :type Boolean))
  (return false))

(fn `Kill_Drone`
  (params (Input :type Boolean))
  (returns (Success :type Boolean)))

(fn `NPC_Apply_Damage`
  (params (Damage_Applied :type "Float (double-precision)"))
  (returns (Success :type Boolean) (Destroyed_Actor :type Boolean))
  (return false false))

(fn `NPC_Start_Shooting`
  (params (`B_Can_Shoot?` :type Boolean))
  (returns (Success :type Boolean) (B_Can_Fire :type Boolean))
  (return false false))

(fn `UserConstructionScript`)