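; A behavior tree task that sets the AI's chase status on the blackboard and updates its gun to match.
; On execute it writes the configured status enum to the chase status key, clears the controller's focus and fetches the pawn's gun through a message.
; For the first status it sends the gun a ready-off message, for the second a kill-drone-off message, then finishes successfully.
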(event `self.ReceiveExecuteAI`
  (params (OwnerController :type "AIController Object Reference") (ControlledPawn :type "Pawn Object Reference"))
  (bind _enum_status (`self.ENUM_Status`))
  (`BTFunctionLibrary.SetBlackboardValueAsEnum` (`self.BB_Chase_Status`) _enum_status)
  (`AIController.K2_ClearFocus` OwnerController)
  (bind _gun_ref (message `/Game/Blueprints/AI/BPI_NPC.Get_Gun_Ref` ControlledPawn))
  (if (`|EnumEquality` _enum_status "NewEnumerator0")
    (bind _childactor (`ChildActorComponent.ChildActor` _gun_ref))
    (message `/Game/Blueprints/AI/BPI_NPC.Gun_Ready` _childactor false)
    (elif (`|EnumEquality` _enum_status "NewEnumerator1")
      (message `/Game/Blueprints/AI/BPI_NPC.Kill_Drone` _childactor false)))
  (`self.FinishExecute` true))