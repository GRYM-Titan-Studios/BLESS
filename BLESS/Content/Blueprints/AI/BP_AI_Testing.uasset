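; BP_AI_Testing is a test AI Blueprint that uses PawnSensing to detect pawns.
; Only sight is active: seeing a pawn prints its display name, while the hearing event does nothing.
; Disconnected leftovers include printing a noise instigator, chasing a pawn with AIMoveTo, and a "CAUGHT" message followed by a delayed return to the main menu level.
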(event `self.PawnSensing.OnSeePawn`
  (params (Pawn :type "Pawn Object Reference"))
  (`KismetSystemLibrary.PrintString` (`KismetSystemLibrary.GetDisplayName` Pawn)))

(event `self.PawnSensing.OnHearNoise`
  (params (Instigator :type "Pawn Object Reference") (Location :type "Vector Structure (by ref)") (Volume :type "Float (single-precision)")))

(fn `UserConstructionScript`)