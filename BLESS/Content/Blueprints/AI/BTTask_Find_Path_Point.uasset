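; Behavior tree task that picks the current patrol point for an AI pawn and writes it to the blackboard.
; It gets the patrol path from the pawn through GetPatrolPathMessage and indexes its points with the blackboard path index.
; If the untransformed point projects onto navigation, it stores the point transformed by the path actor and finishes successfully.
; A failed projection never calls FinishExecute.
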(event `self.ReceiveExecuteAI`
  (params (OwnerController :type "AIController Object Reference") (ControlledPawn :type "Pawn Object Reference"))
  (bind (_b_success _v_pathpoints _bp_patrolpath) (message `/Game/Blueprints/AI/BPI_NPC.Get_PatrolPath` ControlledPawn false))
  (bind _output (`|GetArrayItem` _v_pathpoints (`BTFunctionLibrary.GetBlackboardValueAsInt` (`self.BB_Path_Index`))))
  (if (`.ReturnValue` (`NavigationSystemV1.K2_ProjectPointToNavigation` _output))
    (`BTFunctionLibrary.SetBlackboardValueAsVector` (`self.BB_Path_Vector`) (`KismetMathLibrary.TransformLocation` (`Actor.GetTransform` _bp_patrolpath) _output))
    (`self.FinishExecute` true)))