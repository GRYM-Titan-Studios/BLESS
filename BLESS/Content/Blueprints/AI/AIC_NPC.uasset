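; AI controller for NPCs that runs BT_NPC, seeds its blackboard with patrol path data and turns perception stimuli into blackboard state.
; Sensing_Sort_Macro treats stimuli by array index: sight of a visible player drives a delay-looped detection meter widget, and being shot at boosts it.
; Tagged noises pick a trace channel for a line-of-sight check, and unblocked ones trigger investigation.
; The older SensingSort function is only called from disconnected nodes.
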(event `self.ReceiveBeginPlay`
  (bind _returnvalue (`AIBlueprintHelperLibrary.GetBlackboard` null))
  ;[1 1 1] Begin Play
  (`self.RunBehaviorTree` "/Game/Blueprints/AI/BT_NPC.BT_NPC")
  (bind (_b_success _v_pathpoints _bp_patrolpath _start_index) (message `/Game/Blueprints/AI/BPI_NPC.Get_PatrolPath` (`self.K2_GetPawn`) false))
  (`BlackboardComponent.SetValueAsBool` _returnvalue "B_PathLooping" (`/Game/Blueprints/AI/BP_PatrolPath.B_Is_Looping` _bp_patrolpath))
  (`BlackboardComponent.SetValueAsInt` _returnvalue "I_Direction" 1)
  (`BlackboardComponent.SetValueAsFloat` _returnvalue "F_Wait_Time" (`/Game/Blueprints/AI/BP_PatrolPath.F_Wait_Time` _bp_patrolpath))
  (`BlackboardComponent.SetValueAsInt` _returnvalue "I_PatrolPath_Index" _start_index))

(event `self.AIPerception .OnTargetPerceptionUpdated`
  (params (Actor :type "Actor Object Reference") (Stimulus :type "AIStimulus Structure")))

(event `self.AIPerception .OnPerceptionUpdated`
  (params (UpdatedActors :type "Array of Actor Object Reference (by ref)"))
  (for _array_element UpdatedActors
    (bind _info (`AIPerceptionComponent.GetActorsPerception` (`self.AIPerception `) _array_element))
    (`self.Sensing_Sort_Macro` (`.LastSensedStimuli` (break `ActorPerceptionBlueprintInfo` _info)) (break `ActorPerceptionBlueprintInfo` _info))))

(event `self.ReceiveAnyDamage`
  (params (Damage :type "Float (single-precision)") (DamageType :type "DamageType Object Reference") (InstigatedBy :type "Controller Object Reference") (DamageCauser :type "Actor Object Reference")))

(fn `Alert_Level_1`
  (params (Activate :type Boolean))
  (returns (Success :type Boolean))
  (`BlackboardComponent.SetValueAsBool` (`AIBlueprintHelperLibrary.GetBlackboard` null) "B_Activated" Activate)
  (return false))

(fn `Enter_Charging_Pod`
  (params (B_Occupied :type Boolean))
  (returns (B_Success :type Boolean))
  (return false))

(fn `Get_NPC_Movement_Ref`
  (params (B_Input :type Boolean))
  (returns (B_Success :type Boolean) (NPC_Character_Movement :type "CharacterMovementComponent Object Reference"))
  (return false null))

(fn `Get_PatrolPath`
  (params (B_Input :type Boolean))
  (returns (B_Success :type Boolean) (V_PathPoints :type "Array of Vector Structure") (BP_PatrolPath :type "/Game/Blueprints/AI/BP_PatrolPath Object Reference") (Start_Index :type Integer))
  (return false _ null 0))

(fn `Kill_Drone`
  (params (Input :type Boolean))
  (returns (Success :type Boolean))
  (return false))

(fn `NPC_Apply_Damage`
  (params (Damage_Applied :type "Float (double-precision)"))
  (returns (Success :type Boolean) (Destroyed_Actor :type Boolean))
  (`KismetSystemLibrary.PrintString` "Remove From Viewport" true true (struct :`R` 1.0 :`G` 0.29927 :`A` 1.0))
  (`Widget.RemoveFromParent` (`self.UI_Detection_Meter_Ref`))
  (set `self.UI_Detection_Meter_Ref` null)
  (return true false))

(fn `NPC_Start_Shooting`
  (returns (Success :type Boolean))
  (return false))

(fn `Sensing_Sort`
  (params (Array :type "Array of AIStimulus Structure") (Actor_Ref :type "Actor Object Reference"))
  (locals (STRUCT_Local_Sense :type "AIStimulus Structure"))
  (bind _returnvalue (`AIBlueprintHelperLibrary.GetBlackboard` null))
  (bind _returnvalue_2 (`AIBlueprintHelperLibrary.GetBlackboard` null))
  (bind _f_detectionlevel (`self.F_DetectionLevel`))
  (bind (_age _expirationage _strength _stimuluslocation _receiverlocation _tag) (break `AIStimulus` (`local.STRUCT_Local_Sense`)))
  (bind (_age_2 _expirationage_2 _strength_2 _stimuluslocation_2 _receiverlocation_2 _tag_2 _bsuccessfullysensed) (break `AIStimulus` (`local.STRUCT_Local_Sense`)))
  (bind (_age_3 _expirationage_3 _strength_3 _stimuluslocation_3 _receiverlocation_3 _tag_3 _bsuccessfullysensed_2) (break `AIStimulus` (`local.STRUCT_Local_Sense`)))
  (for (_array_element _array_index) Array
    (set `local.STRUCT_Local_Sense` _array_element)
    (switch `int` _array_index
      (:`0`
        (bind (_success _invisible) (message `/Game/Blueprints/Interfaces/BPI_Data_Transfer.Player_Invisible?` (`GameplayStatics.GetPlayerCharacter` 0)))
        (if _invisible
          (`BlackboardComponent.SetValueAsBool` (`AIBlueprintHelperLibrary.GetBlackboard` null) "B_CanSeePlayer" false)
          (elif _bsuccessfullysensed
            (set `self.B_Detecting` true)
            (set `self.F_DetectionLevel` 0.0)
            (bind _returnvalue_3 (`|CreateWidget` "/Game/UI/Detection/Widget_Detection_Meter.Widget_Detection_Meter_C" (`GameplayStatics.GetPlayerController` 0) 0.0 null))
            (bind _output_get (set `self.UI_Detection_Meter_Ref` _returnvalue_3))
            (`UserWidget.AddToViewport` _output_get 0)
            (`/Game/UI/Detection/Widget_Detection_Meter.Set_Detection_Level` _output_get (+ _f_detectionlevel (select `bool` (`self.B_Detecting`) :`false` -0.01 :`true` 0.01 :!type "Float (single-precision)")))
            (if (> _f_detectionlevel 1.0)
              (`BlackboardComponent.SetValueAsBool` (`AIBlueprintHelperLibrary.GetBlackboard` null) "B_CanSeePlayer" true)
              (elif (< _f_detectionlevel 0.0)
                (`BlackboardComponent.SetValueAsBool` (`AIBlueprintHelperLibrary.GetBlackboard` null) "B_CanSeePlayer" false)
                (elif (not (`self.B_Detecting`))
                  (`Widget.RemoveFromParent` (`self.UI_Detection_Meter_Ref`)))))
            (else
              (set `self.B_Detecting` false)))))
      (:`1`
        (`BlackboardComponent.SetValueAsBool` _returnvalue_2 "B_Shot_At?" _bsuccessfullysensed)
        (`BlackboardComponent.SetValueAsVector` _returnvalue_2 "V_TargetLocation" _stimuluslocation_2)
        (`KismetSystemLibrary.PrintString` (`KismetSystemLibrary.GetDisplayName` Actor_Ref)))
      (:`2`
        (switch `name` _tag
          (:`Noise`
            (bind (_outhit _returnvalue_4) (`KismetSystemLibrary.LineTraceSingleForObjects` :`Start` (`self.K2_GetActorLocation` (`self.K2_GetPawn`)) :`End` _stimuluslocation :`ObjectTypes` (`|MakeArray` "ObjectTypeQuery1" "ObjectTypeQuery2" :!type "EObjectTypeQuery Enum") :`DrawDebugType` "ForDuration" :!label _label))
            (if _returnvalue_4
              (`KismetSystemLibrary.PrintString` "Hit-Object")
              (else
                (`BlackboardComponent.SetValueAsBool` _returnvalue "B_Inestigating" _bsuccessfullysensed_2)
                (`BlackboardComponent.SetValueAsVector` _returnvalue "V_TargetLocation" _stimuluslocation_3)
                (`KismetSystemLibrary.PrintString` (`KismetStringLibrary.Conv_DoubleToString` (`NavigationSystemV1.GetPathLength` (`self.K2_GetActorLocation` (`self.K2_GetPawn`)) _stimuluslocation_3 null null)) true true (struct :`G` 0.66 :`B` 1.0 :`A` 1.0) 5.0))))
          (:`Walk`
            (if (== Actor_Ref (`GameplayStatics.GetPlayerCharacter` 0))
              (goto _label))))))))

(fn `Set_Detecting_Blackboard`
  (params (Detecting :type Boolean))
  (`BlackboardComponent.SetValueAsBool` (`AIBlueprintHelperLibrary.GetBlackboard` null) "B_Detecting" Detecting))

(fn `UserConstructionScript`)