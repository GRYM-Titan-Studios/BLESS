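; Flying NPC drone that spots the player, sounds a horn and raises the game mode's threat level.
; Tick animates blade spin and hover bob.
; Pawn sensing checks player invisibility, reports to the controller and turns the emissive material red until a retriggerable delay resets it.
; Damage adds threat and triggers the rate-limited horn or an exploding death, while interface functions supply patrol path and highlighting, the rest being stubs.
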(event `self.ReceiveBeginPlay`
  (bind _returnvalue (`GameplayStatics.SpawnSoundAttached` "/Game/Audio/FX/Cues/SC_Drone_Rotor_Blades.SC_Drone_Rotor_Blades" (`self.CollisionComponent`) "None" (0.0 0.0 0.0) (struct) "KeepRelativeOffset" false 0.3 1.0 0.0 "/Game/Audio/Attenuation/SA_Doors.SA_Doors" null))
  (set `self.Blade_Noise` _returnvalue))

(event `self.ReceiveTick`
  (params (DeltaSeconds :type "Float (single-precision)"))
  (bind _f_bob (`self.F_Bob`))
  (bind _f_bob_2 (`self.F_Bob`))
  (set `self.F_Rotation` (+ (`self.F_Rotation`) 36.0))
  (if (>= (`self.F_Rotation`) 360.0)
    (set `self.F_Rotation` 0.0))
  (`SceneComponent.K2_SetRelativeRotation` (`self.SM_Steam_Drone_Blades`) (`KismetMathLibrary.MakeRotator` 0.0 0.0 (`self.F_Rotation`)) false false)
  (if (<= _f_bob_2 -55.0)
    (set `self.B_Move_Up` true)
    (elif (>= _f_bob_2 -5.0)
      (set `self.B_Move_Up` false)))
  (if (`self.B_Move_Up`)
    (set `self.F_Bob` (+ _f_bob 0.5))
    (else
      (set `self.F_Bob` (- _f_bob 0.5))))
  (`SceneComponent.K2_SetRelativeLocation` (`self.MeshComponent`) (`KismetMathLibrary.MakeVector` 0.0 0.0 (`self.F_Bob`)) false false))

(event `self.ReceiveAnyDamage`
  (params (Damage :type "Float (single-precision)") (DamageType :type "DamageType Object Reference") (InstigatedBy :type "Controller Object Reference") (DamageCauser :type "Actor Object Reference"))
  (bind _output_get (set `self.F_Current_Health` (- (`self.F_Current_Health`) Damage)))
  (if (< _output_get 0.0)
    (`self.Drone_Death`)
    (else
      (message `/Game/Blueprints/Interfaces/BPI_Threat.Update_Current_Threat_Level` (`GameplayStatics.GetGameMode`) false 0.2 0)
      (`self.Drone_Noise`))))

(event `Drone_Death`
  ;[1 1 1] Drone Death
  (message `/Game/Blueprints/Interfaces/BPI_Threat.Update_Current_Threat_Level` (`GameplayStatics.GetGameMode`) false 0.5 0)
  (`AudioComponent.SetVolumeMultiplier` (`self.Blade_Noise`) 0.0)
  (`SceneComponent.K2_DetachFromComponent` (`self.SkeletalMesh`) "KeepWorld" "KeepWorld" "KeepWorld" true)
  (`SceneComponent.K2_DetachFromComponent` (`self.MeshComponent`) "KeepWorld" "KeepWorld" "KeepWorld" true)
  (`PrimitiveComponent.SetSimulatePhysics` (`self.SkeletalMesh`) true)
  (`PrimitiveComponent.SetSimulatePhysics` (`self.MeshComponent`) true)
  (`GameplayStatics.SpawnEmitterAtLocation` "/Game/Particles/P_S_Explosion.P_S_Explosion" (`SceneComponent.K2_GetComponentLocation` (`self.CollisionComponent`)))
  (`self.K2_DestroyActor` self))

(event `self.PawnSensing.OnSeePawn`
  (params (Pawn :type "Pawn Object Reference"))
  ;[1 1 1] React to the Player
  (bind (_success _invisible) (message `/Game/Blueprints/Interfaces/BPI_Data_Transfer.Player_Invisible?` Pawn))
  (if _success
    (if _invisible
      (message `/Game/Blueprints/AI/BPI_NPC.Drone_Sensed_Player` (`self.GetController`) false :!label _label)
      (else
        (`MaterialInstanceDynamic.SetVectorParameterValue` (`self.DIM_Detail`) "Emissive_Colour" (struct :`R` 1.0 :`B` 0.018721 :`A` 1.0))
        (`self.Unseen`)
        (`self.Drone_Noise`)
        (message `/Game/Blueprints/AI/BPI_NPC.Drone_Sensed_Player` (`self.GetController`) true)))
    (else
      (goto _label))))

(event `Unseen`
  ;[1 1 1] Reset Drone Color
  (`KismetSystemLibrary.RetriggerableDelay` 5.0)
  (`MaterialInstanceDynamic.SetVectorParameterValue` (`self.DIM_Detail`) "Emissive_Colour" (struct :`R` 1.0 :`B` 1.0 :`A` 1.0))
  (message `/Game/Blueprints/AI/BPI_NPC.Drone_Sensed_Player` (`self.GetController`) false))

(event `Noise_Delay`
  ;[1 1 1] Prevent Multiple Noises
  (`KismetSystemLibrary.Delay` (`SoundBase.Duration` (`self.SB_Horn`)))
  (set `self.B_Noise_Active` false))

(fn `Add_To_Player_Inventory`
  (params (Added_Item :type "/Game/Blueprints/Gameplay/STRUCT_Player_Item Structure"))
  (returns (Success :type Boolean))
  (return false))

(fn `Add_To_Ship_Inventory`
  (params (STRUCT_New_Item :type "/Game/Blueprints/Gameplay/STRUCT_Ship_Item Structure"))
  (returns (Success :type Boolean))
  (return false))

(fn `Alert_Level_1`
  (params (Activate :type Boolean) (Alert_Level :type Integer))
  (returns (Success :type Boolean))
  (return false))

(fn `Call_Assist`
  (returns (B_Success :type Boolean))
  (return false))

(fn `Check_Keycard`
  (params (I_Card_Ref :type Integer))
  (returns (B_Keycard_Owned :type Boolean))
  (return false))

(fn `Drone_Noise`
  (if (not (`self.B_Noise_Active`))
    (set `self.B_Noise_Active` true)
    (`GameplayStatics.PlaySoundAtLocation` (`self.SB_Horn`) (`SceneComponent.K2_GetComponentLocation` (`self.CollisionComponent`)) (struct) 1.0 1.0 0.0 null null null)
    (message `/Game/Blueprints/Interfaces/BPI_Threat.Update_Current_Threat_Level` (`GameplayStatics.GetGameMode`) false 0.1 0)
    (`self.Noise_Delay`)))

(fn `Drone_Sensed_Player`
  (params (B_Sensed :type Boolean))
  (returns (Success :type Boolean))
  (return false))

(fn `Enter_Charging_Pod`
  (params (B_Occupied :type Boolean))
  (returns (B_Success :type Boolean))
  (return false))

(fn `Get_Gun_Ref`
  (returns (Gun_Ref :type "ChildActorComponent Object Reference"))
  (return null))

(fn `Get_NPC_Movement_Ref`
  (params (B_Input :type Boolean))
  (returns (B_Success :type Boolean) (NPC_Character_Movement :type "CharacterMovementComponent Object Reference"))
  (return false null))

(fn `Get_PatrolPath`
  (params (B_Input :type Boolean))
  (returns (B_Success :type Boolean) (V_PathPoints :type "Array of Vector Structure") (BP_PatrolPath :type "/Game/Blueprints/AI/BP_PatrolPath Object Reference") (Start_Index :type Integer))
  (bind _patrolpath (`self.PatrolPath`)
    (:`then`
      (return false (`/Game/Blueprints/AI/BP_PatrolPath.V_PathPoints` _patrolpath) _patrolpath (`self.I_Start_Index`)))
    (:`else`)))

(fn `Gun_Ready`
  (params (`Gun_UP?` :type Boolean))
  (returns (Anim_Finished :type Boolean))
  (return false))

(fn `Kill_Drone`
  (params (Input :type Boolean))
  (returns (Success :type Boolean))
  (return false))

(fn `Move_Elevator`
  (params (Elevator_Choice :type Integer) (Start_Point_In :type "Float (double-precision)"))
  (returns (Success :type Boolean) (Start_Point :type "Float (double-precision)") (Chosen_Floor :type "Float (double-precision)"))
  (return false 0.0 0.0))

(fn `NPC_Apply_Damage`
  (params (Damage_Applied :type "Float (double-precision)"))
  (returns (Success :type Boolean) (Destroyed_Actor :type Boolean))
  (return false false))

(fn `NPC_Start_Shooting`
  (params (`B_Can_Shoot?` :type Boolean))
  (returns (Success :type Boolean) (B_Can_Fire :type Boolean))
  (return false false))

(fn `Open_Elevator_Panel`
  (returns (Success :type Boolean))
  (return false))

(fn `Player_Inventory_Update`
  (params (Input :type Boolean))
  (returns (Success :type Boolean) (Player_Inventory :type "Array of /Game/Blueprints/Gameplay/STRUCT_Player_Item Structure"))
  (return false))

(fn `Player_Invisible?`
  (returns (Success :type Boolean) (Invisible :type Boolean))
  (return false false))

(fn `Set_Pod`
  (params (Pod_Ref :type "Actor Object Reference"))
  (returns (Success :type Boolean) (Send_Pod_Ref :type "Actor Object Reference"))
  (return false null))

(fn `Set_Position`
  (returns (Success :type Boolean) (V_Location :type "Vector Structure"))
  (return false (0.0 0.0 0.0)))

(fn `Ship_Energy_Update`
  (params (Input :type Boolean))
  (returns (Success :type Boolean) (Current_Energy :type Integer) (Max_Energy :type Integer))
  (return false 0 0))

(fn `Ship_Inventory_Update`
  (params (Input :type Boolean))
  (returns (Success :type Boolean) (Ship_Inventory :type "Array of /Game/Blueprints/Gameplay/STRUCT_Ship_Inventory Structure") (Current_Inventory_Count :type "Float (double-precision)") (Max_Inventory_Count :type "Float (double-precision)") (Inventory_Value :type Integer))
  (return false _ 0.0 0.0 0))

(fn `Spawn_SDrone`
  (returns (Success :type Boolean))
  (return false))

(fn `Starting_Information`
  (params (STRUCT_Weapon :type "/Game/Blueprints/Gameplay/STRUCT_Weapons Structure") (B_Check :type Boolean) (I_First :type Integer) (I_Second :type Integer) (I_Third :type Integer) (I_Fourth :type Integer) (`Actor Ref` :type "Actor Object Reference") (V_Location :type "Vector Structure"))
  (returns (Success :type Boolean) (B_Second :type Boolean) (S_String :type String) (S_String_Second :type String) (I_Ref_Int :type Integer) (I_Ref_Int_Second :type Integer))
  (return false false "" "" 0 0))

(fn `Update Color`
  (params (B_Alerted :type Boolean))
  (returns (Success :type Boolean))
  (return false))

(fn `Update_Color`
  (params (B_Update :type Boolean))
  (returns (Success :type Boolean))
  (return false))

(fn `Update_Display`
  (params (B_Update :type Boolean))
  (returns (Success :type Boolean) (B_Second_Hint :type Boolean) (S_Interact_Type :type String) (S_Second_Interact :type String) (I_Image_Hint_Ref :type Integer))
  (return false false "" "" 0))

(fn `Update_Highlight`
  (params (Highlight :type Boolean) (Pulse_Exclusive :type Boolean))
  (returns (Success :type Boolean) (F_Percent :type "Float (double-precision)"))
  (`PrimitiveComponent.SetRenderCustomDepth` (`self.MeshComponent`) (and Highlight Pulse_Exclusive))
  (`PrimitiveComponent.SetRenderCustomDepth` (`self.SM_Steam_Drone_Blades`) (and Highlight Pulse_Exclusive))
  (`PrimitiveComponent.SetRenderCustomDepth` (`self.SM_Steam_Drone_Detail`) (and Highlight Pulse_Exclusive))
  (`PrimitiveComponent.SetRenderCustomDepth` (`self.SM_Steam_Drone_Radar`) (and Highlight Pulse_Exclusive))
  (return false 0.0))

(fn `Update_Keycard`
  (params (I_Card_Ref :type Integer))
  (returns (Success :type Boolean))
  (return false))

(fn `UserConstructionScript`
  (bind _returnvalue (`PrimitiveComponent.CreateDynamicMaterialInstance` (`self.SM_Steam_Drone_Detail`) 0 "/Game/Materials/Drone/MI_Drone_Details.MI_Drone_Details" "None"))
  (bind _output_get (set `self.DIM_Detail` _returnvalue))
  (`PrimitiveComponent.SetMaterial` (`self.SM_Steam_Drone_Detail`) 0 _output_get)
  (`MaterialInstanceDynamic.SetVectorParameterValue` (`self.DIM_Detail`) "Emissive_Colour" (struct :`R` 1.0 :`B` 1.0 :`A` 1.0)))

(fn `Within_Ship_Radius`
  (params (B_Within :type Boolean))
  (returns (B_Success :type Boolean))
  (return false))