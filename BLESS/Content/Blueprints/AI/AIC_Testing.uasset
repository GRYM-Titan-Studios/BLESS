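; Test AI controller that walks its BP_AI_Testing pawn along that pawn's waypoint array.
; BeginPlay caches the waypoints, moves to the current one, then pauses briefly before starting Patrol.
; Patrol re-calls itself after each successful move, reversing at either end for a ping-pong route, unless an enemy-found flag is set.
; A looping timer calls Check_Enemy, but it and On_Hunt are empty stubs.
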(event `self.ReceiveBeginPlay`
  (bind _asbp_ai_testing (cast `/Game/Blueprints/AI/BP_AI_Testing` (`self.K2_GetPawn`)))
  (set `self.AC_Waypoints_Local` (`/Game/Blueprints/AI/BP_AI_Testing.AC_Waypoint` _asbp_ai_testing))
  (bind _returnvalue (`KismetSystemLibrary.K2_SetTimer` null "Check_Enemy" 0.3 true))
  (set `self.TH_Clean` _returnvalue)
  (`|AIMoveTo` _asbp_ai_testing (0.0 0.0 0.0) (`|GetArrayItem` (`self.AC_Waypoints_Local`) (`self.I_Current_Waypoint`)) (`self.F_Radius`)
    (:`OnSuccess`
      (`KismetSystemLibrary.Delay` 2.0)
      (`self.Patrol`))))

(event `Patrol`
  (if (not (`self.B_FoundEnemy`))
    (if (`self.B_WalkBack`)
      (`/Engine/EditorBlueprintResources/StandardMacros.DecrementInt` (`self.I_Current_Waypoint`)
        (:`  `
          (`|AIMoveTo` null (0.0 0.0 0.0) (`|GetArrayItem` (`self.AC_Waypoints_Local`) (`self.I_Current_Waypoint`)) (`self.F_Radius`)
            (:`OnSuccess`
              (if (<= (`self.I_Current_Waypoint`) 0)
                (set `self.B_WalkBack` false))))))
      (else
        (`/Engine/EditorBlueprintResources/StandardMacros.IncrementInt` (`self.I_Current_Waypoint`)
          (:`  `
            (`|AIMoveTo` null (0.0 0.0 0.0) (`|GetArrayItem` (`self.AC_Waypoints_Local`) (`self.I_Current_Waypoint`)) (`self.F_Radius`)
              (:`OnSuccess`
                (if (>= (`self.I_Current_Waypoint`) (- (`KismetArrayLibrary.Array_Length` (`self.AC_Waypoints_Local`)) 1))
                  (set `self.B_WalkBack` true))))))))
    (`self.Patrol`)))

(event `On_Hunt`)

(event `Check_Enemy`)

(fn `UserConstructionScript`)