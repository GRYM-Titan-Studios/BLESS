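; Behavior tree task that steps an AI's patrol path index backward by one while the blackboard direction is -1.
; It writes the new index to the blackboard and succeeds as long as the index stays at zero or above.
; At the start of the path it flips the direction to forward and fails without changing the index.
; It also fails immediately for any other direction value.
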(event `self.ReceiveExecuteAI`
  (params (OwnerController :type "AIController Object Reference") (ControlledPawn :type "Pawn Object Reference"))
  (bind _bb_direction (`self.BB_Direction`))
  (bind _returnvalue (- (`BTFunctionLibrary.GetBlackboardValueAsInt` (`self.BB_PatrolPath_Index`)) 1))
  (if (== (`BTFunctionLibrary.GetBlackboardValueAsInt` (`self.BB_Direction`)) -1)
    (if (>= _returnvalue 0)
      (`BTFunctionLibrary.SetBlackboardValueAsInt` _bb_direction -1)
      (`BTFunctionLibrary.SetBlackboardValueAsInt` (`self.BB_PatrolPath_Index`) _returnvalue)
      (`self.FinishExecute` true)
      (else
        (`BTFunctionLibrary.SetBlackboardValueAsInt` _bb_direction 1)
        (`self.FinishExecute` false)))
    (else
      (`self.FinishExecute` false))))