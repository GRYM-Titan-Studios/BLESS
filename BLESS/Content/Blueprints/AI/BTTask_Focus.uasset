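; Behavior Tree task that makes an NPC focus on the player and start its gun shooting.
; On execute it sets controller focus, gets the gun child actor from the pawn, readies it, and relays the pawn's can-fire result through interface messages, then finishes successfully.
; On abort it un-readies the gun and calls Finish Execute rather than Finish Abort.
; The debug prints are disconnected.
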(event `self.ReceiveExecuteAI`
  (params (OwnerController :type "AIController Object Reference") (ControlledPawn :type "Pawn Object Reference"))
  (`AIController.K2_SetFocus` OwnerController (`GameplayStatics.GetPlayerCharacter` 0))
  (bind _gun_ref (message `/Game/Blueprints/AI/BPI_NPC.Get_Gun_Ref` ControlledPawn))
  (bind _childactor (`ChildActorComponent.ChildActor` _gun_ref))
  (message `/Game/Blueprints/AI/BPI_NPC.Gun_Ready` _childactor true)
  (bind (_success _b_can_fire) (message `/Game/Blueprints/AI/BPI_NPC.NPC_Start_Shooting` ControlledPawn false))
  (bind _success_2 (message `/Game/Blueprints/AI/BPI_NPC.NPC_Start_Shooting` _childactor _b_can_fire))
  (`self.FinishExecute` true))

(event `self.ReceiveAbort`
  (params (OwnerActor :type "Actor Object Reference"))
  (bind _anim_finished (message `/Game/Blueprints/AI/BPI_NPC.Gun_Ready` (`ChildActorComponent.ChildActor` (stale `self.ReceiveExecuteAI` _gun_ref)) false))
  (`self.FinishExecute` _anim_finished))