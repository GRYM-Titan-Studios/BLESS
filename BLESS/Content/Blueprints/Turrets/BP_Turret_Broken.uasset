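; Turret actor that opens its shutters and deploys, then sweeps in a seeking rotation.
; The Deploy event plays a timeline that swings five door meshes open and lowers the base mesh, setting a deployed flag when finished.
; While deployed with no target acquired, Tick spins the base by a fixed per-frame yaw step, making the speed frame-rate dependent.
; No targeting or firing logic is present in these graphs.
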(event `Deploy`
  ;[1 1 1] Deploy the Turret when activated
  (bind (_direction _shutters _base_drop) (`Timeline|Deployment`)
    (:`Update`
      (bind _returnvalue (* _shutters 60.0))
      (`SceneComponent.K2_SetRelativeRotation` (`self.SM_Turret_Door_5`) (`KismetMathLibrary.MakeRotator` 0.0 0.0 _returnvalue) false false)
      (`SceneComponent.K2_SetRelativeRotation` (`self.SM_Turret_Door_4`) (`KismetMathLibrary.MakeRotator` 0.0 0.0 _returnvalue) false false)
      (`SceneComponent.K2_SetRelativeRotation` (`self.SM_Turret_Door_3`) (`KismetMathLibrary.MakeRotator` 0.0 0.0 _returnvalue) false false)
      (`SceneComponent.K2_SetRelativeRotation` (`self.SM_Turret_Door_2`) (`KismetMathLibrary.MakeRotator` 0.0 0.0 _returnvalue) false false)
      (`SceneComponent.K2_SetRelativeRotation` (`self.SM_Turret_Door_1`) (`KismetMathLibrary.MakeRotator` 0.0 0.0 _returnvalue) false false)
      (`SceneComponent.K2_SetRelativeLocation` (`self.SM_Turret_Base`) (`KismetMathLibrary.MakeVector` -150.0 -150.0 (- 85.0 (* _base_drop 80.0))) false false))
    (:`Finished`
      (set `self.B_Deployed` true))))

(event `self.ReceiveBeginPlay`)

(event `self.ReceiveTick`
  (params (DeltaSeconds :type "Float (single-precision)"))
  (bind _f_rotation (`self.F_Rotation`))
  ;[1 1 1] Rotation While Seeking
  (if (`self.B_Deployed`)
    (if (not (`self.B_Target_Acquired`))
      (`SceneComponent.K2_SetRelativeRotation` (`self.SM_Turret_Base`) (`KismetMathLibrary.MakeRotator` 0.0 0.0 _f_rotation) false false)
      (set `self.F_Rotation` (+ _f_rotation 1.0))
      (if (== _f_rotation 360.0)
        (set `self.F_Rotation` 0.0)))))

(fn `UserConstructionScript`)