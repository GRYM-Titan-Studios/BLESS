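; Placeable turret that detects NPC or Player actors by name in a scan box, yaws its top to track them and explodes when health runs out.
; The box widens while targeting, and timelines slide three vents to arm, then move one per shot.
; Each shot flares the barrel's dynamic material and light before spawning BP_Projectile_Turret.
; A BeginPlay test loop also fires volleys regardless of targeting.
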(event `Arming Phase`
  ;[1 1 1] Arming Phase
  (if (`self.B_Armed`)
    (if (`self.B_Targetting`) :!label _label
      (`self.Firing Phase` (`|GetArrayItem` (`self.Vent_Array`) (`self.I_Firing_Vent_Ref`)))
      (`self.Gun Barrel Flare`)
      (`KismetSystemLibrary.Delay` 0.6)
      (if (< (`self.I_Firing_Vent_Ref`) 2)
        (`/Engine/EditorBlueprintResources/StandardMacros.IncrementInt` (`self.I_Firing_Vent_Ref`)
          (:`  `
            (goto _label)))
        (else
          (set `self.I_Firing_Vent_Ref` 0)
          (set `self.B_Armed` false)
          (if (`self.B_Targetting`)
            (`self.Arming Phase`)))))
    (else
      (bind (_direction _loading) (`Timeline|Loading` :!via `PlayFromStart`)
        (:`Update`
          (bind _returnvalue (* _loading -7.0))
          (`SceneComponent.K2_SetRelativeLocation` (`self.SM_Small_Turret_Vent_1`) (`KismetMathLibrary.MakeVector` _returnvalue) false false)
          (`SceneComponent.K2_SetRelativeLocation` (`self.SM_Small_Turret_Vent_4`) (`KismetMathLibrary.MakeVector` _returnvalue) false false)
          (`SceneComponent.K2_SetRelativeLocation` (`self.SM_Small_Turret_Vent_5`) (`KismetMathLibrary.MakeVector` _returnvalue) false false))
        (:`Finished`
          (set `self.B_Armed` true)
          (goto _label))))))

(event `self.ReceiveBeginPlay`
  ;[1 0 0] Testing and Debugging
  (`KismetSystemLibrary.Delay` 5.0)
  (`self.Arming Phase` :!label _label_2)
  (`KismetSystemLibrary.Delay` 3.0)
  (`self.Firing Phase` (`|GetArrayItem` (`self.Vent_Array`) (`self.I_Firing_Vent_Ref`)) :!label _label_3)
  (`self.Gun Barrel Flare`)
  (`KismetSystemLibrary.Delay` 0.6)
  (if (< (`self.I_Firing_Vent_Ref`) 2)
    (`/Engine/EditorBlueprintResources/StandardMacros.IncrementInt` (`self.I_Firing_Vent_Ref`)
      (:`  `
        (goto _label_3)))
    (else
      (set `self.I_Firing_Vent_Ref` 0)
      (`KismetSystemLibrary.Delay` 5.0)
      (goto _label_2))))

(event `Firing Phase`
  (params (`Vent Component` :type "StaticMeshComponent Object Reference"))
  ;[1 1 1] Vent closing on shot
  (bind (_direction _loading) (`Timeline|Shooting` :!via `PlayFromStart`)
    (:`Update`
      (`SceneComponent.K2_SetRelativeLocation` `Vent Component` (`KismetMathLibrary.MakeVector` (* _loading -7.0)) false false))))

(event `self.ReceiveTick`
  (params (DeltaSeconds :type "Float (single-precision)"))
  (bind _sm_small_turret_top (`self.SM_Small_Turret_Top`))
  (bind _target_ref (`self.Target_Ref`))
  (bind _scan_box (`self.Scan_Box`))
  (bind (_returnvalue_roll _returnvalue_pitch _returnvalue_yaw) (`KismetMathLibrary.BreakRotator` (`SceneComponent.K2_GetComponentRotation` (`self.DefaultSceneRoot`))))
  (bind (_returnvalue_roll_2 _returnvalue_pitch_2 _returnvalue_yaw_2) (`KismetMathLibrary.BreakRotator` (`KismetMathLibrary.FindLookAtRotation` (`SceneComponent.K2_GetComponentLocation` _sm_small_turret_top) (`SceneComponent.K2_GetComponentLocation` (`Actor.RootComponent` _target_ref)))))
  (bind _returnvalue (+ (- _returnvalue_yaw_2 _returnvalue_yaw) -90.0))
  ;[1 1 1] Tracking Target and Widening the tracking beam with target
  (if (`self.B_Targetting`)
    (`SceneComponent.SetRelativeScale3D` _scan_box (2.0 8.0 1.0))
    (`/Engine/EditorBlueprintResources/StandardMacros.IsValid` _target_ref
      (:`Is Valid`
        (`SceneComponent.K2_SetRelativeRotation` _sm_small_turret_top (`KismetMathLibrary.MakeRotator` 0.0 0.0 _returnvalue) false false)
        (`KismetSystemLibrary.PrintString` (`KismetStringLibrary.Conv_DoubleToString` _returnvalue) true true (struct :`R` 0.671875 :`G` 0.593795 :`A` 1.0) 0.0)))
    (else
      (`SceneComponent.SetRelativeScale3D` _scan_box (0.5 8.0 1.0)))))

(event `self.Scan_Box.OnComponentBeginOverlap`
  (params (OverlappedComponent :type "PrimitiveComponent Object Reference") (OtherActor :type "Actor Object Reference") (OtherComp :type "PrimitiveComponent Object Reference") (OtherBodyIndex :type Integer) (bFromSweep :type Boolean) (SweepResult :type "HitResult Structure (by ref)"))
  (bind _returnvalue (`KismetSystemLibrary.GetDisplayName` OtherActor))
  ;[1 1 1] Acquire a target
  (if (or (`KismetStringLibrary.Contains` _returnvalue "NPC") (and (`KismetStringLibrary.Contains` _returnvalue "Player") (not (`KismetStringLibrary.Contains` (`KismetSystemLibrary.GetDisplayName` OtherComp) "Detection"))))
    (`/Engine/EditorBlueprintResources/StandardMacros.IsValid` OtherActor
      (:`Is Valid`
        (set `self.Target_Ref` OtherActor)
        (set `self.B_Targetting` true)
        (`self.Arming Phase`)
        (`MaterialInstanceDynamic.SetVectorParameterValue` (`self.DMI_Barrel`) "None" (struct :`R` 1.0 :`B` 0.020907 :`A` 1.0))))))

(event `self.Scan_Box.OnComponentEndOverlap`
  (params (OverlappedComponent :type "PrimitiveComponent Object Reference") (OtherActor :type "Actor Object Reference") (OtherComp :type "PrimitiveComponent Object Reference") (OtherBodyIndex :type Integer))
  (bind _returnvalue (`KismetSystemLibrary.GetDisplayName` OtherComp))
  (bind _returnvalue_2 (`KismetStringLibrary.Contains` _returnvalue "collision"))
  (bind _returnvalue_3 (not (`KismetStringLibrary.Contains` _returnvalue "BP_Projectile_Turret")))
  ;[1 1 1] Stop Tracking
  (if (and _returnvalue_2 _returnvalue_3)
    (`KismetSystemLibrary.PrintString` (`KismetStringLibrary.Concat_StrStr` "BP_Tur_Place no longer tracking because = " _returnvalue "  left overlap " (`KismetStringLibrary.Conv_BoolToString` _returnvalue_2) " belonged to " "" (`KismetStringLibrary.Conv_BoolToString` _returnvalue_3)))
    (set `self.B_Targetting` false)))

(event `Gun Barrel Flare`
  (bind _pointlight (`self.PointLight`))
  (bind _dmi_barrel (`self.DMI_Barrel`))
  (bind (_returnvalue_location _returnvalue_rotation) (`KismetMathLibrary.BreakTransform` (`SceneComponent.K2_GetComponentToWorld` (`self.Sphere`))))
  ;[1 1 1] Gun Barrel Flare (and Projectile Shooting
  (bind (_direction _flash_amount) (`Timeline|Muzzle Flash` :!via `PlayFromStart`)
    (:`Update`
      (`MaterialInstanceDynamic.SetScalarParameterValue` (`self.DMI_Barrel`) "Emissive_Power" (+ (* _flash_amount 500.0) 50.0))
      (`MaterialInstanceDynamic.SetVectorParameterValue` _dmi_barrel "Emissive_Colour" (struct :`R` 1.0 :`A` 1.0))
      (`LightComponent.SetLightColor` _pointlight (struct :`R` 1.0 :`A` 1.0) true))
    (:`Finished`
      (`|SpawnActorFromClass` "/Game/Blueprints/Player/Weapons/BP_Projectile_Turret.BP_Projectile_Turret_C" (`KismetMathLibrary.MakeTransform` _returnvalue_location _returnvalue_rotation) "AlwaysSpawn" "OverrideRootScale" self (struct) null)
      (`MaterialInstanceDynamic.SetVectorParameterValue` _dmi_barrel "Emissive_Colour" (struct :`R` 0.938686 :`G` 0.130136 :`A` 1.0))
      (`LightComponent.SetLightColor` _pointlight (struct :`R` 0.9375 :`G` 0.130717 :`A` 1.0) true))))

(event `self.ReceiveAnyDamage`
  (params (Damage :type "Float (single-precision)") (DamageType :type "DamageType Object Reference") (InstigatedBy :type "Controller Object Reference") (DamageCauser :type "Actor Object Reference"))
  (set `self.F_Health` (- (`self.F_Health`) Damage))
  (if (<= (`self.F_Health`) 0.0)
    (`/Engine/EditorBlueprintResources/StandardMacros.DoOnce` false
      (:`Completed`
        (`|SpawnActorFromClass` "/Game/Blueprints/Player/Weapons/BP_Grenade_Explosion.BP_Grenade_Explosion_C" (`SceneComponent.K2_GetComponentToWorld` (`self.DefaultSceneRoot`)) "Undefined" "OverrideRootScale" null null)
        (`KismetSystemLibrary.Delay` 0.05)
        (`self.K2_DestroyActor`)))))

(fn `UserConstructionScript`
  (bind _sm_small_turret_barrel (`self.SM_Small_Turret_Barrel`))
  (bind _returnvalue (`PrimitiveComponent.CreateDynamicMaterialInstance` _sm_small_turret_barrel 0 "/Game/Materials/Turrets/MI_Turret_Top.MI_Turret_Top" "None"))
  (bind _output_get (set `self.DMI_Barrel` _returnvalue))
  (`PrimitiveComponent.SetMaterial` _sm_small_turret_barrel 0 _output_get)
  (set `self.Vent_Array` (`|MakeArray` (`self.SM_Small_Turret_Vent_1`) (`self.SM_Small_Turret_Vent_4`) (`self.SM_Small_Turret_Vent_5`))))