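; BP_TestingThreatArea is a test trigger actor for the threat system.
; When the player's Cylinder component overlaps its Cube, matched by display-name substrings, it asks the game mode to raise area 0's threat level by a fixed step.
; It then reads back the current and active threat levels from the game mode and prints both as a debug string.
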(event `self.Cube.OnComponentBeginOverlap`
  (params (OverlappedComponent :type "PrimitiveComponent Object Reference") (OtherActor :type "Actor Object Reference") (OtherComp :type "PrimitiveComponent Object Reference") (OtherBodyIndex :type Integer) (bFromSweep :type Boolean) (SweepResult :type "HitResult Structure (by ref)"))
  (bind _returnvalue (`GameplayStatics.GetGameMode`))
  ;[1 1 1] Update Threat level on impact
  (if (and (`KismetStringLibrary.Contains` (`KismetSystemLibrary.GetDisplayName` OtherActor) "BP_Main_Player") (`KismetStringLibrary.Contains` (`KismetSystemLibrary.GetDisplayName` OtherComp) "Cylinder"))
    (message `/Game/Blueprints/Interfaces/BPI_Threat.Update_Current_Threat_Level` _returnvalue false 0.1 0)
    (bind (_success _current_threat_level) (message `/Game/Blueprints/Interfaces/BPI_Threat.Get_Current_Threat_Level` _returnvalue false 0))
    (bind (_success_2 _active_threat_level) (message `/Game/Blueprints/Interfaces/BPI_Threat.Get_Active_Threat_Level` _returnvalue false 0))
    (`KismetSystemLibrary.PrintString` (`KismetStringLibrary.Concat_StrStr` "Current Threat Level  " (`KismetStringLibrary.Conv_DoubleToString` _current_threat_level) " - - " "Active Threat Level" "  " (`KismetStringLibrary.Conv_IntToString` _active_threat_level)) true true (struct :`R` 1.0 :`G` 0.060741 :`A` 1.0))))

(fn `UserConstructionScript`)