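; Item Blueprint that shows an outline on the item until it is picked up.
; On BeginPlay it gives SMOutline the static mesh from STRUCTItem and applies the M_Outline_Inst material to slot 0 of SMItem, so two mesh components form the look.
; When the parent's PickedUp succeeds, it destroys SMOutline and then SMItem, passing the parent's result back.
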(event `self.ReceiveBeginPlay`
  (`parent.ReceiveBeginPlay`)
  (`StaticMeshComponent.SetStaticMesh` (`self.SM_Outline`) (`.Static_Mesh_35_5047C0634C5C3351DC70938DD0C66F27` (break `/Game/Blueprints/Gameplay/STRUCT_Item` (`self.STRUCT_Item`))))
  (`PrimitiveComponent.SetMaterial` (`self.SM_Item`) 0 "/Game/Materials/Outline/M_Outline_Inst.M_Outline_Inst"))

(fn `Picked_Up`
  (returns (Success :type Boolean))
  (bind _sm_outline (`self.SM_Outline`))
  (bind _sm_item (`self.SM_Item`))
  (bind _success (`parent.Picked_Up`))
  (if _success
    (`/Engine/EditorBlueprintResources/StandardMacros.IsValid` _sm_outline
      (:`Is Valid`
        (`ActorComponent.K2_DestroyComponent` _sm_outline)
        (`/Engine/EditorBlueprintResources/StandardMacros.IsValid` _sm_item
          (:`Is Valid`
            (`ActorComponent.K2_DestroyComponent` _sm_item))))))
  (return _success))

(fn `UserConstructionScript`
  (`parent.UserConstructionScript`))