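; BP_Item is a world loot item that the player picks up or steals by teleporting it to the ship.
; Construction fills its struct and mesh from DT_Items by item ID.
; Batteries feed player energy and healing or grenades enter player inventory, while other items teleport with a dissolve material if energy, ship capacity and absence of registered emitters allow.
; Interface-style functions, many stubbed, supply interaction text and custom-depth stencil highlighting.
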(event `self.ReceiveTick`
  (params (DeltaSeconds :type "Float (single-precision)")))

(event `self.ReceiveBeginPlay`)

(event `Teleport and Destroy`
  (bind _returnvalue (`PrimitiveComponent.CreateDynamicMaterialInstance` (`self.SM_Item`) 0 "/Game/Materialize/Materials/MI_Teleport.MI_Teleport" "None"))
  (set `self.DIM_Ref` _returnvalue)
  (`MaterialInstanceDynamic.SetTextureParameterValue` (`self.DIM_Ref`) "Texture_BC" (`self.Texture_BC_Ref`))
  (bind (_direction _vanishing_percent) (`Timeline|Teleporting Appearance`)
    (:`Update`
      (`MaterialInstanceDynamic.SetScalarParameterValue` (`self.DIM_Ref`) "Materialize Amount" (- 1.0 _vanishing_percent)))
    (:`Finished`
      (`ActorComponent.K2_DestroyComponent` (`self.SM_Item`)))))

(fn `Add_To_Player_Inventory`
  (params (Added_Item :type "/Game/Blueprints/Gameplay/STRUCT_Player_Item Structure"))
  (returns (Success :type Boolean))
  (return false))

(fn `Add_To_Ship_Inventory`
  (params (STRUCT_New_Item :type "/Game/Blueprints/Gameplay/STRUCT_Ship_Item Structure"))
  (returns (Success :type Boolean))
  (return false))

(fn `Adjust_Energy`
  (params (Adjustment_To_Make :type Integer))
  (returns (Adjustment_Made :type "Float (double-precision)"))
  (bind _struct_item (`self.STRUCT_Item`))
  (bind (_item_id _catagory _name _size _transport_cost _sale_value _healing_value _energy_value _static_mesh _thumbnail_image _spawn_residential _spawn_storage _spawn_medical _spawn_military _threat_value) (break `/Game/Blueprints/Gameplay/STRUCT_Item` _struct_item))
  ;[1 1 1] Adjusting the new value and passing out the amount taken
  (`|VariableSetRef` _struct_item (make `/Game/Blueprints/Gameplay/STRUCT_Item` _item_id _catagory _name _size _transport_cost _sale_value _healing_value (- _energy_value Adjustment_To_Make) _static_mesh _thumbnail_image _spawn_residential _spawn_storage _spawn_medical _spawn_military _threat_value))
  (return (`KismetMathLibrary.Conv_IntToDouble` Adjustment_To_Make)))

(fn `Check_Keycard`
  (params (I_Card_Ref :type Integer))
  (returns (B_Keycard_Owned :type Boolean))
  (return false))

(fn `Doors`
  (params (B_Locked :type Boolean) (B_Paid :type Boolean) (F_Cost :type "Float (double-precision)"))
  (returns (Success :type Boolean))
  (return false))

(fn `Energy_Drain`
  (returns (Success :type Boolean) (Energy_Taken :type "Float (double-precision)") (S_Dialogue :type String))
  (bind (_item_id _catagory _name _size _transport_cost _sale_value _healing_value _energy_value _static_mesh _thumbnail_image _spawn_residential _spawn_storage _spawn_medical _spawn_military _threat_value _max_adjustment) (break `/Game/Blueprints/Gameplay/STRUCT_Item` (`self.STRUCT_Item`)))
  ;[1 1 1] Removing the Maximum Adjustment amount from the item, or whatever the current value is if lower than Maximum
  (if (>= _energy_value _max_adjustment)
    (bind _adjustment_made (`self.Adjust_Energy` _max_adjustment))
    (return false _adjustment_made "")
    (else
      (bind _adjustment_made_2 (`self.Adjust_Energy` _energy_value))
      (return false _adjustment_made_2 ""))))

(fn `Hack_Successful`
  (params (Successful :type Boolean) (Cost_Paid :type Boolean) (I_Door_Cost :type Integer))
  (returns (Success :type Boolean) (Paid :type Boolean))
  (return false false))

(fn `Initiate_Hack`
  (returns (Success :type Boolean) (Unlock_Cost :type Integer) (Open_Cost :type Integer) (Door_Difficulty :type Integer))
  (return false 0 0 0))

(fn `Move_Elevator`
  (params (Elevator_Choice :type Integer) (Start_Point_In :type "Float (double-precision)"))
  (returns (Success :type Boolean) (Start_Point :type "Float (double-precision)") (Chosen_Floor :type "Float (double-precision)"))
  (return false 0.0 0.0))

(fn `Open_Elevator_Panel`
  (returns (Success :type Boolean))
  (return false))

(fn `Pick_Up_Sorting`
  (returns (Success :type Boolean) (S_Type :type String) (S_Name :type String))
  (bind (_item_id _catagory _name) (break `/Game/Blueprints/Gameplay/STRUCT_Item` (`self.STRUCT_Item`)))
  (return false _catagory _name))

(fn `Picked_Up`
  (returns (Success :type Boolean))
  (bind _sm_item (`self.SM_Item`))
  (bind (_item_id _catagory _name _size _transport_cost _sale_value _healing_value _energy_value _static_mesh _thumbnail_image) (break `/Game/Blueprints/Gameplay/STRUCT_Item` (`self.STRUCT_Item`)))
  (switch `string` (`.Catagory_2_81FBF19B4F0CEFEE33CCF98C17C3D7AD` (break `/Game/Blueprints/Gameplay/STRUCT_Item` (`self.STRUCT_Item`)))
    (:`Default`
      _)
    (:`Battery`
      _)
    (:`Healing`
      _)
    (:`Grenade`
      _))
  ;[1 1 1] Remove from World, Mark as Stolen
  (set `self.B_Is_Stolen` true)
  (`/Engine/EditorBlueprintResources/StandardMacros.IsValid` _sm_item
    (:`Is Valid`
      (`ActorComponent.K2_DestroyComponent` _sm_item))
    (:`Is Not Valid`
      _))
  (switch `string` (`.Catagory_2_81FBF19B4F0CEFEE33CCF98C17C3D7AD` (break `/Game/Blueprints/Gameplay/STRUCT_Item` (`self.STRUCT_Item`)))
    (:`Battery`
      ;[1 1 1] Consuming a Battery
      (bind (_success _energy_taken) (`/Game/Blueprints/Interfaces/BPI_Energy.Energy_Drain` self))
      (bind _success_2 (message `/Game/Blueprints/Interfaces/BPI_Energy.Player_Energy_Adjustment` (`GameplayStatics.GetPlayerCharacter` 0) _energy_taken))
      (return _success_2))
    (:`Healing`
      _)
    (:`Grenade`
      _))
  ;[1 1 1] Give the Item to the Player
  (bind _success_3 (message `/Game/Blueprints/Interfaces/BPI_Data_Transfer.Add_To_Player_Inventory` (`GameplayStatics.GetPlayerCharacter` 0) (make `/Game/Blueprints/Gameplay/STRUCT_Player_Item` _item_id _catagory _name _size _transport_cost _healing_value _energy_value _thumbnail_image)))
  (return _success_3))

(fn `Player_Energy_Adjustment`
  (params (Adjustment :type "Float (double-precision)"))
  (returns (Success :type Boolean))
  (return false))

(fn `Player_Health_Adjustment`
  (params (Adjustment :type Integer))
  (returns (Success :type Boolean))
  (return false))

(fn `Player_Inventory_Update`
  (params (Input :type Boolean))
  (returns (Success :type Boolean) (Player_Inventory :type "Array of /Game/Blueprints/Gameplay/STRUCT_Player_Item Structure"))
  (return false))

(fn `Player_Invisible?`
  (returns (Success :type Boolean) (Invisible :type Boolean))
  (return false false))

(fn `Ship_Energy_Update`
  (params (Input :type Boolean))
  (returns (Success :type Boolean) (Current_Energy :type Integer) (Max_Energy :type Integer))
  (return false 0 0))

(fn `Ship_Inventory_Update`
  (params (Input :type Boolean))
  (returns (Success :type Boolean) (Ship_Inventory :type "Array of /Game/Blueprints/Gameplay/STRUCT_Ship_Inventory Structure") (Current_Inventory_Count :type "Float (double-precision)") (Max_Inventory_Count :type "Float (double-precision)") (Inventory_Value :type Integer))
  (return false _ 0.0 0.0 0))

(fn `Starting_Information`
  (params (STRUCT_Weapon :type "/Game/Blueprints/Gameplay/STRUCT_Weapons Structure") (B_Check :type Boolean) (I_First :type Integer) (I_Second :type Integer) (I_Third :type Integer) (I_Fourth :type Integer) (`Actor Ref` :type "Actor Object Reference"))
  (returns (Success :type Boolean) (B_Second :type Boolean) (S_String :type String) (S_String_Second :type String) (I_Ref_Int :type Integer) (I_Ref_Int_Second :type Integer))
  (`/Engine/EditorBlueprintResources/StandardMacros.IsValid` `Actor Ref`
    (:`Is Valid`
      (`KismetArrayLibrary.Array_AddUnique` (`self.B_Emitters_In_Range_Array`) `Actor Ref`)
      (return false false "" "" 0 0))))

(fn `Teleport_Cost`
  (params (Input :type Boolean) (F_Current_Energy :type "Float (double-precision)"))
  (returns (Success :type Boolean) (`I_Teleport Cost` :type Integer))
  (bind (_item_id _catagory _name _size _transport_cost) (break `/Game/Blueprints/Gameplay/STRUCT_Item` (`self.STRUCT_Item`)))
  (bind (_item_id_2 _catagory_2 _name_2 _size_2 _transport_cost_2 _sale_value _healing_value _energy_value _static_mesh _thumbnail_image) (break `/Game/Blueprints/Gameplay/STRUCT_Item` (`self.STRUCT_Item`)))
  ;[1 1 1] Check if Item is Stolen, If Enough Current Energy, If enough capacity remaining
  (bind (_success _ship_inventory _current_inventory_count _max_inventory_count) (message `/Game/Blueprints/Interfaces/BPI_Data_Transfer.Ship_Inventory_Update` (`GameplayStatics.GetGameMode`) false))
  (if (and (not (`self.B_Is_Stolen`)) (>= F_Current_Energy (`KismetMathLibrary.Conv_IntToDouble` _transport_cost)) (>= (- _max_inventory_count _current_inventory_count) _size) (not (> (`KismetArrayLibrary.Array_Length` (`self.B_Emitters_In_Range_Array`)) 0)) (not (or (`KismetStringLibrary.EqualEqual_StrStr` _catagory "Healing") (`KismetStringLibrary.EqualEqual_StrStr` _catagory "Battery") (`KismetStringLibrary.EqualEqual_StrStr` _catagory "Grenade"))))
    ;[1 1 1] Changes to the Item - Add particle Effect Here
    (set `self.B_Is_Stolen` true)
    (`self.Teleport and Destroy`)
    ;[1 1 1] Sending the Item Data to the Ship
    (message `/Game/Blueprints/Interfaces/BPI_Data_Transfer.Add_To_Ship_Inventory` (`GameplayStatics.GetGameMode`) (make `/Game/Blueprints/Gameplay/STRUCT_Ship_Item` _item_id_2 _catagory_2 _name_2 _size_2 _transport_cost_2 _healing_value _energy_value _static_mesh _thumbnail_image _sale_value))
    ;[1 1 1] Report the Cost to the Player for Deduction
    (return false (`.Transport_Cost_10_6FDFECC54960BEFC71D2358791FBC9C7` (break `/Game/Blueprints/Gameplay/STRUCT_Item` (`self.STRUCT_Item`))))
    (else
      (return true 0))))

(fn `Update_Display`
  (params (B_Update :type Boolean))
  (returns (Success :type Boolean) (B_Second_Hint :type Boolean) (S_Interact_Type :type String) (S_Second_Interact :type String) (I_Image_Hint_Ref :type Integer))
  (bind (_item_id _catagory _name _size _transport_cost _sale_value _healing_value _energy_value) (break `/Game/Blueprints/Gameplay/STRUCT_Item` (`self.STRUCT_Item`)))
  (switch `string` _catagory
    (:`Default`
      (`KismetSystemLibrary.PrintString` "BP_Item fucking with interact display")
      (return true false "" "" 0))
    (:`Consumable`
      (`KismetSystemLibrary.PrintString` "BP_Item messing with interact display")
      (return true false "" "" 0))
    (:`Healing`
      (return true false "Add Health Pack" "" 0))
    (:`Object`
      (return true false (`KismetStringLibrary.Concat_StrStr` "Steal (" (`KismetStringLibrary.Conv_IntToString` _transport_cost) " Energy Cost)") "" 0))
    (:`Grenade`
      (return true false (`KismetStringLibrary.Concat_StrStr` "Gain " _name " Grenade") "" 0))
    (:`Battery`
      (return true false (`KismetStringLibrary.Concat_StrStr` "Gain " (`KismetStringLibrary.Conv_IntToString` _energy_value) " Energy") "" 0))))

(fn `Update_Highlight`
  (params (Highlight :type Boolean) (Pulse_Exclusive :type Boolean))
  (returns (Success :type Boolean) (F_Percent :type "Float (double-precision)"))
  (bind _sm_item (`self.SM_Item`))
  (`/Engine/EditorBlueprintResources/StandardMacros.IsValid` _sm_item
    (:`Is Valid`
      (`self.Update_Widget` Highlight)
      (`PrimitiveComponent.SetRenderCustomDepth` _sm_item Highlight)
      (if (not (> (`KismetArrayLibrary.Array_Length` (`self.B_Emitters_In_Range_Array`)) 0))
        (switch `string` (`.Catagory_2_81FBF19B4F0CEFEE33CCF98C17C3D7AD` (break `/Game/Blueprints/Gameplay/STRUCT_Item` (`self.STRUCT_Item`)))
          (:`Default`
            (`PrimitiveComponent.SetCustomDepthStencilValue` _sm_item 251))
          (:`Weapon`
            (`PrimitiveComponent.SetCustomDepthStencilValue` _sm_item 252 :!label _label))
          (:`Consumable`
            (goto _label)))
        (else
          (`PrimitiveComponent.SetCustomDepthStencilValue` _sm_item 254)))
      (return false 0.0))))

(fn `Update_Item`
  (if (!= (`self.I_Item_ID`) 0)
    (bind _returnvalue (`|GetDataTableRow` "/Game/Blueprints/Gameplay/DT_Items.DT_Items" (`KismetStringLibrary.Conv_StringToName` (`KismetStringLibrary.Conv_IntToString` (`self.I_Item_ID`))))
      (:`then`
        (set `self.STRUCT_Item` _returnvalue)
        (`StaticMeshComponent.SetStaticMesh` (`self.SM_Item`) (`.Static_Mesh_35_5047C0634C5C3351DC70938DD0C66F27` (break `/Game/Blueprints/Gameplay/STRUCT_Item` (`self.STRUCT_Item`))))
        (`PrimitiveComponent.SetCustomDepthStencilValue` (`self.SM_Item`) 255)))
    (else
      (`StaticMeshComponent.SetStaticMesh` (`self.SM_Item`) (`.Static_Mesh_35_5047C0634C5C3351DC70938DD0C66F27` (break `/Game/Blueprints/Gameplay/STRUCT_Item` (`self.STRUCT_Item`))))
      (`PrimitiveComponent.SetCustomDepthStencilValue` (`self.SM_Item`) 255))))

(fn `Update_Keycard`
  (params (I_Card_Ref :type Integer))
  (returns (Success :type Boolean))
  (return false))

(fn `Update_Widget`
  (params (B_Update :type Boolean))
  (bind _widget_hint (`self.Widget_Hint`))
  (`SceneComponent.SetVisibility` _widget_hint false false)
  (message `/Game/Blueprints/Interfaces/BPI_Data_Transfer.Update_Display` (`WidgetComponent.GetUserWidgetObject` _widget_hint) B_Update))

(fn `UserConstructionScript`
  (bind (_item_id _catagory _name _size _transport_cost _sale_value _healing_value _energy_value _static_mesh _thumbnail_image _spawn_residential _spawn_storage _spawn_medical _spawn_military _threat_value _max_adjustment _base_texture) (break `/Game/Blueprints/Gameplay/STRUCT_Item` (`self.STRUCT_Item`)))
  (if (!= (`self.I_Item_ID`) 0)
    (bind _returnvalue (`|GetDataTableRow` "/Game/Blueprints/Gameplay/DT_Items.DT_Items" (`KismetStringLibrary.Conv_StringToName` (`KismetStringLibrary.Conv_IntToString` (`self.I_Item_ID`))))
      (:`then`
        (set `self.STRUCT_Item` _returnvalue)
        (`StaticMeshComponent.SetStaticMesh` (`self.SM_Item`) _static_mesh)
        (set `self.Texture_BC_Ref` _base_texture)
        (`PrimitiveComponent.SetCustomDepthStencilValue` (`self.SM_Item`) 38)))
    (else
      (`StaticMeshComponent.SetStaticMesh` (`self.SM_Item`) (`.Static_Mesh_35_5047C0634C5C3351DC70938DD0C66F27` (break `/Game/Blueprints/Gameplay/STRUCT_Item` (`self.STRUCT_Item`))))
      (`PrimitiveComponent.SetCustomDepthStencilValue` (`self.SM_Item`) 255))))

(fn `Within_Ship_Radius`
  (params (B_Within :type Boolean))
  (returns (B_Success :type Boolean))
  (return false))