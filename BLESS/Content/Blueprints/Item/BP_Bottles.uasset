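; BP_Bottles is an item Blueprint that randomizes which of its child actors, presumably bottles, remain in the level when play begins.
; On BeginPlay it loops over a hand-built array of fourteen Child Actor components and destroys each on an independent random boolean, leaving about half on average.
; The construction script is empty, so the random thinning happens only at runtime.
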(event `self.ReceiveBeginPlay`
  (for _array_element (`|MakeArray` (`self.ChildActor1`) (`self.ChildActor3`) (`self.ChildActor4`) (`self.ChildActor5`) (`self.ChildActor6`) (`self.ChildActor7`) (`self.ChildActor8`) (`self.ChildActor`) (`self.ChildActor9`) (`self.ChildActor10`) (`self.ChildActor11`) (`self.ChildActor12`) (`self.ChildActor13`) (`self.ChildActor14`))
    (if (`KismetMathLibrary.RandomBool`)
      (`ActorComponent.K2_DestroyComponent` _array_element))))

(fn `UserConstructionScript`)