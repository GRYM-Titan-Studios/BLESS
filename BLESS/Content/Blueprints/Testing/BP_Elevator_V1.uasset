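; Test elevator actor that moves a Platform between five floors, chosen through a UI_Elevator widget.
; Per-floor overlap volumes record the start floor and timeline time.
; MoveElevator plays or reverses one timeline, clamping its output to stop at the chosen floor, offsetting the platform's relative X by up to 2000 units.
; The inventory, ship and highlight functions are empty stubs.
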(event `self.ReceiveBeginPlay`
  (set `self.F_Elevator_Start_Pos` (.x (`SceneComponent.RelativeLocation` (`self.Platform`)))))

(event `Move Up`
  (bind _platform (`self.Platform`))
  ;[1 1 1] Timeline to Control the Elevator Movement
  (bind (_direction _complete_movement) (`Timeline|Elevator Movement` :`NewTime` (`self.F_Elevator_Start_Time`) :!label _label)
    (:`Update`
      (`SceneComponent.K2_SetRelativeLocation` _platform (`KismetMathLibrary.MakeVector` (+ (`self.F_Elevator_Start_Pos`) (* (`KismetMathLibrary.FClamp` _complete_movement (`self.F_Min_Clamp`) (`self.F_Max_Clamp`)) 2000.0)) (.y (`SceneComponent.RelativeLocation` _platform)) (.z (`SceneComponent.RelativeLocation` _platform))) false false))))

(event `Move Down`
  ;[1 1 1] Timeline to Control the Elevator Movement
  (goto _label :!via `Reverse`))

(event `Set_Timeline`
  ;[1 1 1] Timeline to Control the Elevator Movement
  (goto _label :!via `SetNewTime`))

(event `self.Collision_Ground.OnComponentBeginOverlap`
  (params (OverlappedComponent :type "PrimitiveComponent Object Reference") (OtherActor :type "Actor Object Reference") (OtherComp :type "PrimitiveComponent Object Reference") (OtherBodyIndex :type Integer) (bFromSweep :type Boolean) (SweepResult :type "HitResult Structure (by ref)"))
  ;[1 1 1] Sets the Elevator Start Position Based on where they enter the elevator
  (set `self.F_Elevator_Start_Time` 0.0)
  (`self.Set_Timeline`)
  (set `self.I_Start_Floor` 0))

(event `self.Collision_1ST.OnComponentBeginOverlap`
  (params (OverlappedComponent :type "PrimitiveComponent Object Reference") (OtherActor :type "Actor Object Reference") (OtherComp :type "PrimitiveComponent Object Reference") (OtherBodyIndex :type Integer) (bFromSweep :type Boolean) (SweepResult :type "HitResult Structure (by ref)"))
  ;[1 1 1] Sets the Elevator Start Position Based on where they enter the elevator
  (set `self.F_Elevator_Start_Time` 1.25)
  (`self.Set_Timeline`)
  (set `self.I_Start_Floor` 1))

(event `self.Collision_2ND.OnComponentBeginOverlap`
  (params (OverlappedComponent :type "PrimitiveComponent Object Reference") (OtherActor :type "Actor Object Reference") (OtherComp :type "PrimitiveComponent Object Reference") (OtherBodyIndex :type Integer) (bFromSweep :type Boolean) (SweepResult :type "HitResult Structure (by ref)"))
  ;[1 1 1] Sets the Elevator Start Position Based on where they enter the elevator
  (set `self.F_Elevator_Start_Time` 2.5)
  (`self.Set_Timeline`)
  (set `self.I_Start_Floor` 2))

(event `self.Collision_3RD.OnComponentBeginOverlap`
  (params (OverlappedComponent :type "PrimitiveComponent Object Reference") (OtherActor :type "Actor Object Reference") (OtherComp :type "PrimitiveComponent Object Reference") (OtherBodyIndex :type Integer) (bFromSweep :type Boolean) (SweepResult :type "HitResult Structure (by ref)"))
  ;[1 1 1] Sets the Elevator Start Position Based on where they enter the elevator
  (set `self.F_Elevator_Start_Time` 3.75)
  (`self.Set_Timeline`)
  (set `self.I_Start_Floor` 3))

(event `self.Collision_4TH.OnComponentBeginOverlap`
  (params (OverlappedComponent :type "PrimitiveComponent Object Reference") (OtherActor :type "Actor Object Reference") (OtherComp :type "PrimitiveComponent Object Reference") (OtherBodyIndex :type Integer) (bFromSweep :type Boolean) (SweepResult :type "HitResult Structure (by ref)"))
  ;[1 1 1] Sets the Elevator Start Position Based on where they enter the elevator
  (set `self.F_Elevator_Start_Time` 5.0)
  (`self.Set_Timeline`)
  (set `self.I_Start_Floor` 4))

(fn `Add_To_Player_Inventory`
  (params (Added_Item :type "/Game/Blueprints/Gameplay/STRUCT_Player_Item Structure"))
  (returns (Success :type Boolean))
  (return false))

(fn `Add_To_Ship_Inventory`
  (params (STRUCT_New_Item :type "/Game/Blueprints/Gameplay/STRUCT_Ship_Item Structure"))
  (returns (Success :type Boolean))
  (return false))

(fn `Move_Elevator`
  (params (Elevator_Choice :type Integer) (Start_Point_In :type "Float (double-precision)"))
  (returns (Success :type Boolean) (Start_Point :type "Float (double-precision)") (Chosen_Floor :type "Float (double-precision)"))
  (bind _returnvalue (select `int` Elevator_Choice :`0` 0.0 :`1` 0.25 :`2` 0.5 :`3` 0.75 :`4` 1.0 :!type "Float (single-precision)"))
  ;[1 1 1] Takes the Information from the Widget and Moves the Elevator to the chosen floor
  (set `self.F_Min_Clamp` 0.0)
  (set `self.F_Max_Clamp` 1.0)
  (if (> Elevator_Choice (`self.I_Start_Floor`))
    (set `self.F_Max_Clamp` _returnvalue)
    (`self.Move Up`)
    (else
      (set `self.F_Min_Clamp` _returnvalue)
      (`self.Move Down`)))
  (set `self.I_Start_Floor` Elevator_Choice)
  (return false 0.0 0.0))

(fn `Open_Elevator_Panel`
  (returns (Success :type Boolean))
  ;[1 1 1] On Player activation, open a Elevator Widget
  (bind _returnvalue (`|CreateWidget` "/Game/UI/Testing/UI_Elevator.UI_Elevator_C" (`GameplayStatics.GetPlayerController` 0) 0 (`self.I_Start_Floor`)))
  (`UserWidget.AddToViewport` _returnvalue 0)
  (return false))

(fn `Player_Inventory_Update`
  (params (Input :type Boolean))
  (returns (Success :type Boolean) (Player_Inventory :type "Array of /Game/Blueprints/Gameplay/STRUCT_Player_Item Structure"))
  (return false))

(fn `Ship_Energy_Update`
  (params (Input :type Boolean))
  (returns (Success :type Boolean) (Current_Energy :type Integer) (Max_Energy :type Integer))
  (return false 0 0))

(fn `Ship_Inventory_Update`
  (params (Input :type Boolean))
  (returns (Success :type Boolean) (Ship_Inventory :type "Array of /Game/Blueprints/Gameplay/STRUCT_Ship_Inventory Structure") (Current_Inventory_Count :type "Float (double-precision)") (Max_Inventory_Count :type "Float (double-precision)"))
  (return false _ 0.0 0.0))

(fn `Starting_Information`
  (params (STRUCT_Weapon :type "/Game/Blueprints/Gameplay/STRUCT_Weapons Structure"))
  (returns (Success :type Boolean))
  (return false))

(fn `Update_Highlight`
  (params (Highlight :type Boolean))
  (returns (Success :type Boolean))
  (return false))

(fn `UserConstructionScript`)

(fn `Within_Ship_Radius`
  (params (B_Within :type Boolean))
  (returns (B_Success :type Boolean))
  (return false))