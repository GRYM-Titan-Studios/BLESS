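; GI_BLESS, apparently the game instance, holds arrays of station and notoriety level data.
; Write_Station_Data reads every row of the referenced stations data table, appends each found row to the station array, then logs completion without showing it on screen.
; Write_Noteriety_Level_Data appends each notoriety level struct passed to it to a separate array.
; Neither event clears its array, so repeated calls accumulate entries.
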(event `Write_Station_Data`
  ;[1 1 1] Populate Sation Array From Data Table
  (bind _outrownames (`DataTableFunctionLibrary.GetDataTableRowNames` (`self.DT_Stations_Ref`)))
  (for _array_element _outrownames
    (bind _returnvalue (`|GetDataTableRow` (`self.DT_Stations_Ref`) _array_element)
      (:`then`
        (`KismetArrayLibrary.Array_Add` (`self.STRUCT_Stations_Array`) _returnvalue))))
  (`KismetSystemLibrary.PrintString` "Station Data Array Populated" false true (struct :`G` 0.66 :`B` 1.0 :`A` 1.0) 5.0))

(event `Write_Noteriety_Level_Data`
  (params (STRUCT_NoterietyLevel :type "/Game/Blueprints/Space_Station/STRUCT_NoterietyLevels Structure"))
  ;[1 1 1] Write Noteriety Data
  (`KismetArrayLibrary.Array_Add` (`self.STRUCT_Noteriety_Levels_Array`) STRUCT_NoterietyLevel))