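; BP_Wall_Terminal is a space station wall terminal that can be hacked to set the locked and paid state of linked doors.
; On BeginPlay it passes its door references to its screen widget after a short delay.
; Interface calls toggle the outline highlight, enlarge the screen and run a timeline that slides and tilts out the keyboard.
; Hack success updates every door, shrinks the screen, retracts the keyboard and disables further display and highlight.
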(event `Open Keyboard`
  (bind (_direction _ejection _tilt) (`Timeline|Opening` :!label _label)
    (:`Update`
      (`SceneComponent.K2_SetRelativeLocation` (`self.SM_KeyboardRedone`) (`KismetMathLibrary.MakeVector` 0.0 (- (* _ejection 25.0) 12.0) 100.0) false false)
      (`SceneComponent.K2_SetRelativeRotation` (`self.SM_KeyboardRedone`) (`KismetMathLibrary.MakeRotator` (* _tilt 20.0)) false false))))

(event `Close Keyboard`
  (goto _label :!via `Reverse`))

(event `self.ReceiveBeginPlay`
  (`KismetSystemLibrary.Delay` 0.2)
  (message `/Game/Blueprints/Interfaces/BPI_Hacking.Terminal_Information` (`WidgetComponent.GetUserWidgetObject` (`self.Widget`)) (`self.Door_Ref`)))

(fn `Add_To_Player_Inventory`
  (params (Added_Item :type "/Game/Blueprints/Gameplay/STRUCT_Player_Item Structure"))
  (returns (Success :type Boolean))
  (return false))

(fn `Add_To_Ship_Inventory`
  (params (STRUCT_New_Item :type "/Game/Blueprints/Gameplay/STRUCT_Ship_Item Structure"))
  (returns (Success :type Boolean))
  (return false))

(fn `Aiming_At_Hack_Panel`
  (returns (Success :type Boolean))
  (return true))

(fn `Check_Keycard`
  (params (I_Card_Ref :type Integer))
  (returns (B_Keycard_Owned :type Boolean))
  (return false))

(fn `Hack_Success`
  (params (B_Locked :type Boolean) (B_Paid :type Boolean))
  (returns (B_Is_Locked :type Boolean) (B_Is_Paid :type Boolean))
  (bind _widget (`self.Widget`))
  (for _array_element (`self.Door_Ref`)
    (message `/Game/Blueprints/Interfaces/BPI_Energy.Doors` _array_element B_Locked B_Paid 0.0))
  (`SceneComponent.SetRelativeScale3D` _widget (0.02 0.02 0.02))
  (`SceneComponent.K2_SetRelativeLocation` _widget (0.0 30.0 128.0) false true)
  (`self.Close Keyboard`)
  (set `self.B_Completed` true)
  (`PrimitiveComponent.SetRenderCustomDepth` (`self.SM_Terminal`) false)
  (return false false))

(fn `Move_Elevator`
  (params (Elevator_Choice :type Integer) (Start_Point_In :type "Float (double-precision)"))
  (returns (Success :type Boolean) (Start_Point :type "Float (double-precision)") (Chosen_Floor :type "Float (double-precision)"))
  (return false 0.0 0.0))

(fn `Open_Elevator_Panel`
  (returns (Success :type Boolean))
  (return false))

(fn `Player_Inventory_Update`
  (params (Input :type Boolean))
  (returns (Success :type Boolean) (Player_Inventory :type "Array of /Game/Blueprints/Gameplay/STRUCT_Player_Item Structure"))
  (return false))

(fn `Player_Invisible?`
  (returns (Success :type Boolean) (Invisible :type Boolean))
  (return false false))

(fn `Ship_Energy_Update`
  (params (Input :type Boolean))
  (returns (Success :type Boolean) (Current_Energy :type Integer) (Max_Energy :type Integer))
  (return false 0 0))

(fn `Ship_Inventory_Update`
  (params (Input :type Boolean))
  (returns (Success :type Boolean) (Ship_Inventory :type "Array of /Game/Blueprints/Gameplay/STRUCT_Ship_Inventory Structure") (Current_Inventory_Count :type "Float (double-precision)") (Max_Inventory_Count :type "Float (double-precision)") (Inventory_Value :type Integer))
  (return false _ 0.0 0.0 0))

(fn `Starting_Information`
  (params (STRUCT_Weapon :type "/Game/Blueprints/Gameplay/STRUCT_Weapons Structure") (B_Check :type Boolean) (I_First :type Integer) (I_Second :type Integer) (I_Third :type Integer) (I_Fourth :type Integer) (`Actor Ref` :type "Actor Object Reference"))
  (returns (Success :type Boolean) (B_Second :type Boolean) (S_String :type String) (S_String_Second :type String) (I_Ref_Int :type Integer) (I_Ref_Int_Second :type Integer))
  (return false false "" "" 0 0))

(fn `Swap_Button_Recieving`
  (returns (B_Success :type Boolean))
  (return false))

(fn `Swap_Button_Sending`
  (params (I_Row_Goal :type Integer) (I_Column_Goal :type Integer) (Widget_Ref :type "Widget Object Reference"))
  (returns (B_Success :type Boolean) (I_Row_Position :type Integer) (I_Column_Position :type Integer))
  (return false 0 0))

(fn `Terminal_Information`
  (params (Object_Array :type "Array of Object Object Reference (by ref)"))
  (returns (Success :type Boolean) (I_Open_Cost :type Integer) (I_Unlock_Cost :type Integer) (I_Num_Tiles :type Integer) (I_Num_Columns :type Integer) (I_Puzzle_Choice :type Integer))
  (return false 0 0 0 0 0))

(fn `Update_Display`
  (params (B_Update :type Boolean))
  (returns (Success :type Boolean) (B_Second_Hint :type Boolean) (S_Interact_Type :type String) (S_Second_Interact :type String) (I_Image_Hint_Ref :type Integer))
  (bind _widget (`self.Widget`))
  (if (not (`self.B_Completed`))
    (`SceneComponent.SetRelativeScale3D` _widget (select `bool` B_Update :`false` (0.02 0.02 0.02) :`true` (0.05 0.05 0.05) :!type "Vector Structure"))
    (`SceneComponent.K2_SetRelativeLocation` _widget (select `bool` B_Update :`false` (0.0 30.0 128.0) :`true` (0.0 40.0 138.0) :!type "Vector Structure") false true)
    (if B_Update
      (`self.Open Keyboard`)
      (else
        (`self.Close Keyboard`)))
    (return true true "Scope to Enable Interact" "Shoot to Interact" 1)))

(fn `Update_Highlight`
  (params (Highlight :type Boolean) (Pulse_Exclusive :type Boolean))
  (returns (Success :type Boolean) (F_Percent :type "Float (double-precision)"))
  (`PrimitiveComponent.SetRenderCustomDepth` (`self.SM_Terminal`) (and Highlight (not (`self.B_Completed`))))
  (return false 0.0))

(fn `Update_Keycard`
  (params (I_Card_Ref :type Integer))
  (returns (Success :type Boolean))
  (return false))

(fn `UserConstructionScript`)

(fn `Within_Ship_Radius`
  (params (B_Within :type Boolean))
  (returns (B_Success :type Boolean))
  (return false))