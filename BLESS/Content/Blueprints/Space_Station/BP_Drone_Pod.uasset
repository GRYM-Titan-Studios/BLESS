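; Drone pod for the space station that spawns suicide drone AI once the alert level reaches its activation threshold.
; Activation creates a drone immediately and starts a looping spawn timer; SpawnSDrone also spawns on demand.
; Each drone receives a pod reference, then deploy-point information once the timeline-driven sliding doors are open.
; SetPosition supplies random points in the configurable CoverArea bounds, with a DoN Navigation navigable-world check.
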(event `self.ReceiveBeginPlay`)

(event `Open_Door`
  (bind (_direction _newtrack_0) (`Timeline|Open_Doors` :!via `PlayFromStart`)
    (:`Update`
      (`SceneComponent.K2_SetRelativeLocation` (`self.SM_Drone_Pod_polySurface106`) (`KismetMathLibrary.MakeVector` 0.0 0.0 (* _newtrack_0 110.0)) false false)
      (`SceneComponent.K2_SetRelativeLocation` (`self.SM_Drone_Pod_polySurface108`) (`KismetMathLibrary.MakeVector` 0.0 0.0 (* _newtrack_0 -110.0)) false false))
    (:`Finished`
      (bind _output_get (set `self.B_Door_Open` (== _newtrack_0 1.0)))
      (if _output_get
        (`self.Deploy`)))))

(event `Start_Spawns`
  (`KismetSystemLibrary.K2_SetTimerDelegate` (delegate `Create_Drone`) 30.0 true))

(event `Deploy`
  (message `/Game/Blueprints/Interfaces/BPI_Data_Transfer.Starting_Information` (stale `Create_Drone` _returnvalue) (struct) true 0 0 0 0 null (`SceneComponent.K2_GetComponentLocation` (`self.Deploy_Point`)) :!label _label))

(event `Create_Drone`
  (bind _returnvalue (`AIBlueprintHelperLibrary.SpawnAIFromClass` "/Game/Blueprints/AI/BP_NPC_Drone_Suicide.BP_NPC_Drone_Suicide_C" "/Game/Blueprints/AI/BT_SDrone.BT_SDrone" (`SceneComponent.K2_GetComponentLocation` (`self.Spawn_Point`))))
  (message `/Game/Blueprints/AI/BPI_NPC.Set_Pod` _returnvalue self)
  (if (`self.B_Door_Open`)
    (goto _label)
    (else
      (`self.Open_Door`))))

(fn `Alert_Level_1`
  (params (Activate :type Boolean) (Alert_Level :type Integer))
  (returns (Success :type Boolean))
  (bind _activated_level (`self.Activated_Level`))
  (bind _returnvalue (>= Alert_Level _activated_level))
  (`KismetSystemLibrary.PrintString` (`KismetStringLibrary.Concat_StrStr` (`KismetStringLibrary.Conv_IntToString` Alert_Level) " >= " (`KismetStringLibrary.Conv_IntToString` _activated_level) " = " (`KismetStringLibrary.Conv_BoolToString` _returnvalue)))
  (if _returnvalue
    (if (not (`self.B_Activated`))
      (set `self.B_Activated` true)
      (`self.Create_Drone`)
      (`self.Start_Spawns`)
      (return false))))

(fn `Call_Assist`
  (returns (B_Success :type Boolean))
  (return false))

(fn `Drone_Sensed_Player`
  (params (B_Sensed :type Boolean))
  (returns (Success :type Boolean))
  (return false))

(fn `Enter_Charging_Pod`
  (params (B_Occupied :type Boolean))
  (returns (B_Success :type Boolean))
  (return false))

(fn `Get_Gun_Ref`
  (returns (Gun_Ref :type "ChildActorComponent Object Reference"))
  (return null))

(fn `Get_NPC_Movement_Ref`
  (params (B_Input :type Boolean))
  (returns (B_Success :type Boolean) (NPC_Character_Movement :type "CharacterMovementComponent Object Reference"))
  (return false null))

(fn `Get_PatrolPath`
  (params (B_Input :type Boolean))
  (returns (B_Success :type Boolean) (V_PathPoints :type "Array of Vector Structure") (BP_PatrolPath :type "/Game/Blueprints/AI/BP_PatrolPath Object Reference") (Start_Index :type Integer))
  (return false _ null 0))

(fn `Gun_Ready`
  (params (`Gun_UP?` :type Boolean))
  (returns (Anim_Finished :type Boolean))
  (return false))

(fn `Kill_Drone`
  (params (Input :type Boolean))
  (returns (Success :type Boolean))
  (return false))

(fn `NPC_Apply_Damage`
  (params (Damage_Applied :type "Float (double-precision)"))
  (returns (Success :type Boolean) (Destroyed_Actor :type Boolean))
  (return false false))

(fn `NPC_Start_Shooting`
  (params (`B_Can_Shoot?` :type Boolean))
  (returns (Success :type Boolean) (B_Can_Fire :type Boolean))
  (return false false))

(fn `Set_Pod`
  (params (Pod_Ref :type "Actor Object Reference"))
  (returns (Success :type Boolean) (Send_Pod_Ref :type "Actor Object Reference"))
  (return false null))

(fn `Set_Position`
  (returns (Success :type Boolean) (V_Location :type "Vector Structure"))
  (bind (_origin _boxextent) (`KismetSystemLibrary.GetComponentBounds` (`self.Cover_Area`)))
  (bind _returnvalue (`KismetMathLibrary.RandomPointInBoundingBox` _origin _boxextent))
  (return (`DonNavigationManager.IsLocationWithinNavigableWorld` (`DonNavigationHelper.DonNavigationManager`) _returnvalue) _returnvalue))

(fn `Spawn_SDrone`
  (returns (Success :type Boolean))
  (`self.Create_Drone`)
  (return false))

(fn `Update Color`
  (params (B_Alerted :type Boolean))
  (returns (Success :type Boolean))
  (return false))

(fn `UserConstructionScript`
  (`SceneComponent.K2_SetRelativeLocation` (`self.Cover_Area`) (`self.V_Roaming_Area`) false false)
  (`SphereComponent.SetSphereRadius` (`self.Cover_Area`) (`self.F_Area_Scale`) true))