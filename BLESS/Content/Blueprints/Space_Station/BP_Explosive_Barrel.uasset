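; Explosive barrel actor that blows up the first time it takes damage of any kind.
; AnyDamage prints a debug message, then a one-shot flag guards spawning BP_Standard_BlowUP slightly above the mesh's transform and destroying the barrel.
; The component hit event is empty, and an older spawn-and-destroy chain is left unconnected, so impacts alone do not detonate it.
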(event `self.ReceiveAnyDamage`
  (params (Damage :type "Float (single-precision)") (DamageType :type "DamageType Object Reference") (InstigatedBy :type "Controller Object Reference") (DamageCauser :type "Actor Object Reference"))
  (bind _returnvalue (`SceneComponent.K2_GetComponentToWorld` (`self.StaticMeshComponent`)))
  (`KismetSystemLibrary.PrintString` (`KismetStringLibrary.Concat_StrStr` (`KismetSystemLibrary.GetDisplayName` self) " - Dead - "))
  (if (not (`self.B_Exploded`))
    (set `self.B_Exploded` true)
    (`|SpawnActorFromClass` "/Game/Blueprints/Player/Weapons/BP_Standard_BlowUP.BP_Standard_BlowUP_C" (`KismetMathLibrary.MakeTransform` (`KismetMathLibrary.MakeVector` (.x (.location _returnvalue)) (.y (.location _returnvalue)) (+ (.z (.location _returnvalue)) 10.0)) (.rotation _returnvalue) (.scale _returnvalue)) "Undefined" "OverrideRootScale" null null)
    (`self.K2_DestroyActor`)))

(event `self.StaticMeshComponent.OnComponentHit`
  (params (HitComponent :type "PrimitiveComponent Object Reference") (OtherActor :type "Actor Object Reference") (OtherComp :type "PrimitiveComponent Object Reference") (NormalImpulse :type "Vector Structure") (Hit :type "HitResult Structure (by ref)")))

(fn `UserConstructionScript`)