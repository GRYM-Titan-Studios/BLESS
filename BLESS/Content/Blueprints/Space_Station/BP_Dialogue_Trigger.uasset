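; Space Station dialogue trigger volume with a configurable dialogue reference and a box extent set in the construction script.
; Entering sends the reference to the overlapping actor through MoveElevatorMessage, reusing its ElevatorChoice parameter, and leaving sends zero.
; On exit, reference 3 also calls StartingInformationMessage on the game mode.
; After a short delay, the trigger destroys itself if the exiting actor's name contains "Player".
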(event `self.Box.OnComponentEndOverlap`
  (params (OverlappedComponent :type "PrimitiveComponent Object Reference") (OtherActor :type "Actor Object Reference") (OtherComp :type "PrimitiveComponent Object Reference") (OtherBodyIndex :type Integer))
  (message `/Game/Blueprints/Interfaces/BPI_Data_Transfer.Move_Elevator` OtherActor 0 0.0)
  (if (== (`self.I_Dialogue_Ref`) 3)
    (message `/Game/Blueprints/Interfaces/BPI_Data_Transfer.Starting_Information` (`GameplayStatics.GetGameMode`) (struct) false 0 0 0 0 null))
  (`KismetSystemLibrary.Delay` 0.2)
  (if (`KismetStringLibrary.Contains` (`KismetStringLibrary.Conv_ObjectToString` OtherActor) "Player")
    (`self.K2_DestroyActor`)))

(event `self.Box.OnComponentBeginOverlap`
  (params (OverlappedComponent :type "PrimitiveComponent Object Reference") (OtherActor :type "Actor Object Reference") (OtherComp :type "PrimitiveComponent Object Reference") (OtherBodyIndex :type Integer) (bFromSweep :type Boolean) (SweepResult :type "HitResult Structure (by ref)"))
  (message `/Game/Blueprints/Interfaces/BPI_Data_Transfer.Move_Elevator` OtherActor (`self.I_Dialogue_Ref`) 0.0))

(fn `UserConstructionScript`
  (`BoxComponent.SetBoxExtent` (`self.Box`) (`self.V_Box_Size`) true))