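; Space station security turret that opens its shutters and drops out shortly after BeginPlay, then sweeps a full or limited arc.
; Each tick, two stacked box traces query hit actors through a keycard check against the turret's zone.
; A detection makes it track the player, allowing for crouch, and fire twin projectiles after a lock-on delay.
; The construction script sizes scan fields from arrow components; death at zero health only prints.
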(event `Deploy`
  ;[1 1 1] Deploy the Turret when activated
  (bind (_direction _shutters _base_drop) (`Timeline|Deployment` :!label _label)
    (:`Update`
      (bind _returnvalue (* _shutters 60.0))
      (`SceneComponent.K2_SetRelativeRotation` (`self.SM_Turret_Door_5`) (`KismetMathLibrary.MakeRotator` 0.0 0.0 _returnvalue) false false)
      (`SceneComponent.K2_SetRelativeRotation` (`self.SM_Turret_Door_4`) (`KismetMathLibrary.MakeRotator` 0.0 0.0 _returnvalue) false false)
      (`SceneComponent.K2_SetRelativeRotation` (`self.SM_Turret_Door_3`) (`KismetMathLibrary.MakeRotator` 0.0 0.0 _returnvalue) false false)
      (`SceneComponent.K2_SetRelativeRotation` (`self.SM_Turret_Door_2`) (`KismetMathLibrary.MakeRotator` 0.0 0.0 _returnvalue) false false)
      (`SceneComponent.K2_SetRelativeRotation` (`self.SM_Turret_Door_1`) (`KismetMathLibrary.MakeRotator` 0.0 0.0 _returnvalue) false false)
      (`SceneComponent.K2_SetRelativeLocation` (`self.SM_Turret_Base`) (`KismetMathLibrary.MakeVector` -150.0 -150.0 (- 85.0 (* _base_drop 80.0))) false false))
    (:`Finished`
      (set `self.B_Deployed` true))))

(event `self.ReceiveBeginPlay`
  (`KismetSystemLibrary.Delay` 1.0)
  (goto _label))

(event `self.ReceiveTick`
  (params (DeltaSeconds :type "Float (single-precision)"))
  (bind (_v_start _v_end _v_upper_field_size _r_head_rotation) (`self.Box_Trace_Input`))
  (bind (_v_start_2 _v_end_2 _v_upper_field_size_2 _r_head_rotation_2) (`self.Box_Trace_Input`))
  (bind _cylinder (`self.Cylinder`))
  (bind (_v_start_adjusted _v_end_adjusted _v_lower_field_size) (`self.Lower_Box_Trace_Input` _v_start _v_end))
  ;[1 1 1] Rotation While Seeking
  (if (`self.B_Deployed`)
    (bind _outhit (`KismetSystemLibrary.BoxTraceSingle` :`Start` _v_start_2 :`End` _v_end_2 :`HalfSize` _v_upper_field_size_2 :`Orientation` _r_head_rotation_2 :`TraceChannel` "TraceTypeQuery1" :`DrawDebugType` (select `bool` (`self.B_Setup`) :`true` "ForOneFrame" :!type "EDrawDebugTrace Enum")))
    (bind _b_keycard_owned (message `/Game/Blueprints/Interfaces/BPI_Data_Transfer.Check_Keycard` (`.HitActor` (`GameplayStatics.BreakHitResult` _outhit)) (`self.I_Turret_Zone_Ref`)))
    (bind _outhit_2 (`KismetSystemLibrary.BoxTraceSingle` :`Start` _v_start_adjusted :`End` _v_end_adjusted :`HalfSize` _v_lower_field_size :`Orientation` _r_head_rotation :`TraceChannel` "TraceTypeQuery1" :`DrawDebugType` (select `bool` (`self.B_Setup`) :`true` "ForOneFrame" :!type "EDrawDebugTrace Enum")))
    (bind _b_keycard_owned_2 (message `/Game/Blueprints/Interfaces/BPI_Data_Transfer.Check_Keycard` (`.HitActor` (`GameplayStatics.BreakHitResult` _outhit_2)) (`self.I_Turret_Zone_Ref`)))
    (set `self.B_Target_Acquired` (or _b_keycard_owned_2 _b_keycard_owned))
    (if (`self.B_Target_Acquired`)
      (`SceneComponent.K2_SetRelativeRotation` (`self.SM_Turret_Head`) (`KismetMathLibrary.MakeRotator` 0.0 0.0 (`self.Look_At_Player_Yaw`)) false false)
      (`SceneComponent.K2_SetRelativeRotation` (`self.SM_Turret_Barrel`) (`KismetMathLibrary.MakeRotator` 0.0 (`self.Look_At_Player_Pitch`)) false false)
      (`self.Shooting`)
      (`SceneComponent.SetVisibility` _cylinder true false)
      (else
        (`self.Resume_Rotation`)
        (`SceneComponent.K2_SetRelativeRotation` (`self.SM_Turret_Barrel`) (`KismetMathLibrary.MakeRotator` 0.0) false false)
        (if (`self.B_Full_Rotation`)
          (`self.Full_Rotation`)
          (else
            (`self.Restricted Rotation`)))
        (`SceneComponent.SetVisibility` _cylinder false false)))))

(event `Restricted Rotation`
  (bind _f_rotation (`self.F_Rotation`))
  (bind _f_rotation_2 (`self.F_Rotation`))
  (bind _f_speed (`self.F_Speed`))
  ;[1 1 1] Rotation While Seeking
  ;;[1 1 1] Fixed Field Rotation
  (`SceneComponent.K2_SetRelativeRotation` (`self.SM_Turret_Head`) (`KismetMathLibrary.MakeRotator` 0.0 0.0 (`self.F_Rotation`)) false false)
  (if (`self.B_Clockwise`)
    (set `self.F_Rotation` (+ _f_rotation_2 _f_speed))
    (if (>= _f_rotation_2 (`self.F_Maximum_Rotation`))
      (set `self.B_Clockwise` false))
    (else
      (set `self.F_Rotation` (- _f_rotation _f_speed))
      (if (<= _f_rotation (`self.F_Minimum_Rotation`))
        (set `self.B_Clockwise` true)))))

(event `Full_Rotation`
  (bind _f_rotation (`self.F_Rotation`))
  ;[1 1 1] Rotation While Seeking
  ;;[1 1 1] Default 360 Rotation
  (`SceneComponent.K2_SetRelativeRotation` (`self.SM_Turret_Head`) (`KismetMathLibrary.MakeRotator` 0.0 0.0 _f_rotation) false false)
  (set `self.F_Rotation` (+ _f_rotation (`self.F_Speed`)))
  (if (== _f_rotation 360.0)
    (set `self.F_Rotation` 0.0)))

(event `Shooting`
  ;[1 1 1] Shooting Projectiles
  (if (`self.B_Locked_On`)
    (set `self.B_Locking_On` false)
    (if (`self.B_Can_Fire`)
      (set `self.B_Can_Fire` false)
      (for _index (range 2)
        (`|SpawnActorFromClass` "/Game/Blueprints/Player/Weapons/BP_Projectile_Turret.BP_Projectile_Turret_C" (select `int` _index :`0` (`SceneComponent.K2_GetComponentToWorld` (`self.Left_Barrel_Ref`)) :`1` (`SceneComponent.K2_GetComponentToWorld` (`self.Right_Barrel_Ref`))) "Undefined" "OverrideRootScale" null (struct) null))
      (`KismetSystemLibrary.Delay` 1.0)
      (set `self.B_Can_Fire` true))
    (elif (not (`self.B_Locking_On`))
      (set `self.B_Locking_On` true)
      (`KismetSystemLibrary.Delay` (`self.F_Locking_On_Duration`))
      (set `self.B_Locked_On` true))))

(event `self.ReceiveAnyDamage`
  (params (Damage :type "Float (single-precision)") (DamageType :type "DamageType Object Reference") (InstigatedBy :type "Controller Object Reference") (DamageCauser :type "Actor Object Reference"))
  (`KismetSystemLibrary.PrintString` (`KismetStringLibrary.Conv_DoubleToString` Damage))
  (bind _output_get (set `self.F_Turret_Health` (- (`self.F_Turret_Health`) Damage)))
  (if (<= _output_get 0.0)
    (`KismetSystemLibrary.PrintString` "Turret go boom")))

(fn `Box_Trace_Input`
  (returns (V_Start :type "Vector Structure") (V_End :type "Vector Structure") (V_Upper_Field_Size :type "Vector Structure") (R_Head_Rotation :type "Rotator Structure"))
  (return (`KismetMathLibrary.MakeVector` (+ (.x (`SceneComponent.K2_GetComponentLocation` (`self.SM_Turret_Base`))) 10.0) (.y (`SceneComponent.K2_GetComponentLocation` (`self.SM_Turret_Base`))) (- (.z (`SceneComponent.K2_GetComponentLocation` (`self.SM_Turret_Base`))) (`self.F_Upper_Field_Offset`))) (`SceneComponent.K2_GetComponentLocation` (`self.Distance_Arrow`)) (`self.V_Upper_Field_Size`) (`SceneComponent.RelativeRotation` (`self.SM_Turret_Head`))))

(fn `Look_At_Player_Pitch`
  (returns (Player_Pitch :type "Float (double-precision)"))
  (bind (_returnvalue_roll _returnvalue_pitch) (`KismetMathLibrary.BreakRotator` (`KismetMathLibrary.FindLookAtRotation` (`SceneComponent.K2_GetComponentLocation` (`self.SM_Turret_Barrel`)) (`KismetMathLibrary.MakeVector` (.x (`self.Player_Location`)) (.y (`self.Player_Location`)) (+ (.z (`self.Player_Location`)) (select `bool` (`NavMovementComponent.IsCrouching` (`Character.CharacterMovement` (`GameplayStatics.GetPlayerCharacter` 0))) :`false` 96.0 :`true` 40.0 :!type "Float (single-precision)"))))))
  (return _returnvalue_pitch))

(fn `Look_At_Player_Yaw`
  (returns (`Return Value Z (Yaw)` :type "Float (double-precision)"))
  (bind (_returnvalue_roll _returnvalue_pitch _returnvalue_yaw) (`KismetMathLibrary.BreakRotator` (`SceneComponent.K2_GetComponentRotation` (`self.SharedRoot`))))
  (bind (_returnvalue_roll_2 _returnvalue_pitch_2 _returnvalue_yaw_2) (`KismetMathLibrary.BreakRotator` (`KismetMathLibrary.FindLookAtRotation` (`SceneComponent.K2_GetComponentLocation` (`self.SM_Turret_Head`)) (`self.Player_Location`))))
  (return (- _returnvalue_yaw_2 _returnvalue_yaw)))

(fn `Lower_Box_Trace_Input`
  (params (V_Start :type "Vector Structure") (V_End :type "Vector Structure"))
  (returns (V_Start_Adjusted :type "Vector Structure") (V_End_Adjusted :type "Vector Structure") (V_Lower_Field_Size :type "Vector Structure") (F_Debug :type "Float (double-precision)"))
  (return (`KismetMathLibrary.MakeVector` (+ (.x (`SceneComponent.K2_GetComponentLocation` (`self.SM_Turret_Base`))) 10.0) (.y (`SceneComponent.K2_GetComponentLocation` (`self.SM_Turret_Base`))) (- (.z (`SceneComponent.K2_GetComponentLocation` (`self.SM_Turret_Base`))) (`self.F_Lower_Field_Add_Offset`))) (`SceneComponent.K2_GetComponentLocation` (`self.Lower_Distance_Arrow`)) (`self.V_Lower_Field_Size`) 0.0))

(fn `Player_Location`
  (returns (ReturnValue :type "Vector Structure"))
  (return (`SceneComponent.K2_GetComponentLocation` (`Character.Mesh` (`GameplayStatics.GetPlayerCharacter` 0)))))

(fn `Resume_Rotation`
  (bind (_relativerotation_roll _relativerotation_pitch _relativerotation_yaw) (`KismetMathLibrary.BreakRotator` (`SceneComponent.RelativeRotation` (`self.SM_Turret_Head`))))
  (bind _returnvalue (- _relativerotation_yaw (`self.F_Rotation`)))
  (set `self.B_Locking_On` false)
  (set `self.B_Locked_On` false)
  (if (or (>= _returnvalue 3.0) (<= _returnvalue -3.0))
    (set `self.F_Rotation` _relativerotation_yaw)))

(fn `UserConstructionScript`
  (bind _f_top_arrow_height (`self.F_Top_Arrow_Height`))
  (bind _f_middle_arrow_height (`self.F_Middle_Arrow_Height`))
  (bind _z (.z (`SceneComponent.RelativeLocation` (`self.Top_Arrow`))))
  (bind _z_2 (.z (`SceneComponent.RelativeLocation` (`self.Middle_Arrow`))))
  (bind _returnvalue (/ (- _z _z_2) 2.0))
  (bind _returnvalue_2 (/ (- _z_2 (.z (`SceneComponent.RelativeLocation` (`self.Bottom_Arrow`)))) 2.0))
  (`SceneComponent.K2_SetRelativeLocation` (`self.SM_Turret_Base`) (`KismetMathLibrary.MakeVector` -150.0 -150.0 (select `bool` (`self.B_Setup`) :`false` 85.0 :`true` 5.0 :!type "Float (single-precision)")) false false)
  ;[1 1 1] Setting Arrow Postitions via Float Variables
  (`SceneComponent.K2_SetRelativeLocation` (`self.Top_Arrow`) (`KismetMathLibrary.MakeVector` 0.0 0.0 (- 0.0 (`self.F_Top_Arrow_Height`))) false false)
  (`SceneComponent.K2_SetRelativeLocation` (`self.Middle_Arrow`) (`KismetMathLibrary.MakeVector` 0.0 0.0 (- 0.0 (`self.F_Middle_Arrow_Height`))) false false)
  (`SceneComponent.K2_SetRelativeLocation` (`self.Bottom_Arrow`) (`KismetMathLibrary.MakeVector` 0.0 0.0 (- 0.0 (`self.F_Lower_Arrow_Height`))) false false)
  (`SceneComponent.K2_SetRelativeLocation` (`self.Distance_Arrow`) (`KismetMathLibrary.MakeVector` (`self.F_Turret_Range`) 16.666599 (- 0.0 (+ _f_top_arrow_height (/ (- (`self.F_Middle_Arrow_Height`) _f_top_arrow_height) 2.0)))) false false)
  (`SceneComponent.K2_SetRelativeLocation` (`self.Lower_Distance_Arrow`) (`KismetMathLibrary.MakeVector` (`self.F_Turret_Range`) 16.666599 (- 0.0 (+ _f_middle_arrow_height (/ (- (`self.F_Lower_Arrow_Height`) _f_middle_arrow_height) 2.0)))) false false)
  ;[1 1 1] Setting range Based on Distance Arrow
  (`SceneComponent.K2_SetRelativeLocation` (`self.Target_Point`) (`KismetMathLibrary.MakeVector` (.x (`SceneComponent.RelativeLocation` (`self.Distance_Arrow`))) 16.666599 (.z (`SceneComponent.RelativeLocation` (`self.Distance_Arrow`)))) false false)
  ;[1 1 1] Setting the Height of the Scan Boxes based on distance between arrows
  (set `self.V_Upper_Field_Size` (`KismetMathLibrary.MakeVector` 1.0 25.0 _returnvalue))
  (set `self.V_Lower_Field_Size` (`KismetMathLibrary.MakeVector` 1.0 25.0 _returnvalue_2))
  (set `self.F_Upper_Field_Offset` (- _returnvalue _z))
  (set `self.F_Lower_Field_Add_Offset` (- _returnvalue_2 _z_2)))