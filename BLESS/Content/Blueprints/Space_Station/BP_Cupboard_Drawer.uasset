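; BP_Cupboard_Drawer is a space station cupboard prop that randomizes its drawers for visual variety.
; The Construction Script rolls one-in-five chances to slide the large drawer open and to remove one small drawer.
; A remaining small drawer and the second small drawer always get random slide offsets.
; Randomization is unseeded, so the layout rerolls whenever construction reruns, and there is no runtime logic.
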(fn `UserConstructionScript`
  (bind _returnvalue (>= (`KismetMathLibrary.RandomFloatInRange` 0.0 5.0) 4.0))
  (set `self.B_Missing_TL` _returnvalue)
  (bind _output_get (set `self.B_Open_B` _returnvalue))
  (if _output_get
    (`SceneComponent.K2_SetRelativeLocation` (`self.SM_Cupboard_Draw_L`) (`KismetMathLibrary.MakeVector` 0.0 (`KismetMathLibrary.RandomFloatInRange` 0.0 45.0)) false false))
  (if (`self.B_Missing_TL`)
    (`ActorComponent.K2_DestroyComponent` (`self.SM_Cupboard_Draw_S`))
    (else
      (`SceneComponent.K2_SetRelativeLocation` (`self.SM_Cupboard_Draw_S`) (`KismetMathLibrary.MakeVector` 0.0 (`KismetMathLibrary.RandomFloatInRange` 0.0 45.0)) false false)))
  (`SceneComponent.K2_SetRelativeLocation` (`self.SM_Cupboard_Draw_S1`) (`KismetMathLibrary.MakeVector` 56.0 (`KismetMathLibrary.RandomFloatInRange` 0.0 45.0)) false false))