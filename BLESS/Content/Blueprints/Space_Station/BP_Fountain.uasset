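; BP_Fountain is an animated space station fountain prop that also displays alert levels.
; Tick slowly yaws the fountain TV mesh and pitches three turbine meshes, spaced 120 degrees apart in yaw, from an accumulating wheel rotation with fixed per-frame steps, independent of delta time.
; The Alert_Level_1 function forwards activation and level to three widget components' user widgets, while the other drone and NPC-related functions are empty stubs.
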(event `self.ReceiveTick`
  (params (DeltaSeconds :type "Float (single-precision)"))
  (`SceneComponent.K2_AddRelativeRotation` (`self.SM_ATR_Fountain_SM_Fountain_TV`) (struct :`Yaw` 0.5) false false)
  (`SceneComponent.K2_SetRelativeRotation` (`self.SM_ATR_Fountain__Turbine`) (`KismetMathLibrary.MakeRotator` 0.0 (`self.F_Wheel_Rotation`)) false false)
  (`SceneComponent.K2_SetRelativeRotation` (`self.SM_ATR_Fountain__Turbine1`) (`KismetMathLibrary.MakeRotator` 0.0 (`self.F_Wheel_Rotation`) 120.0) false false)
  (`SceneComponent.K2_SetRelativeRotation` (`self.SM_ATR_Fountain__Turbine2`) (`KismetMathLibrary.MakeRotator` 0.0 (`self.F_Wheel_Rotation`) 240.0) false false)
  (set `self.F_Wheel_Rotation` (+ (`self.F_Wheel_Rotation`) 0.2)))

(fn `Alert_Level_1`
  (params (Activate :type Boolean) (Alert_Level :type Integer))
  (returns (Success :type Boolean))
  (message `/Game/Blueprints/AI/BPI_NPC.Alert_Level_1` (`WidgetComponent.GetUserWidgetObject` (`self.Alert_Level_Widget`)) Activate Alert_Level)
  (message `/Game/Blueprints/AI/BPI_NPC.Alert_Level_1` (`WidgetComponent.GetUserWidgetObject` (`self.Alert_Level_Widget1`)) Activate Alert_Level)
  (bind _success (message `/Game/Blueprints/AI/BPI_NPC.Alert_Level_1` (`WidgetComponent.GetUserWidgetObject` (`self.Alert_Level_Widget2`)) Activate Alert_Level))
  (return _success))

(fn `Call_Assist`
  (returns (B_Success :type Boolean))
  (return false))

(fn `Drone_Sensed_Player`
  (params (B_Sensed :type Boolean))
  (returns (Success :type Boolean))
  (return false))

(fn `Enter_Charging_Pod`
  (params (B_Occupied :type Boolean))
  (returns (B_Success :type Boolean))
  (return false))

(fn `Get_Gun_Ref`
  (returns (Gun_Ref :type "ChildActorComponent Object Reference"))
  (return null))

(fn `Get_NPC_Movement_Ref`
  (params (B_Input :type Boolean))
  (returns (B_Success :type Boolean) (NPC_Character_Movement :type "CharacterMovementComponent Object Reference"))
  (return false null))

(fn `Get_PatrolPath`
  (params (B_Input :type Boolean))
  (returns (B_Success :type Boolean) (V_PathPoints :type "Array of Vector Structure") (BP_PatrolPath :type "/Game/Blueprints/AI/BP_PatrolPath Object Reference") (Start_Index :type Integer))
  (return false _ null 0))

(fn `Gun_Ready`
  (params (`Gun_UP?` :type Boolean))
  (returns (Anim_Finished :type Boolean))
  (return false))

(fn `Kill_Drone`
  (params (Input :type Boolean))
  (returns (Success :type Boolean))
  (return false))

(fn `NPC_Apply_Damage`
  (params (Damage_Applied :type "Float (double-precision)"))
  (returns (Success :type Boolean) (Destroyed_Actor :type Boolean))
  (return false false))

(fn `NPC_Start_Shooting`
  (params (`B_Can_Shoot?` :type Boolean))
  (returns (Success :type Boolean) (B_Can_Fire :type Boolean))
  (return false false))

(fn `Set_Pod`
  (params (Pod_Ref :type "Actor Object Reference"))
  (returns (Success :type Boolean) (Send_Pod_Ref :type "Actor Object Reference"))
  (return false null))

(fn `Set_Position`
  (returns (Success :type Boolean) (V_Location :type "Vector Structure"))
  (return false (0.0 0.0 0.0)))

(fn `Spawn_SDrone`
  (returns (Success :type Boolean))
  (return false))

(fn `Update Color`
  (params (B_Alerted :type Boolean))
  (returns (Success :type Boolean))
  (return false))

(fn `UserConstructionScript`)