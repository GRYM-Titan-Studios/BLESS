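; BP_Radio_Tower is a space station radio tower prop whose dish mesh spins continuously around its vertical axis.
; On BeginPlay, a looping timer calls Rotate at a fixed short interval instead of using Tick.
; Each call applies the stored yaw to the dishes' relative rotation, then increments it and wraps it back to zero after a full turn.
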(event `self.ReceiveBeginPlay`
  (`KismetSystemLibrary.K2_SetTimerDelegate` (delegate `Rotate`) 0.1 true))

(event `Rotate`
  (`SceneComponent.K2_SetRelativeRotation` (`self.SM_Tower_Dishes`) (`KismetMathLibrary.MakeRotator` 0.0 0.0 (`self.F_Rotation`)) false false)
  (set `self.F_Rotation` (+ (`self.F_Rotation`) 0.5))
  (if (>= (`self.F_Rotation`) 360.0)
    (set `self.F_Rotation` 0.0)))

(fn `UserConstructionScript`)