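; Interactable space station cupboard with two hinged doors that randomly keeps or removes its child actor on BeginPlay, with a one-in-four chance to keep it.
; The PickUpSorting interface call toggles the open state, playing or reversing a timeline that swings the doors in opposite yaw directions.
; UpdateDisplay and UpdateHighlight outline the meshes through custom depth, with UpdateDisplay also supplying an "Open" prompt.
; The remaining interface functions are stubs returning failure.
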(event `Open_Doors`
  (bind (_direction _open_percent) (`Timeline|Toggle Doors` :!label _label)
    (:`Update`
      (bind _returnvalue (* _open_percent 90.0))
      (`SceneComponent.K2_SetRelativeRotation` (`self.SM_Cupboard_Door_R`) (`KismetMathLibrary.MakeRotator` 0.0 0.0 _returnvalue) false false)
      (`SceneComponent.K2_SetRelativeRotation` (`self.SM_Cupboard_Door_L`) (`KismetMathLibrary.MakeRotator` 0.0 0.0 (* _returnvalue -1.0)) false false))))

(event `Close_Doors`
  (goto _label :!via `Reverse`))

(event `self.ReceiveBeginPlay`
  (if (not (== (`KismetMathLibrary.RandomIntegerInRange` 0 3) 3))
    (`ActorComponent.K2_DestroyComponent` (`self.ChildActor`))))

(fn `Add_To_Player_Inventory`
  (params (Added_Item :type "/Game/Blueprints/Gameplay/STRUCT_Player_Item Structure"))
  (returns (Success :type Boolean))
  (return false))

(fn `Add_To_Ship_Inventory`
  (params (STRUCT_New_Item :type "/Game/Blueprints/Gameplay/STRUCT_Ship_Item Structure"))
  (returns (Success :type Boolean))
  (return false))

(fn `Check_Keycard`
  (params (I_Card_Ref :type Integer))
  (returns (B_Keycard_Owned :type Boolean))
  (return false))

(fn `Doors`
  (params (B_Locked :type Boolean) (B_Paid :type Boolean) (F_Cost :type "Float (double-precision)"))
  (returns (Success :type Boolean))
  (return false))

(fn `Energy_Drain`
  (returns (Success :type Boolean) (Energy_Taken :type "Float (double-precision)") (S_Dialogue :type String))
  (return false 0.0 ""))

(fn `Hack_Successful`
  (params (Successful :type Boolean) (Cost_Paid :type Boolean) (I_Door_Cost :type Integer))
  (returns (Success :type Boolean) (Paid :type Boolean))
  (return false false))

(fn `Initiate_Hack`
  (returns (Success :type Boolean) (Unlock_Cost :type Integer) (Open_Cost :type Integer) (Door_Difficulty :type Integer))
  (return false 0 0 0))

(fn `Move_Elevator`
  (params (Elevator_Choice :type Integer) (Start_Point_In :type "Float (double-precision)"))
  (returns (Success :type Boolean) (Start_Point :type "Float (double-precision)") (Chosen_Floor :type "Float (double-precision)"))
  (return false 0.0 0.0))

(fn `Open_Elevator_Panel`
  (returns (Success :type Boolean))
  (return false))

(fn `Pick_Up_Sorting`
  (returns (Success :type Boolean) (S_Type :type String) (S_Name :type String))
  (if (`self.B_Open`)
    (`self.Close_Doors`)
    (set `self.B_Open` false)
    (else
      (`self.Open_Doors`)
      (set `self.B_Open` true)))
  (return false "" ""))

(fn `Picked_Up`
  (returns (Success :type Boolean))
  (return false))

(fn `Player_Energy_Adjustment`
  (params (Adjustment :type "Float (double-precision)"))
  (returns (Success :type Boolean))
  (return false))

(fn `Player_Health_Adjustment`
  (params (Adjustment :type Integer))
  (returns (Success :type Boolean))
  (return false))

(fn `Player_Inventory_Update`
  (params (Input :type Boolean))
  (returns (Success :type Boolean) (Player_Inventory :type "Array of /Game/Blueprints/Gameplay/STRUCT_Player_Item Structure"))
  (return false))

(fn `Player_Invisible?`
  (returns (Success :type Boolean) (Invisible :type Boolean))
  (return false false))

(fn `Ship_Energy_Update`
  (params (Input :type Boolean))
  (returns (Success :type Boolean) (Current_Energy :type Integer) (Max_Energy :type Integer))
  (return false 0 0))

(fn `Ship_Inventory_Update`
  (params (Input :type Boolean))
  (returns (Success :type Boolean) (Ship_Inventory :type "Array of /Game/Blueprints/Gameplay/STRUCT_Ship_Inventory Structure") (Current_Inventory_Count :type "Float (double-precision)") (Max_Inventory_Count :type "Float (double-precision)") (Inventory_Value :type Integer))
  (return false _ 0.0 0.0 0))

(fn `Starting_Information`
  (params (STRUCT_Weapon :type "/Game/Blueprints/Gameplay/STRUCT_Weapons Structure") (B_Check :type Boolean) (I_First :type Integer) (I_Second :type Integer) (I_Third :type Integer) (I_Fourth :type Integer) (`Actor Ref` :type "Actor Object Reference") (V_Location :type "Vector Structure"))
  (returns (Success :type Boolean) (B_Second :type Boolean) (S_String :type String) (S_String_Second :type String) (I_Ref_Int :type Integer) (I_Ref_Int_Second :type Integer))
  (return false false "" "" 0 0))

(fn `Teleport_Cost`
  (params (Input :type Boolean) (F_Current_Energy :type "Float (double-precision)"))
  (returns (Success :type Boolean) (`I_Teleport Cost` :type Integer))
  (return false 0))

(fn `Update_Color`
  (params (B_Update :type Boolean) (B_Stunned :type Boolean))
  (returns (Success :type Boolean))
  (return false))

(fn `Update_Display`
  (params (B_Update :type Boolean))
  (returns (Success :type Boolean) (B_Second_Hint :type Boolean) (S_Interact_Type :type String) (S_Second_Interact :type String) (I_Image_Hint_Ref :type Integer))
  (bind _sm_cupboard_door_r (`self.SM_Cupboard_Door_R`))
  (bind _sm_cupboard_door_l (`self.SM_Cupboard_Door_L`))
  (bind _sm_cupboard (`self.SM_Cupboard`))
  (`/Engine/EditorBlueprintResources/StandardMacros.IsValid` _sm_cupboard_door_r
    (:`Is Valid`
      (`PrimitiveComponent.SetRenderCustomDepth` _sm_cupboard_door_r B_Update)
      (`/Engine/EditorBlueprintResources/StandardMacros.IsValid` _sm_cupboard_door_l
        (:`Is Valid`
          (`PrimitiveComponent.SetRenderCustomDepth` _sm_cupboard_door_l B_Update)
          (`/Engine/EditorBlueprintResources/StandardMacros.IsValid` _sm_cupboard
            (:`Is Valid`
              (`PrimitiveComponent.SetRenderCustomDepth` _sm_cupboard B_Update)
              (return B_Update false "Open" "" 0))))))))

(fn `Update_Highlight`
  (params (Highlight :type Boolean) (Pulse_Exclusive :type Boolean))
  (returns (Success :type Boolean) (F_Percent :type "Float (double-precision)"))
  (bind _sm_cupboard_door_r (`self.SM_Cupboard_Door_R`))
  (bind _sm_cupboard_door_l (`self.SM_Cupboard_Door_L`))
  (bind _sm_cupboard (`self.SM_Cupboard`))
  (`/Engine/EditorBlueprintResources/StandardMacros.IsValid` _sm_cupboard_door_r
    (:`Is Valid`
      (`PrimitiveComponent.SetRenderCustomDepth` _sm_cupboard_door_r Highlight)
      (`/Engine/EditorBlueprintResources/StandardMacros.IsValid` _sm_cupboard_door_l
        (:`Is Valid`
          (`PrimitiveComponent.SetRenderCustomDepth` _sm_cupboard_door_l Highlight)
          (`/Engine/EditorBlueprintResources/StandardMacros.IsValid` _sm_cupboard
            (:`Is Valid`
              (`PrimitiveComponent.SetRenderCustomDepth` _sm_cupboard Highlight)
              (return Highlight 0.0))))))))

(fn `Update_Keycard`
  (params (I_Card_Ref :type Integer))
  (returns (Success :type Boolean))
  (return false))

(fn `UserConstructionScript`)

(fn `Within_Ship_Radius`
  (params (B_Within :type Boolean))
  (returns (B_Success :type Boolean))
  (return false))