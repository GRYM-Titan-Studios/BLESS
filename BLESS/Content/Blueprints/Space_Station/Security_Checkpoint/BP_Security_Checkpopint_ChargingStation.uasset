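; Security checkpoint charging station whose two hinged doors open on entry and close behind the occupant.
; Overlapping the entry collision plays a timeline that swings both doors outward in opposite yaw directions, with no actor filtering.
; Overlapping the charging point marks the station occupied and reverses the timeline, as does the CloseDoors event.
; An occupancy-checking message to the entering actor is left unconnected, and the NPC-related functions are stubs returning failure.
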(event `self.Entry_Collision.OnComponentBeginOverlap`
  (params (OverlappedComponent :type "PrimitiveComponent Object Reference") (OtherActor :type "Actor Object Reference") (OtherComp :type "PrimitiveComponent Object Reference") (OtherBodyIndex :type Integer) (bFromSweep :type Boolean) (SweepResult :type "HitResult Structure (by ref)"))
  (bind (_direction _door_movement) (`Timeline|Open_Doors` :!label _label)
    (:`Update`
      (`SceneComponent.K2_SetRelativeRotation` (`self.SM_Security_Charging_Door_Right`) (`KismetMathLibrary.MakeRotator` 0.0 0.0 (`KismetMathLibrary.Lerp` 0.0 60.0 _door_movement)) false false)
      (`SceneComponent.K2_SetRelativeRotation` (`self.SM_Security_Charging_Door_Left`) (`KismetMathLibrary.MakeRotator` 0.0 0.0 (`KismetMathLibrary.Lerp` 0.0 -60.0 _door_movement)) false false))))

(event `Close Doors`
  (goto _label :!via `Reverse`))

(event `self.Charging_Point.OnComponentBeginOverlap`
  (params (OverlappedComponent :type "PrimitiveComponent Object Reference") (OtherActor :type "Actor Object Reference") (OtherComp :type "PrimitiveComponent Object Reference") (OtherBodyIndex :type Integer) (bFromSweep :type Boolean) (SweepResult :type "HitResult Structure (by ref)"))
  (set `self.B_Occupied` true)
  (goto _label :!via `Reverse`))

(fn `Enter_Charging_Pod`
  (params (B_Occupied :type Boolean))
  (returns (B_Success :type Boolean))
  (return false))

(fn `Get_NPC_Movement_Ref`
  (params (B_Input :type Boolean))
  (returns (B_Success :type Boolean) (NPC_Character_Movement :type "CharacterMovementComponent Object Reference"))
  (return false null))

(fn `Get_PatrolPath`
  (params (B_Input :type Boolean))
  (returns (B_Success :type Boolean) (V_PathPoints :type "Array of Vector Structure") (BP_PatrolPath :type "/Game/Blueprints/AI/BP_PatrolPath Object Reference") (Start_Index :type Integer))
  (return false _ null 0))

(fn `NPC_Apply_Damage`
  (params (Damage_Applied :type "Float (double-precision)"))
  (returns (Success :type Boolean) (Destroyed_Actor :type Boolean))
  (return false false))

(fn `NPC_Start_Shooting`
  (returns (Success :type Boolean))
  (return false))

(fn `UserConstructionScript`)