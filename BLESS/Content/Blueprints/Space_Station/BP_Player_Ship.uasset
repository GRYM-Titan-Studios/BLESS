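; Player ship actor in the space station that de-cloaks when play begins and tells other actors when they are inside its radius.
; The construction script puts fully set-up M_Dissolve dynamic materials, with the ship's textures, on both mesh slots.
; Reappear plays a timeline that animates Dissolve_Amount on both materials.
; Ship_Area overlaps send WithinShipRadiusMessage true or false, with begin overlaps ignoring components named "Detection".
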(event `self.ReceiveBeginPlay`
  (`self.Reappear`))

(event `self.Ship_Area.OnComponentBeginOverlap`
  (params (OverlappedComponent :type "PrimitiveComponent Object Reference") (OtherActor :type "Actor Object Reference") (OtherComp :type "PrimitiveComponent Object Reference") (OtherBodyIndex :type Integer) (bFromSweep :type Boolean) (SweepResult :type "HitResult Structure (by ref)"))
  (if (not (`KismetStringLibrary.Contains` (`KismetSystemLibrary.GetDisplayName` OtherComp) "Detection"))
    (message `/Game/Blueprints/Interfaces/BPI_Data_Transfer.Within_Ship_Radius` OtherActor true)))

(event `self.Ship_Area.OnComponentEndOverlap`
  (params (OverlappedComponent :type "PrimitiveComponent Object Reference") (OtherActor :type "Actor Object Reference") (OtherComp :type "PrimitiveComponent Object Reference") (OtherBodyIndex :type Integer))
  (message `/Game/Blueprints/Interfaces/BPI_Data_Transfer.Within_Ship_Radius` OtherActor false))

(event `Reappear`
  (bind (_direction _appearance) (`Timeline|DeCloaking`)
    (:`Update`
      (`MaterialInstanceDynamic.SetScalarParameterValue` (`self.DIM_Dissolve`) "Dissolve_Amount" _appearance)
      (`MaterialInstanceDynamic.SetScalarParameterValue` (`self.DMI_Dissolve_Body`) "Dissolve_Amount" _appearance))))

(fn `UserConstructionScript`
  (bind _dim_dissolve (`self.DIM_Dissolve`))
  (bind _dmi_dissolve_body (`self.DMI_Dissolve_Body`))
  (bind _returnvalue (`PrimitiveComponent.CreateDynamicMaterialInstance` (`self.SM_Ship`) 0 "/Game/Materials/Stealth/M_Dissolve.M_Dissolve" "None"))
  (bind _output_get (set `self.DIM_Dissolve` _returnvalue))
  (`MaterialInstanceDynamic.SetScalarParameterValue` _output_get "Dissolve_Amount" 1.0)
  (`MaterialInstanceDynamic.SetTextureParameterValue` _dim_dissolve "Texture_BC" "/Game/Textures/Ship/T_Ship_Attachments_BC.T_Ship_Attachments_BC")
  (`MaterialInstanceDynamic.SetTextureParameterValue` _dim_dissolve "Texture_M" "/Game/Textures/Ship/T_Ship_Attachments_M.T_Ship_Attachments_M")
  (`MaterialInstanceDynamic.SetTextureParameterValue` _dim_dissolve "Texture_N" "/Game/Textures/Ship/T_Ship_Attachments_N.T_Ship_Attachments_N")
  (bind _returnvalue_2 (`PrimitiveComponent.CreateDynamicMaterialInstance` (`self.SM_Ship`) 1 "/Game/Materials/Stealth/M_Dissolve.M_Dissolve" "None"))
  (bind _output_get_2 (set `self.DMI_Dissolve_Body` _returnvalue_2))
  (`MaterialInstanceDynamic.SetScalarParameterValue` _output_get_2 "Dissolve_Amount" 1.0)
  (`MaterialInstanceDynamic.SetTextureParameterValue` _dmi_dissolve_body "Texture_BC" "/Game/Textures/Ship/T_Ship_BC.T_Ship_BC")
  (`MaterialInstanceDynamic.SetTextureParameterValue` _dmi_dissolve_body "Texture_M" "/Game/Textures/Ship/T_Ship_M.T_Ship_M")
  (`MaterialInstanceDynamic.SetTextureParameterValue` _dmi_dissolve_body "Texture_N" "/Game/Textures/Ship/T_Ship_N.T_Ship_N"))