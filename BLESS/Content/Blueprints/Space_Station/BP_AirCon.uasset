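; BP_AirCon is a Space Station air conditioner prop that animates three louvre blades swinging back and forth.
; A looping timer started on BeginPlay steps a shared roll angle between zero and minus sixty degrees, with a boolean flipping direction at each limit.
; Cog rotation logic derived from the same angle is present but disconnected, so only the blades move.
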(event `self.ReceiveBeginPlay`
  (`KismetSystemLibrary.K2_SetTimerDelegate` (delegate `Movement`) 0.1 true))

(event `Movement`
  (bind _f_rotation (`self.F_Rotation`))
  (bind _f_rotation_2 (`self.F_Rotation`))
  (`SceneComponent.K2_SetRelativeRotation` (`self.SM_AirCon_Blade`) (`KismetMathLibrary.MakeRotator` (`self.F_Rotation`) -90.0) false false)
  (`SceneComponent.K2_SetRelativeRotation` (`self.SM_AirCon_Blade1`) (`KismetMathLibrary.MakeRotator` (`self.F_Rotation`) -90.0) false false)
  (`SceneComponent.K2_SetRelativeRotation` (`self.SM_AirCon_Blade2`) (`KismetMathLibrary.MakeRotator` (`self.F_Rotation`) -90.0) false false)
  (if (`self.B_Forward`)
    (set `self.F_Rotation` (- _f_rotation 1.0))
    (if (<= _f_rotation_2 -60.0)
      (set `self.B_Forward` false))
    (else
      (set `self.F_Rotation` (+ _f_rotation 1.0))
      (if (>= _f_rotation_2 0.0)
        (set `self.B_Forward` true)))))

(fn `UserConstructionScript`)