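; Space station sliding door, single or double, that can be locked behind a hacking puzzle and carry an open cost.
; Overlapping actors are tracked and sent lock and cost state via DoorsMessage; their reply, or an unlock through Doors, plays the opening timeline.
; The timeline reverses once tracked actors leave, with optional sounds.
; Construction script applies configurable meshes; InitiateHack and TerminalInformation report puzzle size and costs, while other interface functions are mostly stubs.
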(event `Unlocked`
  (bind _b_noise (`self.B_Noise`))
  (bind _sm_door (`self.SM_Door`))
  (bind _sm_door_2 (`self.SM_Door_2`))
  (bind _returnvalue (`SceneComponent.K2_GetComponentLocation` (`self.DefaultSceneRoot`)))
  ;[1 1 1] Open After the Door has been hacked initially
  (`|ExecutionSequence`
    (:`then_0`
      (if _b_noise :!label _label
        ;[1 1 1] Moving the door(s)
        (`GameplayStatics.PlaySoundAtLocation` "/Game/Audio/FX/Cues/SC_Door_Open.SC_Door_Open" _returnvalue (struct) 1.0 1.0 0.0 null null null)
        (set `self.B_Open` true)
        (bind (_direction _f_open_percent) (`Timeline|Timeline_Open` :!label _label_2)
          (:`Update`
            (`SceneComponent.K2_SetRelativeLocation` _sm_door (`KismetMathLibrary.MakeVector` (`KismetMathLibrary.Lerp` (`self.F_Door_1_Origin`) (`self.F_Door_1_Movement_Distance`) _f_open_percent) (.y (`SceneComponent.RelativeLocation` _sm_door)) (.z (`SceneComponent.RelativeLocation` _sm_door))) false false)
            (`/Engine/EditorBlueprintResources/StandardMacros.IsValid` _sm_door_2
              (:`Is Valid`
                (`SceneComponent.K2_SetRelativeLocation` _sm_door_2 (`KismetMathLibrary.MakeVector` (`KismetMathLibrary.Lerp` (`self.F_Door_2_Origin`) (`self.F_Door_2_Movement_Distance`) _f_open_percent) (.y (`SceneComponent.RelativeLocation` _sm_door_2)) (.z (`SceneComponent.RelativeLocation` _sm_door_2))) false false)))))
        (else
          (goto _label_2))))
    (:`then_1`
      (`KismetSystemLibrary.Delay` 5.0)
      (bind _b_can_close (`self.Closing_Check` null))
      (if _b_can_close
        (if _b_noise :!label _label_3
          (if (`self.B_Open`)
            (`GameplayStatics.PlaySoundAtLocation` "/Game/Audio/FX/Cues/SC_Door_Close.SC_Door_Close" _returnvalue (struct) 1.0 1.0 0.0 null null null)
            (set `self.B_Open` false)
            (goto _label_2 :!via `Reverse`)
            (else
              (goto _label_2 :!via `Reverse`)))
          (else
            (goto _label_2 :!via `Reverse`)))))))

(event `self.Player_Collision.OnComponentBeginOverlap`
  (params (OverlappedComponent :type "PrimitiveComponent Object Reference") (OtherActor :type "Actor Object Reference") (OtherComp :type "PrimitiveComponent Object Reference") (OtherBodyIndex :type Integer) (bFromSweep :type Boolean) (SweepResult :type "HitResult Structure (by ref)"))
  ;[1 1 1] Checking if the entering actor can open the door and adding them to the array of actors
  (if (not (`KismetStringLibrary.Contains` (`KismetSystemLibrary.GetDisplayName` OtherComp) "Detection_Sphere"))
    (`KismetArrayLibrary.Array_AddUnique` (`self.Overlapped Actors Array`) OtherActor)
    (bind _success (message `/Game/Blueprints/Interfaces/BPI_Energy.Doors` OtherActor (`self.B_Locked`) (`self.B_Paid`) (`self.F_Open_Cost`)))
    (if _success
      (goto _label))))

(event `self.Player_Collision.OnComponentEndOverlap`
  (params (OverlappedComponent :type "PrimitiveComponent Object Reference") (OtherActor :type "Actor Object Reference") (OtherComp :type "PrimitiveComponent Object Reference") (OtherBodyIndex :type Integer))
  ;[1 1 1] Check if everything that has entered the door area has exited
  (if (!= OtherComp (`self.SM_Door`))
    (bind _b_can_close (`self.Closing_Check` OtherActor))
    (if _b_can_close
      (goto _label_3))))

(fn `Add_To_Player_Inventory`
  (params (Added_Item :type "/Game/Blueprints/Gameplay/STRUCT_Player_Item Structure"))
  (returns (Success :type Boolean))
  (return false))

(fn `Add_To_Ship_Inventory`
  (params (STRUCT_New_Item :type "/Game/Blueprints/Gameplay/STRUCT_Ship_Item Structure"))
  (returns (Success :type Boolean))
  (return false))

(fn `Aiming_At_Hack_Panel`
  (returns (Success :type Boolean))
  (return false))

(fn `Closing_Check`
  (params (Leaving_Actor_Ref :type "Actor Object Reference"))
  (returns (B_Can_Close :type Boolean))
  (bind _overlapped_actors_array (`self.Overlapped Actors Array`))
  (bind _returnvalue (`KismetArrayLibrary.Array_Length` _overlapped_actors_array))
  (if (> _returnvalue 0)
    (for _array_element _overlapped_actors_array
      (`/Engine/EditorBlueprintResources/StandardMacros.IsValid` _array_element
        (:`Is Valid`
          (if (== Leaving_Actor_Ref _array_element)
            (`KismetArrayLibrary.Array_RemoveItem` _overlapped_actors_array _array_element)))
        (:`Is Not Valid`
          (`KismetArrayLibrary.Array_RemoveItem` _overlapped_actors_array _array_element))))
    (return (== _returnvalue 0))))

(fn `Doors`
  (params (B_Locked :type Boolean) (B_Paid :type Boolean) (F_Cost :type "Float (double-precision)"))
  (returns (Success :type Boolean))
  (set `self.B_Locked` B_Locked)
  (set `self.B_Paid` B_Paid)
  (if (not B_Locked)
    (`self.Unlocked`))
  (return false))

(fn `Energy_Drain`
  (returns (Success :type Boolean) (Energy_Taken :type "Float (double-precision)") (S_Dialogue :type String))
  (return false 0.0 ""))

(fn `Hack_Success`
  (params (B_Locked :type Boolean) (B_Paid :type Boolean))
  (returns (B_Is_Locked :type Boolean) (B_Is_Paid :type Boolean))
  (return false false))

(fn `Hack_Successful`
  (params (Successful :type Boolean) (Cost_Paid :type Boolean) (I_Door_Cost :type Integer))
  (returns (Success :type Boolean) (Paid :type Boolean))
  (return false false))

(fn `Initiate_Hack`
  (returns (Success :type Boolean) (Unlock_Cost :type Integer) (Open_Cost :type Integer) (Door_Difficulty :type Integer))
  (bind _i_num_of_tiles (`self.I_Num_Of_Tiles`))
  (if (`self.B_Locked`)
    (`KismetSystemLibrary.PrintString` (`KismetStringLibrary.Conv_IntToString` _i_num_of_tiles) true true (struct :`R` 1.0 :`G` 0.005931 :`A` 1.0) 5.0)
    (return true (`self.I_Unlock_Cost`) (`KismetMathLibrary.FTrunc` (`self.F_Open_Cost`)) _i_num_of_tiles)
    (else
      (return false 0 0 _i_num_of_tiles))))

(fn `Move_Elevator`
  (params (Elevator_Choice :type Integer) (Start_Point_In :type "Float (double-precision)"))
  (returns (Success :type Boolean) (Start_Point :type "Float (double-precision)") (Chosen_Floor :type "Float (double-precision)"))
  (return false 0.0 0.0))

(fn `Open_Elevator_Panel`
  (returns (Success :type Boolean))
  (return false))

(fn `Pick_Up_Sorting`
  (returns (Success :type Boolean) (S_Type :type String) (S_Name :type String))
  (return false "" ""))

(fn `Picked_Up`
  (returns (Success :type Boolean))
  (return false))

(fn `Player_Energy_Adjustment`
  (params (Adjustment :type "Float (double-precision)"))
  (returns (Success :type Boolean))
  (return false))

(fn `Player_Health_Adjustment`
  (params (Adjustment :type Integer))
  (returns (Success :type Boolean))
  (return false))

(fn `Player_Inventory_Update`
  (params (Input :type Boolean))
  (returns (Success :type Boolean) (Player_Inventory :type "Array of /Game/Blueprints/Gameplay/STRUCT_Player_Item Structure"))
  (return false))

(fn `Player_Invisible?`
  (returns (Success :type Boolean) (Invisible :type Boolean))
  (return false false))

(fn `Ship_Energy_Update`
  (params (Input :type Boolean))
  (returns (Success :type Boolean) (Current_Energy :type Integer) (Max_Energy :type Integer))
  (return false 0 0))

(fn `Ship_Inventory_Update`
  (params (Input :type Boolean))
  (returns (Success :type Boolean) (Ship_Inventory :type "Array of /Game/Blueprints/Gameplay/STRUCT_Ship_Inventory Structure") (Current_Inventory_Count :type "Float (double-precision)") (Max_Inventory_Count :type "Float (double-precision)") (Inventory_Value :type Integer))
  (return false _ 0.0 0.0 0))

(fn `Starting_Information`
  (params (STRUCT_Weapon :type "/Game/Blueprints/Gameplay/STRUCT_Weapons Structure") (B_Check :type Boolean) (I_First :type Integer) (I_Second :type Integer) (I_Third :type Integer) (I_Fourth :type Integer) (`Actor Ref` :type "Actor Object Reference"))
  (returns (Success :type Boolean) (B_Second :type Boolean) (S_String :type String) (S_String_Second :type String) (I_Ref_Int :type Integer) (I_Ref_Int_Second :type Integer))
  (return false false "" "" 0 0))

(fn `Swap_Button_Recieving`
  (returns (B_Success :type Boolean))
  (return false))

(fn `Swap_Button_Sending`
  (params (I_Row_Goal :type Integer) (I_Column_Goal :type Integer) (Widget_Ref :type "Widget Object Reference"))
  (returns (B_Success :type Boolean) (I_Row_Position :type Integer) (I_Column_Position :type Integer))
  (return false 0 0))

(fn `Teleport_Cost`
  (params (Input :type Boolean) (F_Current_Energy :type "Float (double-precision)"))
  (returns (Success :type Boolean) (`I_Teleport Cost` :type Integer))
  (return false 0))

(fn `Terminal_Information`
  (params (Object_Array :type "Array of Object Object Reference (by ref)"))
  (returns (Success :type Boolean) (I_Open_Cost :type Integer) (I_Unlock_Cost :type Integer) (I_Num_Tiles :type Integer) (I_Num_Columns :type Integer) (I_Puzzle_Choice :type Integer))
  (`KismetSystemLibrary.PrintString` "Hello")
  (return true (`KismetMathLibrary.FTrunc` (`self.F_Open_Cost`)) (`self.I_Unlock_Cost`) (`self.I_Num_Of_Tiles`) (`self.I_Num_of_Columns`) 0))

(fn `Update_Display`
  (params (B_Update :type Boolean))
  (returns (Success :type Boolean) (B_Second_Hint :type Boolean) (S_Interact_Type :type String) (S_Second_Interact :type String) (I_Image_Hint_Ref :type Integer))
  (return false false "" "" 0))

(fn `Update_Highlight`
  (params (Highlight :type Boolean))
  (returns (Success :type Boolean) (F_Percent :type "Float (double-precision)"))
  (return false 0.0))

(fn `UserConstructionScript`
  (`|ExecutionSequence`
    (:`then_0`
      (`StaticMeshComponent.SetStaticMesh` (`self.SM_Door_Frame`) (`self.SM_Door_Frame_Ref`)))
    (:`then_1`
      (`StaticMeshComponent.SetStaticMesh` (`self.SM_Door`) (`self.SM_Door_Ref`)))
    (:`then_2`
      (`StaticMeshComponent.SetStaticMesh` (`self.SM_Door_2`) (`self.SM_Door_2_Ref`)))
    (:`then_3`
      (`StaticMeshComponent.SetStaticMesh` (`self.SM_Door_Frame_S`) (`self.SM_Door_Frame_S_Ref`)))))

(fn `Within_Ship_Radius`
  (params (B_Within :type Boolean))
  (returns (B_Success :type Boolean))
  (return false))