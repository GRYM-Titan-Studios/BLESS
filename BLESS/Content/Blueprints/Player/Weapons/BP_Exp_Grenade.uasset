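; Thrown-grenade actor that explodes on a timer and makes AI-audible noise when it hits surfaces.
; BeginPlay sets detonation just before InitialLifeSpan expires, spawning an enlarged BP_Grenade_Explosion at the grenade component's transform.
; Hit events report noise, throttled by a wrapping impact counter.
; Construction loads the LaserShotgun row from DT_Weapons, though nothing reads it; interface functions are stubs, including a disconnected StartingInformation.
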(event `self.ReceiveBeginPlay`
  (`KismetSystemLibrary.K2_SetTimerDelegate` (delegate `Detonate`) (- (`self.InitialLifeSpan`) 0.2)))

(event `Detonate`
  (bind (_returnvalue_location _returnvalue_rotation) (`KismetMathLibrary.BreakTransform` (`SceneComponent.K2_GetComponentToWorld` (`self.Greande`))))
  (`|SpawnActorFromClass` "/Game/Blueprints/Player/Weapons/BP_Grenade_Explosion.BP_Grenade_Explosion_C" (`KismetMathLibrary.MakeTransform` _returnvalue_location _returnvalue_rotation (2.5 2.5 2.5)) "Undefined" "OverrideRootScale" null null))

(event `self.Greande.OnComponentHit`
  (params (HitComponent :type "PrimitiveComponent Object Reference") (OtherActor :type "Actor Object Reference") (OtherComp :type "PrimitiveComponent Object Reference") (NormalImpulse :type "Vector Structure") (Hit :type "HitResult Structure (by ref)"))
  (bind _i_impact (`self.I_Impact`))
  (if (== _i_impact 0)
    (`AISense_Hearing.ReportNoiseEvent` Hit_Location 1.0 (`self.GetOwner`) 0.0 "Noise")
    (`/Engine/EditorBlueprintResources/StandardMacros.IncrementInt` (`self.I_Impact`))
    (else
      (bind _result (`/Engine/EditorBlueprintResources/StandardMacros.IncrementInt` _i_impact)
        (:`  `
          (if (== _result 20)
            (set `self.I_Impact` 0)))))))

(fn `Add_To_Player_Inventory`
  (params (Added_Item :type "/Game/Blueprints/Gameplay/STRUCT_Player_Item Structure"))
  (returns (Success :type Boolean))
  (return false))

(fn `Add_To_Ship_Inventory`
  (params (STRUCT_New_Item :type "/Game/Blueprints/Gameplay/STRUCT_Ship_Item Structure"))
  (returns (Success :type Boolean))
  (return false))

(fn `Check_Keycard`
  (params (I_Card_Ref :type Integer))
  (returns (B_Keycard_Owned :type Boolean))
  (return false))

(fn `Move_Elevator`
  (params (Elevator_Choice :type Integer) (Start_Point_In :type "Float (double-precision)"))
  (returns (Success :type Boolean) (Start_Point :type "Float (double-precision)") (Chosen_Floor :type "Float (double-precision)"))
  (return false 0.0 0.0))

(fn `Open_Elevator_Panel`
  (returns (Success :type Boolean))
  (return false))

(fn `Player_Inventory_Update`
  (params (Input :type Boolean))
  (returns (Success :type Boolean) (Player_Inventory :type "Array of /Game/Blueprints/Gameplay/STRUCT_Player_Item Structure"))
  (return false))

(fn `Player_Invisible?`
  (returns (Success :type Boolean) (Invisible :type Boolean))
  (return false false))

(fn `Ship_Energy_Update`
  (params (Input :type Boolean))
  (returns (Success :type Boolean) (Current_Energy :type Integer) (Max_Energy :type Integer))
  (return false 0 0))

(fn `Ship_Inventory_Update`
  (params (Input :type Boolean))
  (returns (Success :type Boolean) (Ship_Inventory :type "Array of /Game/Blueprints/Gameplay/STRUCT_Ship_Inventory Structure") (Current_Inventory_Count :type "Float (double-precision)") (Max_Inventory_Count :type "Float (double-precision)") (Inventory_Value :type Integer))
  (return false _ 0.0 0.0 0))

(fn `Starting_Information`
  (params (STRUCT_Weapon :type "/Game/Blueprints/Gameplay/STRUCT_Weapons Structure") (B_Check :type Boolean) (I_First :type Integer) (I_Second :type Integer) (I_Third :type Integer) (I_Fourth :type Integer) (`Actor Ref` :type "Actor Object Reference"))
  (returns (Success :type Boolean) (B_Second :type Boolean) (S_String :type String) (S_String_Second :type String) (I_Ref_Int :type Integer) (I_Ref_Int_Second :type Integer))
  ;[1 1 1] Adjusting details about the bullet upon launch
)

(fn `Update_Display`
  (params (B_Update :type Boolean))
  (returns (Success :type Boolean) (B_Second_Hint :type Boolean) (S_Interact_Type :type String) (S_Second_Interact :type String) (I_Image_Hint_Ref :type Integer))
  (return false false "" "" 0))

(fn `Update_Highlight`
  (params (Highlight :type Boolean) (Pulse_Exclusive :type Boolean))
  (returns (Success :type Boolean) (F_Percent :type "Float (double-precision)"))
  (return false 0.0))

(fn `Update_Keycard`
  (params (I_Card_Ref :type Integer))
  (returns (Success :type Boolean))
  (return false))

(fn `UserConstructionScript`
  (bind _returnvalue (`|GetDataTableRow` "/Game/Blueprints/Gameplay/DT_Weapons.DT_Weapons" "LaserShotgun")
    (:`then`
      (set `self.STRUCT_Bullet_Infomation` _returnvalue))))

(fn `Within_Ship_Radius`
  (params (B_Within :type Boolean))
  (returns (B_Success :type Boolean))
  (return false))