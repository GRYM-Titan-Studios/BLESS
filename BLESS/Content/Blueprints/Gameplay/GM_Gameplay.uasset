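; Gameplay GameMode holding shared state for area threat levels, ship inventory and dialogue.
; Areas load from a data table on BeginPlay; threat increases floor into alert levels that message all BPI_NPC actors, with one-time dialogue at levels 1 and 5.
; Ship items stack by ID, with total sale value recomputed on query.
; Dialogue rows drive HUD text and audio, queueing low-numbered lines while one plays; many other functions are stubs.
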(event `Dialogue_Delay`
  (params (F_Delay :type "Float (double-precision)"))
  (bind _i_queued_dialogue_array (`self.I_Queued_Dialogue_Array`))
  (`KismetSystemLibrary.Delay` F_Delay)
  (`/Game/Blueprints/Interfaces/BPI_Dialogue.Call_Dialogue` (`self.HUD_Ref`) 0 "")
  (set `self.B_Dialogue_Playing` false)
  (`KismetSystemLibrary.Delay` 0.5)
  (if (`KismetArrayLibrary.Array_IsValidIndex` (`self.I_Queued_Dialogue_Array`))
    (message `/Game/Blueprints/Interfaces/BPI_Dialogue.Call_Dialogue` (`GameplayStatics.GetGameMode`) (`|GetArrayItem` _i_queued_dialogue_array) "")
    (`KismetArrayLibrary.Array_Remove` _i_queued_dialogue_array)))

(event `self.ReceiveBeginPlay`
  (bind _outrownames (`DataTableFunctionLibrary.GetDataTableRowNames` (`self.DT_Areas_Ref`)))
  (for _array_element _outrownames
    (bind _returnvalue (`|GetDataTableRow` (`self.DT_Areas_Ref`) _array_element)
      (:`then`
        (`KismetArrayLibrary.Array_Add` (`self.STRUCT_Areas_Array`) _returnvalue)))))

(event `Update_Threat_Level`
  (params (Area_Name :type String) (Threat_Level_ :type "Float (double-precision)") (Area_ID :type Integer))
  (bind _struct_areas_array (`self.STRUCT_Areas_Array`))
  (bind (_area_id _area_name _curent_threat_level) (break `/Game/Blueprints/Gameplay/STRUCT_Areas` (`|GetArrayItem` _struct_areas_array Area_ID)))
  (bind _returnvalue (+ _curent_threat_level Threat_Level_))
  (bind _returnvalue_2 (`KismetMathLibrary.FFloor` _returnvalue))
  (bind _returnvalue_3 (>= _returnvalue_2 1))
  (`KismetArrayLibrary.Array_Set` _struct_areas_array Area_ID (make `/Game/Blueprints/Gameplay/STRUCT_Areas` _area_id _area_name _returnvalue _returnvalue_2))
  (if _returnvalue_3
    (bind _outactors (`GameplayStatics.GetAllActorsWithInterface` "/Game/Blueprints/AI/BPI_NPC.BPI_NPC_C"))
    (for _array_element _outactors
      (message `/Game/Blueprints/AI/BPI_NPC.Alert_Level_1` _array_element _returnvalue_3 _returnvalue_2))))

(fn `Add_Inventory_Quantity`
  (params (I_Array_Reference :type Integer))
  (bind _struct_current_ship_inventory_array (`self.STRUCT_Current_Ship_Inventory_Array`))
  (bind (_ship_item _current_quantity) (break `/Game/Blueprints/Gameplay/STRUCT_Ship_Inventory` (`|GetArrayItem` _struct_current_ship_inventory_array I_Array_Reference)))
  ;[1 1 1] Increment the Quantity of an item
  (`KismetArrayLibrary.Array_Set` _struct_current_ship_inventory_array I_Array_Reference (make `/Game/Blueprints/Gameplay/STRUCT_Ship_Inventory` _ship_item (+ _current_quantity 1))))

(fn `Add_To_Player_Inventory`
  (params (Added_Item :type "/Game/Blueprints/Gameplay/STRUCT_Player_Item Structure"))
  (returns (Success :type Boolean))
  (return false))

(fn `Add_To_Ship_Inventory`
  (params (STRUCT_New_Item :type "/Game/Blueprints/Gameplay/STRUCT_Ship_Item Structure"))
  (returns (Success :type Boolean))
  (locals (B_Item_Exists :type Boolean) (I_Array_Ref :type Integer) (F_Item_Size :type "Float (double-precision)"))
  ;[1 1 1] A function to Check if the item has been found before and if it has, increment the quantity, if not, add to Ship Array, -- In both events add the weight to the current value
  (for (_array_element _array_index) (`self.STRUCT_Current_Ship_Inventory_Array`)
    (bind (_item_id _category _name _size) (break `/Game/Blueprints/Gameplay/STRUCT_Ship_Item` (`.Ship_Item_2_1EB012044B865AF19B1805BE0AC7B31E` (break `/Game/Blueprints/Gameplay/STRUCT_Ship_Inventory` _array_element))))
    (if (== _item_id (`.Item_ID_30_E8212CB94383FF30D654D3B5CD902DCB` (break `/Game/Blueprints/Gameplay/STRUCT_Ship_Item` STRUCT_New_Item)))
      (set `local.B_Item_Exists` true)
      (set `local.I_Array_Ref` _array_index)
      (set `local.F_Item_Size` _size)))
  (if (`local.B_Item_Exists`)
    (`self.Add_Inventory_Quantity` (`local.I_Array_Ref`))
    (else
      (`KismetArrayLibrary.Array_AddUnique` (`self.STRUCT_Current_Ship_Inventory_Array`) (make `/Game/Blueprints/Gameplay/STRUCT_Ship_Inventory` STRUCT_New_Item 1))
      (`KismetSystemLibrary.PrintString` "GM - Add Ship - Added Unique")))
  (set `self.I_Current_Inventory_Count` (+ (`self.I_Current_Inventory_Count`) (`local.F_Item_Size`)))
  (`self.Ship_Inventory_Update` false)
  (return false))

(fn `Alert_Level_Notifies`
  (params (I_Alert_Level :type Integer))
  (if (== I_Alert_Level 1)
    (if (not (`self.B_Alert_Lv1_Notified`))
      (set `self.B_Alert_Lv1_Notified` true)
      (message `/Game/Blueprints/Interfaces/BPI_Dialogue.Call_Dialogue` (`GameplayStatics.GetGameMode`) 8 ""))
    (elif (== I_Alert_Level 5)
      (if (not (`self.B_Alert_Lv5_Notified`))
        (set `self.B_Alert_Lv5_Notified` true)
        (message `/Game/Blueprints/Interfaces/BPI_Dialogue.Call_Dialogue` (`GameplayStatics.GetGameMode`) 9 "")))))

(fn `Call_Dialogue`
  (params (I_Reference :type Integer) (S_Dialogue :type String))
  (returns (Success :type Boolean))
  (if (`self.B_Dialogue_Playing`)
    (if (<= I_Reference 9)
      (`KismetArrayLibrary.Array_AddUnique` (`self.I_Queued_Dialogue_Array`) I_Reference)
      (return true)
      (else
        (return true)))
    (else
      (set `self.B_Dialogue_Playing` true)
      (bind _returnvalue (`|GetDataTableRow` "/Game/Blueprints/Gameplay/DT_Dialogue.DT_Dialogue" (`KismetStringLibrary.Conv_StringToName` (`KismetStringLibrary.Conv_IntToString` I_Reference)))
        (:`then`
          (bind (_i_reference _s_dialogue _sc_dialogue _f_duration) (break `/Game/Blueprints/Gameplay/STRUCT_Dialogue` _returnvalue))
          (`/Game/Blueprints/Interfaces/BPI_Dialogue.Call_Dialogue` (`self.HUD_Ref`) 0 _s_dialogue)
          (`GameplayStatics.PlaySound2D` _sc_dialogue 1.0 1.0 0.0 null null)
          (`self.Dialogue_Delay` _f_duration)
          (return true))))))

(fn `Check_Keycard`
  (params (I_Card_Ref :type Integer))
  (returns (B_Keycard_Owned :type Boolean))
  (return false))

(fn `Get_Active_Threat_Level`
  (params (Input :type Boolean) (Area_ID :type Integer))
  (returns (Success :type Boolean) (Active_Threat_Level :type Integer))
  (bind (_output_area_id _output_area_name _output_curent_threat_level _output_active_threat_level) (break `/Game/Blueprints/Gameplay/STRUCT_Areas` (`|GetArrayItem` (`self.STRUCT_Areas_Array`) Area_ID)))
  (return false _output_active_threat_level))

(fn `Get_Current_Threat_Level`
  (params (Input :type Boolean) (Area_ID :type Integer))
  (returns (Success :type Boolean) (Current_Threat_Level :type "Float (double-precision)"))
  (bind (_output_area_id _output_area_name _output_curent_threat_level) (break `/Game/Blueprints/Gameplay/STRUCT_Areas` (`|GetArrayItem` (`self.STRUCT_Areas_Array`) Area_ID)))
  (return false _output_curent_threat_level))

(fn `Move_Elevator`
  (params (Elevator_Choice :type Integer) (Start_Point_In :type "Float (double-precision)"))
  (returns (Success :type Boolean) (Start_Point :type "Float (double-precision)") (Chosen_Floor :type "Float (double-precision)"))
  (return false 0.0 0.0))

(fn `Open_Elevator_Panel`
  (returns (Success :type Boolean))
  (return false))

(fn `Player_Inventory_Update`
  (params (Input :type Boolean))
  (returns (Success :type Boolean) (Player_Inventory :type "Array of /Game/Blueprints/Gameplay/STRUCT_Player_Item Structure"))
  (return false))

(fn `Player_Invisible?`
  (returns (Success :type Boolean) (Invisible :type Boolean))
  (return false false))

(fn `Setup_Dialogue`
  (params (HUD_Ref :type "/Game/UI/UI_Crosshair Object Reference"))
  (returns (Success :type Boolean))
  (set `self.HUD_Ref` HUD_Ref)
  (return false))

(fn `Ship_Energy_Update`
  (params (Input :type Boolean))
  (returns (Success :type Boolean) (Current_Energy :type Integer) (Max_Energy :type Integer))
  (return false 150 3000))

(fn `Ship_Inventory_Update`
  (params (Input :type Boolean))
  (returns (Success :type Boolean) (Ship_Inventory :type "Array of /Game/Blueprints/Gameplay/STRUCT_Ship_Inventory Structure") (Current_Inventory_Count :type "Float (double-precision)") (Max_Inventory_Count :type "Float (double-precision)") (Inventory_Value :type Integer))
  (set `self.I_Inventory_Value` 0)
  (for _array_element (`self.STRUCT_Current_Ship_Inventory_Array`)
    (bind (_ship_item _current_quantity) (break `/Game/Blueprints/Gameplay/STRUCT_Ship_Inventory` _array_element))
    (set `self.I_Inventory_Value` (+ (`self.I_Inventory_Value`) (* (`.Sale_Value_26_E65888134A8B7D621CB52EB17197F3D9` (break `/Game/Blueprints/Gameplay/STRUCT_Ship_Item` _ship_item)) _current_quantity))))
  (return false (`self.STRUCT_Current_Ship_Inventory_Array`) (`self.I_Current_Inventory_Count`) (`self.I_Max_Inventory_Count`) (`self.I_Inventory_Value`)))

(fn `Starting_Information`
  (params (STRUCT_Weapon :type "/Game/Blueprints/Gameplay/STRUCT_Weapons Structure") (B_Check :type Boolean) (I_First :type Integer) (I_Second :type Integer) (I_Third :type Integer) (I_Fourth :type Integer) (`Actor Ref` :type "Actor Object Reference") (V_Location :type "Vector Structure"))
  (returns (Success :type Boolean) (B_Second :type Boolean) (S_String :type String) (S_String_Second :type String) (I_Ref_Int :type Integer) (I_Ref_Int_Second :type Integer))
  (set `self.F_Countdown_Time` (+ (`KismetSystemLibrary.GetGameTimeInSeconds`) 600.0))
  (return false false "" "" 0 0))

(fn `Update_Color`
  (params (B_Update :type Boolean))
  (returns (Success :type Boolean))
  (return false))

(fn `Update_Current_Threat_Level`
  (params (Input :type Boolean) (Threat_Level_Increase :type "Float (double-precision)") (Area_ID :type Integer))
  (returns (Success :type Boolean))
  (locals (I_Display_Level :type Integer :default 0))
  (bind _struct_areas_array (`self.STRUCT_Areas_Array`))
  (bind (_area_id _area_name _curent_threat_level) (break `/Game/Blueprints/Gameplay/STRUCT_Areas` (`|GetArrayItem` (`self.STRUCT_Areas_Array`) Area_ID)))
  (bind _returnvalue (+ Threat_Level_Increase _curent_threat_level))
  (bind _returnvalue_2 (`KismetMathLibrary.FFloor` _returnvalue))
  (bind _returnvalue_3 (>= _returnvalue_2 1))
  (set `local.I_Display_Level` _returnvalue_2)
  (if _returnvalue_3
    (`KismetArrayLibrary.Array_Set` _struct_areas_array Area_ID (make `/Game/Blueprints/Gameplay/STRUCT_Areas` _area_id _area_name _returnvalue (`local.I_Display_Level`)))
    (`self.Alert_Level_Notifies` (`local.I_Display_Level`))
    (bind _outactors (`GameplayStatics.GetAllActorsWithInterface` "/Game/Blueprints/AI/BPI_NPC.BPI_NPC_C"))
    (for _array_element _outactors
      (message `/Game/Blueprints/AI/BPI_NPC.Alert_Level_1` _array_element _returnvalue_3 (`local.I_Display_Level`)))
    (return false)
    (else
      (`KismetArrayLibrary.Array_Set` _struct_areas_array Area_ID (make `/Game/Blueprints/Gameplay/STRUCT_Areas` _area_id _area_name _returnvalue (`local.I_Display_Level`))))))

(fn `Update_Display`
  (params (B_Update :type Boolean))
  (returns (Success :type Boolean) (B_Second_Hint :type Boolean) (S_Interact_Type :type String) (S_Second_Interact :type String) (I_Image_Hint_Ref :type Integer))
  (set `self.B_Using_Controller` B_Update)
  (return false false "" "" 0))

(fn `Update_Highlight`
  (params (Highlight :type Boolean) (Pulse_Exclusive :type Boolean))
  (returns (Success :type Boolean) (F_Percent :type "Float (double-precision)"))
  (return (`self.B_Using_Controller`) 0.0))

(fn `Update_Keycard`
  (params (I_Card_Ref :type Integer))
  (returns (Success :type Boolean))
  (return false))

(fn `UserConstructionScript`)

(fn `Within_Ship_Radius`
  (params (B_Within :type Boolean))
  (returns (B_Success :type Boolean))
  (return false))