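; BP_Red_Light is a flashing lamp that turns its Colour1 green when its Doors function is called.
; The construction script puts a dynamic MI_Flashing_Light instance on SMLamp, and Doors recolours that instance, ignoring its lock, payment and cost inputs.
; The other gameplay functions, covering hacking, pickups, energy, health and teleport cost, are stubs returning defaults, and the event graph is inactive.
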(fn `Doors`
  (params (B_Locked :type Boolean) (B_Paid :type Boolean) (F_Cost :type "Float (double-precision)"))
  (returns (Success :type Boolean))
  (`MaterialInstanceDynamic.SetVectorParameterValue` (`self.MI_Light`) "Colour1" (struct :`G` 1.0 :`A` 1.0))
  (return false))

(fn `Energy_Drain`
  (returns (Success :type Boolean) (Energy_Taken :type "Float (double-precision)") (S_Dialogue :type String))
  (return false 0.0 ""))

(fn `Hack_Successful`
  (params (Successful :type Boolean) (Cost_Paid :type Boolean) (I_Door_Cost :type Integer))
  (returns (Success :type Boolean) (Paid :type Boolean))
  (return false false))

(fn `Initiate_Hack`
  (returns (Success :type Boolean) (Unlock_Cost :type Integer) (Open_Cost :type Integer) (Door_Difficulty :type Integer))
  (return false 0 0 0))

(fn `Pick_Up_Sorting`
  (returns (Success :type Boolean) (S_Type :type String) (S_Name :type String))
  (return false "" ""))

(fn `Picked_Up`
  (returns (Success :type Boolean))
  (return false))

(fn `Player_Energy_Adjustment`
  (params (Adjustment :type "Float (double-precision)"))
  (returns (Success :type Boolean))
  (return false))

(fn `Player_Health_Adjustment`
  (params (Adjustment :type Integer))
  (returns (Success :type Boolean))
  (return false))

(fn `Teleport_Cost`
  (params (Input :type Boolean) (F_Current_Energy :type "Float (double-precision)"))
  (returns (Success :type Boolean) (`I_Teleport Cost` :type Integer))
  (return false 0))

(fn `UserConstructionScript`
  (bind _returnvalue (`PrimitiveComponent.CreateDynamicMaterialInstance` (`self.SM_Lamp`) 0 "/Game/Materials/Lights/MI_Flashing_Light.MI_Flashing_Light" "None"))
  (set `self.MI_Light` _returnvalue))