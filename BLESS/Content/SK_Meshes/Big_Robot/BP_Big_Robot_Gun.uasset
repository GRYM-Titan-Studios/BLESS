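; Big robot's gun turret that deploys, tracks the player and fires LaserShotgun projectiles from the weapons data table.
; A timeline raises and lowers the mount, while Tick turns two mount meshes toward the player's head.
; Interface calls drive deployment, alert/stun glow and shooting, gated by deployment and shot delay; most others are stubs.
; Shots scatter around the player, with vertical spread scaled by distance; ammo is never decremented.
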(event `self.ReceiveBeginPlay`
  ;[1 1 1] Begin Play
  (bind _returnvalue (`|GetDataTableRow` "/Game/Blueprints/Gameplay/DT_Weapons.DT_Weapons" "LaserShotgun")
    (:`then`
      (set `self.STRUCT_Equipped_Weapon` _returnvalue))))

(event `Gun_Shot_Delay`
  (params (F_Delay :type "Float (double-precision)"))
  ;[1 1 1] Delays
  (`KismetSystemLibrary.Delay` F_Delay)
  (set `self.B_Shot_Delay_Passed` true))

(event `Gun_Reload_Delay`
  (params (F_Delay :type "Float (double-precision)"))
  ;[1 1 1] Delays
  (`KismetSystemLibrary.Delay` F_Delay)
  (set `self.B_Gun_Reloaded` true))

(event `Cinematic_Up`
  ;[1 1 1] Deploy Gun
  (bind (_direction _gun_rise) (`Timeline|Gun_Rise` :!label _label)
    (:`Update`
      (`SceneComponent.K2_SetRelativeRotation` (`self.SM_Big_Robot_Gun_Mount_1`) (`KismetMathLibrary.MakeRotator` (+ (* 90 _gun_rise) -90.0)) false false))
    (:`Finished`
      (set `self.B_Gun_UP/Down_Finished` true)
      (bind _returnvalue (== _gun_rise 1.0))
      (set `self.B_Gun_Deployed` _returnvalue)
      (bind _returnvalue_2 (select `bool` _returnvalue :`false` (struct :`R` 1.0 :`B` 1.0 :`A` 1.0) :`true` (struct :`R` 1.0 :`A` 1.0) :!type "LinearColor Structure"))
      (`MaterialInstanceDynamic.SetVectorParameterValue` (`self.DMI_Gun`) "Emissive_Colour" _returnvalue_2)
      (`MaterialInstanceDynamic.SetVectorParameterValue` (`self.DMI_Ball`) "Colour" _returnvalue_2))))

(event `Gun_Up`
  ;[1 1 1] Deploy Gun
  (if (`self.B_Gun_Deployed`)
    _
    (elif (`self.B_Gun_UP/Down_Finished`)
      (set `self.B_Gun_UP/Down_Finished` false)
      (goto _label :!via `PlayFromStart`))))

(event `Gun_Down`
  ;[1 1 1] Deploy Gun
  (set `self.B_Gun_UP/Down_Finished` false)
  (goto _label :!via `ReverseFromEnd`))

(event `Cinematic_Down`
  ;[1 1 1] Deploy Gun
  (goto _label :!via `ReverseFromEnd`))

(event `self.ReceiveTick`
  (params (DeltaSeconds :type "Float (single-precision)"))
  (bind (_returnvalue_roll _returnvalue_pitch _returnvalue_yaw) (`KismetMathLibrary.BreakRotator` (`SceneComponent.K2_GetComponentRotation` (`self.DefaultSceneRoot`))))
  (bind (_returnvalue_roll_2 _returnvalue_pitch_2 _returnvalue_yaw_2) (`KismetMathLibrary.BreakRotator` (`KismetMathLibrary.FindLookAtRotation` (`SceneComponent.K2_GetComponentLocation` (`self.SM_Big_Robot_Gun_Mount_2`)) (`SceneComponent.GetSocketLocation` (`Character.Mesh` (`GameplayStatics.GetPlayerCharacter` 0)) "head"))))
  ;[1 1 1] Track the Player With Gun Barrel
  (if (and (`self.B_Gun_UP/Down_Finished`) (`self.Gun_UP?`) (not (`self.B_Searching`)))
    (`SceneComponent.K2_SetRelativeRotation` (`self.SM_Big_Robot_Gun_Mount_2`) (`KismetMathLibrary.MakeRotator` 0.0 0.0 (+ (- _returnvalue_yaw_2 _returnvalue_yaw) -90.0)) false false)
    (`SceneComponent.K2_SetRelativeRotation` (`self.SM_Big_Robot_Gun_Mount_3`) (`KismetMathLibrary.MakeRotator` (* _returnvalue_pitch_2 -1.0)) false false)
    (else
      (`self.Reset_Gun_Pos`))))

(fn `Alert_Level_1`
  (params (Activate :type Boolean) (Alert_Level :type Integer))
  (returns (Success :type Boolean))
  (return false))

(fn `Call_Assist`
  (returns (B_Success :type Boolean))
  (return false))

(fn `Can_Shoot`
  (returns (Can_Shoot :type Boolean))
  (return (and (`self.B_Gun_Reloaded`) (`self.B_Shot_Delay_Passed`) (`self.B_Gun_Deployed`))))

(fn `Drone_Sensed_Player`
  (params (B_Sensed :type Boolean))
  (returns (Success :type Boolean))
  (return false))

(fn `Enter_Charging_Pod`
  (params (B_Occupied :type Boolean))
  (returns (B_Success :type Boolean))
  (return false))

(fn `Get_Gun_Ref`
  (returns (Gun_Ref :type "ChildActorComponent Object Reference"))
  (return null))

(fn `Get_NPC_Movement_Ref`
  (params (B_Input :type Boolean))
  (returns (B_Success :type Boolean) (NPC_Character_Movement :type "CharacterMovementComponent Object Reference"))
  (return false null))

(fn `Get_PatrolPath`
  (params (B_Input :type Boolean))
  (returns (B_Success :type Boolean) (V_PathPoints :type "Array of Vector Structure") (BP_PatrolPath :type "/Game/Blueprints/AI/BP_PatrolPath Object Reference") (Start_Index :type Integer))
  (return false _ null 0))

(fn `Gun_Ready`
  (params (`Gun_UP?` :type Boolean))
  (returns (Anim_Finished :type Boolean))
  (bind _output_get (set `self.Gun_UP?` `Gun_UP?`))
  (if _output_get
    (`self.Gun_Up`)
    (else
      (`self.Gun_Down`)))
  (return (`self.B_Gun_UP/Down_Finished`)))

(fn `Kill_Drone`
  (params (Input :type Boolean))
  (returns (Success :type Boolean))
  (set `self.B_Searching` true)
  (`self.Reset_Gun_Pos`)
  (return false))

(fn `NPC_Apply_Damage`
  (params (Damage_Applied :type "Float (double-precision)"))
  (returns (Success :type Boolean) (Destroyed_Actor :type Boolean))
  (return false false))

(fn `NPC_Start_Shooting`
  (params (`B_Can_Shoot?` :type Boolean))
  (returns (Success :type Boolean) (B_Can_Fire :type Boolean))
  (bind (_weapon_id _weapon_name _weapon_icon _weapon_skeletal_mesh _bullets_per_shot _rate_of_fire _current_ammo _max_ammo _single_shot_mode _area_damge _weapon_spread _damage_per_shot _bullet_speed _projectile_class _projectile_type _crosshair_image _fire_sound _muzzle_flash_effect _auto_reload _holster_socket _reload_time _weapon_shooting_animation _reload_animation _equip_animation _unequip_animation _zoom_values _sniper_scope_image _invisible_while_shooting) (break `/Game/Blueprints/Gameplay/STRUCT_Weapons` (`self.STRUCT_Equipped_Weapon`)))
  (bind _location (.location (`SceneComponent.K2_GetComponentToWorld` (`self.Shooting_Sphere`))))
  (if (and `B_Can_Shoot?` (`self.Can_Shoot`))
    (set `self.B_Searching` false)
    (set `self.B_Shot_Delay_Passed` false)
    (`self.Gun_Shot_Delay` _rate_of_fire)
    (bind _i_new_ammo (`self.Reduce_Ammo` _current_ammo _max_ammo _reload_time))
    (`|SpawnActorFromClass` _projectile_class (`KismetMathLibrary.MakeTransform` _location (`KismetMathLibrary.FindLookAtRotation` _location (`self.Weapon_Scatter` _weapon_spread))) "AdjustIfPossibleButAlwaysSpawn" "OverrideRootScale" self null)
    (`|SpawnActorFromClass` "/Game/Particles/BP_Impact_Spark.BP_Impact_Spark_C" (`KismetMathLibrary.MakeTransform` _location (.rotation (`SceneComponent.K2_GetComponentToWorld` (`self.Shooting_Sphere`)))) "Undefined" "OverrideRootScale" null null)
    (`GameplayStatics.PlaySoundAtLocation` "/Game/Audio/FX/Cues/SC_Blaster_Shot.SC_Blaster_Shot" (`SceneComponent.K2_GetComponentLocation` (`self.DefaultSceneRoot`)) (struct) 1.0 1.0 0.0 null null null)
    (return true false)))

(fn `Reduce_Ammo`
  (params (I_Current_Ammo :type Integer) (I_Max_Ammo :type Integer) (F_Reload_Time :type "Float (double-precision)"))
  (returns (I_New_Ammo :type Integer))
  (return I_Current_Ammo))

(fn `Reset_Gun_Pos`
  (bind _sm_big_robot_gun_mount_2 (`self.SM_Big_Robot_Gun_Mount_2`))
  (bind (_relativerotation_roll _relativerotation_pitch _relativerotation_yaw) (`KismetMathLibrary.BreakRotator` (`SceneComponent.RelativeRotation` _sm_big_robot_gun_mount_2)))
  (set `self.B_Gun_Pos_Reset` (== _relativerotation_yaw 0.0))
  (if (not (`self.B_Gun_Pos_Reset`))
    (`SceneComponent.K2_SetRelativeRotation` _sm_big_robot_gun_mount_2 (`KismetMathLibrary.MakeRotator` 0.0) false false)
    (`SceneComponent.K2_SetRelativeRotation` (`self.SM_Big_Robot_Gun_Mount_3`) (`KismetMathLibrary.MakeRotator` 0.0) false false)))

(fn `Set_Pod`
  (params (Pod_Ref :type "Actor Object Reference"))
  (returns (Success :type Boolean) (Send_Pod_Ref :type "Actor Object Reference"))
  (return false null))

(fn `Set_Position`
  (returns (Success :type Boolean) (V_Location :type "Vector Structure"))
  (return false (0.0 0.0 0.0)))

(fn `Spawn_SDrone`
  (returns (Success :type Boolean))
  (return false))

(fn `Stunned`
  (returns (B_Success :type Boolean))
  (return false))

(fn `Update Color (NPC)`
  (params (B_Alerted :type Boolean) (B_Stunned :type Boolean))
  (returns (Success :type Boolean))
  (`KismetSystemLibrary.PrintString` "Gun Got Message")
  (if (not B_Stunned)
    (`MaterialInstanceDynamic.SetScalarParameterValue` (`self.DMI_Gun`) "Emissive_Power" 250.0)
    (`MaterialInstanceDynamic.SetVectorParameterValue` (`self.DMI_Gun`) "Emissive_Colour" (select `bool` B_Alerted :`false` (struct :`R` 1.0 :`B` 1.0 :`A` 1.0) :`true` (struct :`R` 1.0 :`A` 1.0) :!type "LinearColor Structure"))
    (`SceneComponent.SetVisibility` (`self.Shooting_Sphere`) true false)
    (else
      (`MaterialInstanceDynamic.SetScalarParameterValue` (`self.DMI_Gun`) "Emissive_Power" 0.0)
      (`SceneComponent.SetVisibility` (`self.Shooting_Sphere`) false false)))
  (return false))

(fn `UserConstructionScript`
  (bind _returnvalue (`PrimitiveComponent.CreateDynamicMaterialInstance` (`self.SM_Big_Robot_Gun_Gun`) 0 "/Game/Materials/Robots/M_Big_Robot_Gun.M_Big_Robot_Gun" "None"))
  (set `self.DMI_Gun` _returnvalue)
  (bind _returnvalue_2 (`PrimitiveComponent.CreateDynamicMaterialInstance` (`self.Shooting_Sphere`) 0 "/Game/Materials/Particles/M_Glow_Ball.M_Glow_Ball" "None"))
  (bind _output_get (set `self.DMI_Ball` _returnvalue_2))
  (`MaterialInstanceDynamic.SetVectorParameterValue` _output_get "Colour" (struct :`R` 1.0 :`B` 1.0 :`A` 1.0)))

(fn `Weapon_Scatter`
  (params (F_Weapon_Spread :type "Float (double-precision)"))
  (returns (V_Adjusted_Aim :type "Vector Structure"))
  (bind _returnvalue (* F_Weapon_Spread -1.0))
  (bind (_returnvalue_x _returnvalue_y _returnvalue_z) (`KismetMathLibrary.BreakVector` (`SceneComponent.K2_GetComponentLocation` (`Character.Mesh` (`GameplayStatics.GetPlayerCharacter` 0)))))
  (bind _returnvalue_2 (/ (- (`KismetMathLibrary.Vector_Distance` (`SceneComponent.K2_GetComponentLocation` (`Character.Mesh` (`GameplayStatics.GetPlayerCharacter` 0))) (`SceneComponent.K2_GetComponentLocation` (`self.DefaultSceneRoot`))) 240.0) 1000.0))
  (return (`KismetMathLibrary.MakeVector` (+ _returnvalue_x (`KismetMathLibrary.RandomFloatInRange` _returnvalue F_Weapon_Spread)) (+ _returnvalue_y (`KismetMathLibrary.RandomFloatInRange` _returnvalue F_Weapon_Spread)) (+ (+ _returnvalue_z 130.0) (`KismetMathLibrary.RandomFloatInRange` (* _returnvalue_2 _returnvalue) (* _returnvalue_2 F_Weapon_Spread))))))